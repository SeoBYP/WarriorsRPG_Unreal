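; Base quest object that tracks one quest's objective progress through stages defined in DT_QuestDataTable.
; On BeginPlay it loads the current stage, binds to the hero's objective-ID event and seeds Collect objectives from inventory.
; Reported values update a progress map and broadcast changes; each completed objective shows a notification.
; Finished stages load the next, and the last marks completion, auto-turning in through BP_QuestLogComponent if configured.
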(event EventBeginPlay
  (CallFunction|GetQuestDetails)
  (EventDispatchers|AssignOnRequestObjectiveID (Class|WarriorFunctionLibrary|GetWarriorHeroCharacter) (EventDispatchers|CreateEvent :!event OnObjectiveIDHeard))
  (bind _array_element (Utilities|Array|ForEachLoopwithBreak (.Objectives (Utilities|Struct|BreakStageDetails (Variables|Default|GetCurrentStageDetails))))
    (:LoopBody
      (if (Utilities|Enum|Equal(Enum) (.Type (Utilities|Struct|BreakObjectiveDetails _array_element)) "Collect")
        (CallFunction|OnObjectiveIDHeard (.ObjectiveID (Utilities|Struct|BreakObjectiveDetails _array_element)) (.OutQuantity (Class|InventoryComponent|QueryInventory (Variables|/Script/Warriors.WarriorHeroCharacter|GetInventoryComponent (Class|WarriorFunctionLibrary|GetWarriorHeroCharacter)) (Utilities|String|StringToName (.ObjectiveID (Utilities|Struct|BreakObjectiveDetails _array_element))))))))
    (:Completed
      (bind _alliobjectivescomplete (CallFunction|AreObjectivesComplete))
      (Variables|Default|SetIsCompleted _alliobjectivescomplete))))

(fn ConstructionScript)

(fn OnObjectiveIDHeard
  (params (ObjectiveID :type String) (Value :type Integer))
  (bind _currentobjectiveprogress (Variables|Default|GetCurrentObjectiveProgress))
  (bind _outobjectivedetails (CallFunction|GetObjectiveDatabyID ObjectiveID))
  (bind (_value _returnvalue) (Utilities|Map|Find _currentobjectiveprogress ObjectiveID))
  (bind _quantity (Utilities|Struct|BreakObjectiveDetails _outobjectivedetails))
  (if (> (Class|KismetMathLibrary|SignOfInteger Value) 0)
    (if _returnvalue
      (if (< _value _quantity)
        (Utilities|Map|Add (Variables|Default|GetCurrentObjectiveProgress) ObjectiveID (+ _value Value))
        (CallFunction|IsObjectiveComplete ObjectiveID)
        (Default|CallOnQuestObjectiveUpdated)
        (return)
        (else
          (Development|PrintString (Utilities|String|ToString(Text) (Utilities|Text|FormatText "{current}/{max}" _value _quantity)))))
      (else
        (return)))
    (else
      (Utilities|Map|Add (Variables|Default|GetCurrentObjectiveProgress) ObjectiveID (+ (.Value (Utilities|Map|Find (Variables|Default|GetCurrentObjectiveProgress) ObjectiveID)) Value))
      (return))))

(fn GetQuestDetails
  (bind _returnvalue (Utilities|GetDataTableRow "/Game/DataTables/DT_QuestDataTable.DT_QuestDataTable" (Variables|Default|GetQuestID))
    (:then
      (bind _output_get (Variables|Default|SetQuestDetails _returnvalue))
      (bind _output_get_2 (Variables|Default|SetCurrentStageDetails (Utilities|Array|Get(acopy) (.Stages (Utilities|Struct|BreakQuestDataTable _output_get)) (Variables|Default|GetCurrentStage))))
      (Utilities|Map|Clear (Variables|Default|GetCurrentObjectiveProgress))
      (for _array_element (Utilities|Struct|BreakStageDetails _output_get_2)
        (Utilities|Map|Add (Variables|Default|GetCurrentObjectiveProgress) (.ObjectiveID (Utilities|Struct|BreakObjectiveDetails _array_element)) 0)))))

(fn GetObjectiveDatabyID
  (params (ObjectiveID :type String))
  (for _array_element (.Objectives (Utilities|Struct|BreakStageDetails (Variables|Default|GetCurrentStageDetails)))
    (if (Utilities|Enum|Equal(Enum) (.ObjectiveID (Utilities|Struct|BreakObjectiveDetails _array_element)) ObjectiveID)
      (return _array_element))))

(fn IsObjectiveComplete
  (params (ObjectiveID :type String))
  (bind _outobjectivedetails (CallFunction|GetObjectiveDatabyID ObjectiveID))
  (bind (_objectivename _description _type _objectiveid _quantity) (Utilities|Struct|BreakObjectiveDetails _outobjectivedetails))
  (if (>= (.Value (Utilities|Map|Find (Variables|Default|GetCurrentObjectiveProgress) ObjectiveID)) _quantity)
    (bind _returnvalue (UserInterface|CreateWidget "/Game/Widgets/QuestWidget/WBP_QuestNotification.WBP_QuestNotification_C" 0 _description))
    (UserInterface|Viewport|AddtoViewport _returnvalue 0)
    (bind _alliobjectivescomplete (CallFunction|AreObjectivesComplete))
    (if _alliobjectivescomplete
      (bind _result (Math|Integer|IncrementInt (Variables|Default|GetCurrentStage))
        (:%20%20
          (if (Utilities|Array|IsValidIndex (.stages (Variables|Default|GetQuestDetails)) _result)
            (CallFunction|GetQuestDetails)
            (else
              (Variables|Default|SetIsCompleted true)
              (if (.bautocomplete (Variables|Default|GetQuestDetails))
                (Default|TurninQuest (Actor|GetComponentbyClass (Class|WarriorFunctionLibrary|GetWarriorHeroCharacter) "/Game/Quest/BP_QuestLogComponent.BP_QuestLogComponent_C") (Variables|Default|GetQuestID))))))))))

(fn AreObjectivesComplete
  (for _array_element (.Objectives (Utilities|Struct|BreakStageDetails (Variables|Default|GetCurrentStageDetails)))
    (if (not (>= (.Value (Utilities|Map|Find (Variables|Default|GetCurrentObjectiveProgress) (.ObjectiveID (Utilities|Struct|BreakObjectiveDetails _array_element)))) (.Quantity (Utilities|Struct|BreakObjectiveDetails (CallFunction|GetObjectiveDatabyID (.ObjectiveID (Utilities|Struct|BreakObjectiveDetails _array_element)))))))
      (bind _output_get (LocalVariables|SetAllComplete false))
      (return _output_get)))
  (return (LocalVariables|GetAllComplete)))