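; Quest log component that records active and completed quests by ID and manages their lifecycle.
; Adding a quest spawns a BP_QuestBase actor to hold its state, which other functions find by searching on ID.
; Turn-in only prints the stage's XP reward, then completes the quest, flagging it turned in and firing OnQuestCompleted.
; Tracking creates or updates a single on-screen WBP_QuestTracker widget.
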(event EventBeginPlay)

(event EventTick
  (params (DeltaSeconds :type Float%20%28single-precision%29)))

(fn AddNewQuest
  (params (QuestID :type Name))
  (Utilities|Array|AddUnique (Variables|Default|GetCurrentActiveQuests) QuestID)
  (bind _returnvalue (Game|SpawnActorfromClass "/Game/Quest/BP_QuestBase.BP_QuestBase_C" (Math|Transform|MakeTransform "0, 0, 0" "0, 0, 0" "1.000000,1.000000,1.000000") "Undefined" "MultiplyWithRoot" 0 QuestID 0))
  (Utilities|Array|Add (Variables|Default|GetCurrentQuests) _returnvalue)
  (return _returnvalue))

(fn CompleteQuest
  (params (QuestID :type Name))
  (Utilities|Array|AddUnique (Variables|Default|GetCompletedQuests) QuestID)
  (Utilities|Array|RemoveItem (Variables|Default|GetCurrentActiveQuests) QuestID)
  (bind _array_element (CallFunction|GetQuestActor QuestID))
  (Variables|/Script/Warriors.QuestBase|SetIsTurned _array_element true)
  (Default|CallOnQuestCompleted _array_element))

(fn QueryActiveQuest
  (params (QuestID :type Name))
  (return (Utilities|Array|ContainsItem (Variables|Default|GetCurrentActiveQuests) QuestID)))

(fn TrackQuest
  (params (QuestActor :type Quest%20Base%20Object%20Reference))
  (bind _quest_tracker_widget (Variables|Default|GetQuest%20Tracker%20Widget)
    (:then
      (Default|Update _quest_tracker_widget QuestActor))
    (:else
      (bind _returnvalue (UserInterface|CreateWidget "/Game/Widgets/QuestWidget/WBP_QuestTracker.WBP_QuestTracker_C" 0 QuestActor))
      (bind _output_get (Variables|Default|SetQuest%20Tracker%20Widget _returnvalue))
      (UserInterface|Viewport|AddtoViewport _output_get -1))))

(fn GetQuestActor
  (params (QuestID :type Name))
  (for _array_element (Variables|Default|GetCurrentQuests)
    (if (== (Variables|/Script/Warriors.QuestBase|GetQuestID _array_element) QuestID)
      (return _array_element))))

(fn TurninQuest
  (params (QuestID :type Name))
  (Utilities|FlowControl|Sequence
    (:then_0
      (bind _array_element (CallFunction|GetQuestActor QuestID))
      (Development|PrintString (Utilities|String|ToString(Text) (Utilities|Text|FormatText "XP = {a}" (.XPReward (Utilities|Struct|BreakStageDetails (Variables|/Script/Warriors.QuestBase|GetCurrentStageDetails _array_element)))))))
    (:then_1
      (CallFunction|CompleteQuest QuestID))))

(fn QueryCompletedQuests
  (params (QuestID :type Name))
  (bind _completedquests (Variables|Default|GetCompletedQuests))
  (bind _returnvalue (Utilities|Array|ContainsItem _completedquests QuestID))
  (bind _array_element (CallFunction|GetQuestActor QuestID))
  (Utilities|IsValid _array_element
    (:Is%20Valid
      (return _returnvalue (Variables|/Script/Warriors.QuestBase|GetIsTurned _array_element)))
    (:Is%20Not%20Valid
      (return _returnvalue true))))