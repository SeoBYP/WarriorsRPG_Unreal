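; BP_NPC_Test is a test NPC that can be interacted with to report a quest objective.
; On BeginPlay it sets up its Interactable component from the "Talk" row of the interaction data table.
; On interact, it gets the objective ID from its quest giver component and passes it with a value of 1 to the interactor's owning WarriorHeroCharacter.
; GetObjectiveID also exposes that ID.
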(event OnInteract(Interactable)
  (params (Interactor :type Interactor%20Component%20Object%20Reference) (Interactable :type Interactable%20Component%20Object%20Reference))
  (bind _returnvalue (Class|QuestInterafece|GetObjectiveID(Message) (Variables|Default|GetBP_QuestGiverComponent)))
  (bind _aswarrior_hero_character (Utilities|Casting|CastToWarriorHeroCharacter (Components|GetOwner Interactor)))
  (Default|CallOnRequestObjectiveID _aswarrior_hero_character _returnvalue 1))

(event EventBeginPlay
  (|CallParentFunction)
  (Class|InteractableComponent|SetInteractableDataBasedonDataTable (Variables|Default|GetInteractable) "/Game/DataTables/DT_InteractDataTable.DT_InteractDataTable" "Talk"))

(event Collision|EventActorBeginOverlap
  (params (OtherActor :type Actor%20Object%20Reference)))

(event EventTick
  (params (DeltaSeconds :type Float%20%28single-precision%29)))

(fn ConstructionScript
  (|CallParentFunction))

(fn GetObjectiveID
  (bind _returnvalue (Class|QuestInterafece|GetObjectiveID(Message) (Variables|Default|GetBP_QuestGiverComponent)))
  (return _returnvalue))