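; Player hero character Blueprint that handles quest persistence and input for interaction and menus.
; BeginPlay loads quests from the game instance's save object into the quest log component, while hardcoded keys save quests to a slot or remove save data.
; Enhanced Input drives InteractorComponent, the async-loaded pause screen, the quest log, and an inventory toggle tracked through a widget subsystem.
; The HeroDialogueComponent calls are unwired and never run.
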(event Input|EnhancedActionEvents|EnhancedInputActionIA_PauseMenu
  (params (ActionValue :type Boolean) (ElapsedSeconds :type Float%20%28double-precision%29) (TriggeredSeconds :type Float%20%28double-precision%29) (InputAction :type Input%20Action%20Object%20Reference :default "/Game/Input/Actions/IA_PauseMenu.IA_PauseMenu"))
  (:Started
    (bind _class (Utilities|AsyncLoadClassAsset "/Game/Widgets/GameModeWidgets/WBP_PauseScreen.WBP_PauseScreen_C")
      (:then
        (bind _asuser_widget (Utilities|Casting|CastToUserWidgetClass _class))
        (bind _returnvalue (UserInterface|CreateWidget _asuser_widget))
        (UserInterface|Viewport|AddtoViewport _returnvalue 0)))))

(event Input|EnhancedActionEvents|EnhancedInputActionIA_Interact
  (params (ActionValue :type Boolean) (ElapsedSeconds :type Float%20%28double-precision%29) (TriggeredSeconds :type Float%20%28double-precision%29) (InputAction :type Input%20Action%20Object%20Reference :default "/Game/Input/Actions/IA_Interact.IA_Interact"))
  (:Started
    (Class|InteractorComponent|InteractionInput (Variables|Default|GetInteractorComponent) "DefaultKey" true))
  (:Canceled
    (Class|InteractorComponent|InteractionInput (Variables|Default|GetInteractorComponent) "DefaultKey" false :!label _label) ; Game Mode Input 수정시 오류 있음
  )
  (:Completed
    (goto _label)))

(event Input|EnhancedActionEvents|EnhancedInputActionIA_QuestDisplay
  (params (ActionValue :type Boolean) (ElapsedSeconds :type Float%20%28double-precision%29) (TriggeredSeconds :type Float%20%28double-precision%29) (InputAction :type Input%20Action%20Object%20Reference :default "/Game/Input/Actions/IA_QuestDisplay.IA_QuestDisplay"))
  (:Started
    (bind _returnvalue (UserInterface|CreateWidget "/Game/Widgets/QuestWidget/WBP_QuestLog.WBP_QuestLog_C"))
    (UserInterface|Viewport|AddtoViewport _returnvalue 0)))

(event Input|EnhancedActionEvents|EnhancedInputActionIA_Inventory
  (params (ActionValue :type Boolean) (ElapsedSeconds :type Float%20%28double-precision%29) (TriggeredSeconds :type Float%20%28double-precision%29) (InputAction :type Input%20Action%20Object%20Reference :default "/Game/Input/Actions/IA_Inventory.IA_Inventory"))
  (:Started
    (Utilities|IsValid (Variables|/Script/Warriors.WidgetSubSystem|GetHeroInventoryWidget (Subsystems|GetWidgetSubSystem))
      (:Is%20Valid
        (Widget|RemovefromParent (Variables|/Script/Warriors.WidgetSubSystem|GetHeroInventoryWidget (Subsystems|GetWidgetSubSystem)))
        (Class|WidgetSubSystem|SetInventoryWidget (Subsystems|GetWidgetSubSystem)))
      (:Is%20Not%20Valid
        (bind _returnvalue (UserInterface|CreateWidget "/Game/Widgets/InventoryWidget/WBP_Inventory.WBP_Inventory_C"))
        (Class|WidgetSubSystem|SetInventoryWidget (Subsystems|GetWidgetSubSystem) _returnvalue)
        (UserInterface|Viewport|AddtoViewport _returnvalue 0)))))

(event EventBeginPlay
  ;[1 1 1] Quest Save Data Load
  (bind _asbp_warrior_game_instance (Utilities|Casting|CastToBP_WarriorGameInstance (Class|WarriorFunctionLibrary|GetWarriorGameInstance)))
  (Utilities|IsValid _asbp_warrior_game_instance
    (:Is%20Valid
      (Utilities|IsValid (Variables|/Game/Generic/BP_WarriorGameInstance.BP_WarriorGameInstance_C|GetQuestSaveGame _asbp_warrior_game_instance)
        (:Is%20Valid
          (Default|LoadQuests (Variables|/Game/Generic/BP_WarriorGameInstance.BP_WarriorGameInstance_C|GetQuestSaveGame _asbp_warrior_game_instance) (Variables|Default|GetBP_QuestLogComponent)))))))

(event Collision|EventActorBeginOverlap
  (params (OtherActor :type Actor%20Object%20Reference)))

(event EventTick
  (params (DeltaSeconds :type Float%20%28single-precision%29)))

(event Input|KeyboardEvents|2
  (params (Key :type Key%20Structure :default "None"))
  (:Pressed
    (bind _asbp_warrior_game_instance (Utilities|Casting|CastToBP_WarriorGameInstance (Class|WarriorFunctionLibrary|GetWarriorGameInstance)))
    (Utilities|IsValid _asbp_warrior_game_instance
      (:Is%20Valid
        (for _array_element (Variables|/Script/Warriors.QuestLogComponent|GetCurrentQuests (Variables|Default|GetBP_QuestLogComponent))
          (Default|SaveQuestDetails (Variables|/Game/Generic/BP_WarriorGameInstance.BP_WarriorGameInstance_C|GetQuestSaveGame _asbp_warrior_game_instance) _array_element))
        (Default|SaveQuestLog (Variables|/Game/Generic/BP_WarriorGameInstance.BP_WarriorGameInstance_C|GetQuestSaveGame _asbp_warrior_game_instance) (Variables|Default|GetBP_QuestLogComponent))
        (SaveGame|SaveGametoSlot (Variables|/Game/Generic/BP_WarriorGameInstance.BP_WarriorGameInstance_C|GetQuestSaveGame _asbp_warrior_game_instance) "QuestSaveData" 1)))))

(event Input|KeyboardEvents|3
  (params (Key :type Key%20Structure :default "None"))
  (:Pressed
    (bind _asbp_warrior_game_instance (Utilities|Casting|CastToBP_WarriorGameInstance (Class|WarriorFunctionLibrary|GetWarriorGameInstance)))
    (Default|RemoveSaveData _asbp_warrior_game_instance)))

(fn ConstructionScript)