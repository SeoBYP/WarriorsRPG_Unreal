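; Blueprint interface for actors that take part in melee combat.
; Setters toggle the melee hit volume's collision type and the staggering state.
; Getters report melee attacking, spell casting, blocking, parrying, bleeding damage amount and duration, and whether the opponent was disarmed.
; It holds only signatures with empty default returns, so implementing classes supply the behavior.
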(fn SetMeleeVolumeCollisionEnabled
  (params (NewType :type ECollisionEnabled%20Enum :default "NoCollision")))

(fn SetIsStaggering
  (params (IsStaggering :type Boolean)))

(fn GetIsMeleeAttacking
  (return false))

(fn GetIsCastingSpell
  (return false))

(fn GetIsBlocking
  (return false))

(fn GetIsParrying
  (return false))

(fn GetBleedingDamage
  (return 0 0.0))

(fn GetHasDisarmedOpponent
  (return false))