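; Blueprint interface through which other objects read and change a character's stats in the MRPGT RPG framework.
; It exposes getters for health, power and stamina fractions, armour rating, name, visibility, perks, spell effects, character info and initialization state.
; It also declares calls to subtract health, power or stamina, set status, advance weapon skill progress and refresh carried weight and its UI.
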(fn GetHealthasFrac
  (return 0.0))

(fn GetPowerasFrac
  (return 0.0))

(fn GetStaminaasFrac
  (return 0.0))

(fn CharInfo
  (return ""))

(fn UpdateWeightUI)

(fn SubtractHealth
  (params (Hitpoints :type Integer)))

(fn RefreshWeight)

(fn SubtractStamina
  (params (Amount :type Integer)))

(fn SubtractPower
  (params (Amount :type Integer)))

(fn IncreaseProgressOfWeaponSkill
  (params (Skill :type String) (Amount :type Float%20%28double-precision%29)))

(fn GetAllPerks
  (return 0))

(fn IsCharacterInitialized
  (return false))

(fn SetCharStatus
  (params (NewStatus :type CharacterStatusEnum%20Enum :default "NewEnumerator0")))

(fn GetArmourRating
  (return 0))

(fn GetAllSpellEffects
  (return 0))

(fn GetCharVisibility
  (return false))

(fn GetCharName
  (return ""))