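; Blueprint interface that defines the contract for mounts that riders can use.
; It exposes a mounted-state setter and getter, plus queries for alive state, health and stamina fractions.
; Further getters report movement and pose data: speed, look direction, roll, distance from ground and rear amount.
; A mounting point query takes a rider and returns a mount side; the file holds only signatures with default returns.
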(fn SetIsMounted
  (params (NewValue :type Boolean)))

(fn GetIsAlive
  (return false))

(fn GetSpeed
  (return 0.0))

(fn GetLookDirection
  (return 0.0))

(fn GetRoll
  (return 0.0))

(fn GetMountingPointTransform
  (params (Rider :type Actor%20Object%20Reference))
  (return "NewEnumerator0" ""))

(fn GetHealthFraction
  (return 0.0))

(fn GetStaminaFraction
  (return 0.0))

(fn GetIsMounted
  (return false))

(fn GetDistancefromGround
  (return 0.0))

(fn GetRearAmount
  (return 0.0))