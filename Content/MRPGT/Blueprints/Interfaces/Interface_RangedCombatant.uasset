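; Blueprint interface for ranged combatants, declaring the contract for bow-style projectile attacks.
; Action functions cover spawning a projectile in hand, charging, pulling and releasing the bowstring, and firing toward a desired distance.
; State queries report attacking, loading and ready-to-fire status, with a setter for loading.
; Getters expose weapon, enchantment, critical hit and perk damage values plus the current ranged target actor.
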(fn SpawnProjectileinHand)

(fn FireProjectile
  (params (DesiredDistance :type Float%20%28double-precision%29)))

(fn ChargeBow)

(fn PullBowString)

(fn ReleaseBowString)

(fn IsRangedAttacking
  (return false))

(fn GetIsLoadingWeapon
  (return false))

(fn GetWantstoLoadWeapon
  (return false))

(fn GetIsWeaponReadytoFire
  (return false))

(fn SetIsLoadingWeapon
  (params (NewValue :type Boolean)))

(fn GetBaseDamageMultiplier
  (return 0.0))

(fn WasLastHitACriticalHit?
  (return false))

(fn GetPerkCriticalHitDamageMultiplier
  (return 0.0))

(fn GetWeaponDamageAmount
  (return 0.0))

(fn GetWeaponEnchantmentDamageAmount
  (return 0.0))

(fn GetRangedTargetActor
  (return 0))