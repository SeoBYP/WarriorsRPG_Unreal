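; Blueprint interface for general characters in the MRPGT RPG, exposing shared calls for both player and NPC characters without hard casts.
; It declares queries for life, invisibility, crouch, speed, stamina drain, hostility and interaction or dialogue state.
; It also declares commands for horse mounting and dismounting, camera and view modes, movement input, attack queueing, follower targets, and damage or kill notifications.
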(fn IsAlive
  (return false))

(fn IsInvisible
  (return false))

(fn SuccessfullyCausedDamagetoNPC
  (params (Amount :type Integer) (DamageType :type DamageTypeEnum%20Enum :default "NewEnumerator2")))

(fn GetActorTargettedbyNPC
  (return 0))

(fn CanMountHorses
  (return false))

(fn SetIsMounted
  (params (NewIsMounted :type Boolean)))

(fn MoveTowardsMount
  (params (Mount :type Actor%20Object%20Reference) (MountSide :type MountSideEnum%20Enum :default "NewEnumerator0") (MountPointTransform :type Transform) (Teleport :type Boolean)))

(fn IsNearMountingLocation
  (return false))

(fn Dismount
  (params (DismountPointTransform :type Transform)))

(fn ActivateCamera
  (params (NewViewMode :type ViewModeEnum%20Enum :default "NewEnumerator0")))

(fn GetIsUsingAMount
  (return false))

(fn SetIsHavingDialogue
  (params (NewValue :type Boolean)))

(fn GetIsHavingDialogue
  (return false))

(fn WantstoKillPlayer
  (return false))

(fn SetMouseSensitivity
  (params (NewValue :type Float%20%28double-precision%29)))

(fn ActivateMountingCamera
  (params (PointOfView :type Transform)))

(fn SetFollowersNewTarget
  (params (AttackTarget :type Actor%20Object%20Reference) (FollowerTypes :type Array%20of%20FollowerTypeEnum%20Enums :default "NewEnumerator0")))

(fn DeathCaused
  (params (Victim :type Actor%20Object%20Reference)))

(fn GetIsMounted
  (return false))

(fn GetCharacterSpeed
  (return 0.0))

(fn DoesRunningCauseLossOfStamina
  (return false))

(fn DoesSprintingCauseLossOfStamina
  (return false))

(fn UpdateMaxSpeed)

(fn IsCharCrouched
  (return false))

(fn IsthePlayerCharacter
  (return false))

(fn SetIsInteractingwithObject
  (params (NewValue :type Boolean)))

(fn GetIsInteractingwithObject
  (return false))

(fn GetActiveCamera
  (return 0))

(fn DisableMovementInput)

(fn EnableMovementInput)

(fn GetIsMovementInputEnabled
  (return false))

(fn AllowAttackQueueing)

(fn PreventAttackQueuing)

(fn GetBookReadingCamera
  (return 0))

(fn GetViewMode
  (return "NewEnumerator0"))