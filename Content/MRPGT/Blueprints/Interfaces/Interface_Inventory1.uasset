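; Blueprint interface for a player inventory in what appears to be an RPG, with function signatures only.
; It covers adding an item and checking whether the player holds one by item ID.
; It also reports whether a chainmail hood or hoodless chainmail torso is worn.
; Lockpick functions get the count, read or set lockpick health, and destroy a lockpick.
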(fn AddItem
  (params (Item :type Item%20Struct%20Structure))
  (return false))

(fn GetIsWearingChainmailTorsoWithoutHood
  (return false))

(fn GetIsWearingChainmailHood
  (return false))

(fn GetNumLockpicks
  (return 0))

(fn GetLockpickHealth
  (return 0.0))

(fn SetLockpickHealth
  (params (LockpickHealth :type Float%20%28double-precision%29)))

(fn DestroyLockpick)

(fn PlayerHasItembyItemID
  (params (ItemID :type String))
  (return false))