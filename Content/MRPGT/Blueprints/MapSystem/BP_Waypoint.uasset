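; World waypoint actor that marks a location with a minimap icon, compass icon, 3D icon with distance text, and main-map data.
; Construction copies the data table row matching WaypointID into WaypointInfo, which drives appearance and visibility.
; Looping timers create the widgets once the player character exists, then refresh positions, distance, and distance-scaled compass size and alpha.
; Overlaps report follower arrivals or unvisited waypoint entries to the player controller, optionally showing the name.
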(event Custom|CreateIconWidgets
  (bind _waypointinfo (Variables|MRPGT|ReferenceOnly|GetWaypointInfo))
  (bind _waypointinfo_2 (Variables|MRPGT|ReferenceOnly|GetWaypointInfo))
  (bind _waypointinfo_3 (Variables|MRPGT|ReferenceOnly|GetWaypointInfo))
  (bind (_bisvisibleonminimap _bpreventiconleavingminimap) (Utilities|Struct|BreakWaypointStruct _waypointinfo_3))
  (bind (_minimapicontexture _minimapiconsize) (Utilities|Struct|BreakWaypointStruct _waypointinfo))
  (bind (_compassicontexture _compassiconsize) (Utilities|Struct|BreakWaypointStruct _waypointinfo_2))
  ;[1 1 1] At Begin Play, when the PlayerCharacter is available, spawn a minimap icon that represents this actor and add it to the viewport
  (Utilities|IsValid (Game|GetPlayerCharacter 0)
    (:Is%20Valid
      (Utilities|Time|ClearandInvalidateTimerbyHandle (Variables|Default|GetCreateIconTimer))
      (Utilities|FlowControl|Sequence
        (:then_0
          (if _bisvisibleonminimap
            ;;[1 1 1] Create minimap icon
            (bind _returnvalue (UserInterface|CreateWidget "/Game/MRPGT/Blueprints/MapSystem/WBP_Minimap_Icon.WBP_Minimap_Icon_C" 0 _bpreventiconleavingminimap))
            (bind _output_get (Variables|Default|SetMinimapIcon _returnvalue))
            (Default|ChangeIcon _output_get _minimapicontexture)
            (Default|ChangeSize (Variables|Default|GetMinimapIcon) _minimapiconsize)
            (UserInterface|Viewport|AddtoViewport (Variables|Default|GetMinimapIcon) 1)
            (Transformation|AttachComponentToComponent (Variables|Default|GetCalcHelper) (Variables|/Script/Engine.Actor|GetRootComponent (Game|GetPlayerCharacter 0)) "None" "KeepWorld" "KeepWorld" "KeepWorld" false)))
        (:then_1
          (if (.bIsVisibleOnCompass (Utilities|Struct|BreakWaypointStruct (Variables|MRPGT|ReferenceOnly|GetWaypointInfo)))
            ;;[1 1 1] Create compass icon
            (bind _asbp_character (Utilities|Casting|CastToBP_Character (Game|GetPlayerCharacter 0)))
            (Variables|Default|SetPlayerCharacter (Utilities|ResolveSoftReference _asbp_character))
            (bind _returnvalue_2 (UserInterface|CreateWidget "/Game/MRPGT/Blueprints/MapSystem/WBP_Compass_Icon.WBP_Compass_Icon_C"))
            (bind _output_get_2 (Variables|Default|SetCompassIcon _returnvalue_2))
            (Default|ChangeIcon _output_get_2 _compassicontexture)
            (Default|ChangeSize (Variables|Default|GetCompassIcon) _compassiconsize)
            (bind _ashud_minimap (Utilities|Casting|CastToHUD_Minimap (HUD|GetHUD (Game|GetPlayerController 0))))
            (bind _returnvalue_3 (Class|CanvasPanel|AddChildtoCanvas (Variables|/Game/MRPGT/Blueprints/MapSystem/WBP_Compass.WBP_Compass_C|GetCanvasPanel_Inner2 (Variables|/Game/MRPGT/Blueprints/MapSystem/HUD_Minimap.HUD_Minimap_C|GetCompass _ashud_minimap)) (Variables|Default|GetCompassIcon)))
            (Class|CanvasPanelSlot|SetAlignment _returnvalue_3 "(X=0.500000,Y=0.500000)")
            (Class|CanvasPanelSlot|SetAnchors _returnvalue_3 (Utilities|Struct|MakeAnchors "(X=0.500000,Y=0.500000)" "(X=0.500000,Y=0.500000)"))))))))

(event Custom|UpdateIcons
  ;[1 1 1] 60 times per second, update the icon's position on the minimap, distance text in 3D space and compass icon position on the compass
  (Utilities|FlowControl|Sequence
    (:then_0
      (Variables|Default|GetWaypointWidgetIn3DSpace
        (:then
          ;;[1 1 1] Update the 3d space icon's distance text
          (CallFunction|Update3DIconDistance))
        (:else)))
    (:then_1
      (Variables|Default|GetMinimapIcon
        (:then
          ;;[1 1 1] Update minimap icon position
          (CallFunction|UpdateMinimapIconPosition))
        (:else)))
    (:then_2
      (Variables|Default|GetCompassIcon
        (:then
          ;;[1 1 1] Update compass icon position and appearance
          (CallFunction|UpdateCompassIconPosition)
          (CallFunction|UpdateCompassIconAppearance))
        (:else)))))

(event EventBeginPlay
  (Utilities|FlowControl|Sequence
    (:then_0
      ;[1 1 1] Get a reference to PlayerController
      (bind _asbp_in_game_player_controller (Utilities|Casting|CastToBP_InGamePlayerController (Game|GetPlayerController 0)))
      (Variables|Default|SetPlayerController _asbp_in_game_player_controller))
    (:then_1
      ;[1 1 1] This blueprint may have been spawned during runtime. If so then assign the waypoint data to the WaypointInfo variable.
      (if (Utilities|Enum|Equal(Enum) (.ID (Utilities|Struct|BreakWaypointStruct (Variables|MRPGT|ReferenceOnly|GetWaypointInfo))) "Unset")
        (Development|PrintString "Waypoint ID unset" false false)))
    (:then_2
      ;[1 1 1] Initialize appearance of waypoint icon in 3D space
      (if (.bIsVisibleIn3DSpace (Utilities|Struct|BreakWaypointStruct (Variables|MRPGT|ReferenceOnly|GetWaypointInfo)))
        (CallFunction|InitializeIconandTextWidgetin3DSpace)
        (else
          (CallFunction|HideIconandTextWidgetin3DSpace))))
    (:then_3
      ;[1 1 1] At Begin Play, when the PlayerCharacter is available, spawn a minimap icon that represents this actor and add it to the viewport
      (bind _returnvalue (Utilities|Time|SetTimerbyEvent (delegate Custom|CreateIconWidgets) 1.0 true))
      (Variables|Default|SetCreateIconTimer _returnvalue)
      ;[1 1 1] 60 times per second, update the icon's position on the minimap, distance text in 3D space and compass icon position on the compass
      (bind _returnvalue_2 (Utilities|Time|SetTimerbyEvent (delegate Custom|UpdateIcons) 0.015 true))
      (Variables|Default|SetUpdateIconTimer _returnvalue_2))))

(event Collision|EventActorBeginOverlap
  (params (OtherActor :type Actor%20Object%20Reference))
  (bind _returnvalue (Utilities|GetClass OtherActor))
  (if (Utilities|DoesObjectImplementInterface OtherActor "/Game/MRPGT/Blueprints/Interfaces/Interface_Follower.Interface_Follower_C")
    ;[0 0 0] Update any quests related to a follower entering this waypoint
    (bind _npcid (Class|InterfaceFollower|GetNPCID(Message) OtherActor))
    (Class|InterfacePCFollowers|FollowerEnteredWaypoint(Message) (Game|GetPlayerController 0) _npcid (Variables|MRPGT|Customizable|GetWaypointID))
    (else
      ;[0 0 0] If the player character has not visited this waypoint already then send a message to the screen to tell the player that s/he has reached this waypoint
      (if (not (Default|HasVisitedWaypoint (Variables|Default|GetPlayerController) (Utilities|Struct|BreakWaypointStruct (Variables|MRPGT|ReferenceOnly|GetWaypointInfo))))
        (if (Utilities|Struct|BreakWaypointStruct (Variables|MRPGT|ReferenceOnly|GetWaypointInfo))
          (if (or (== _returnvalue "/Game/MRPGT/Blueprints/Characters/BP_Character.BP_Character_C") (== _returnvalue "/Game/MRPGT/Blueprints/Characters/BP_Horse.BP_Horse_C"))
            (Default|SendMessagetoScreen (Variables|/Game/MRPGT/Blueprints/Controllers/BP_InGamePlayerController.BP_InGamePlayerController_C|GetMessagesWidget (Variables|Default|GetPlayerController)) (.Name (Utilities|Struct|BreakWaypointStruct (Variables|MRPGT|ReferenceOnly|GetWaypointInfo))) "NewEnumerator2"))
          (Default|WaypointEntered (Variables|Default|GetPlayerController) (Utilities|Struct|BreakWaypointStruct (Variables|MRPGT|ReferenceOnly|GetWaypointInfo))))))))

(fn ConstructionScript
  (Utilities|FlowControl|Sequence
    (:then_0
      (if (not (Utilities|Enum|Equal(Enum) (Variables|MRPGT|Customizable|GetWaypointID) "Unset"))
        ;[1 1 1] Get waypoint info from the WorldWaypointDataTable according to the value of the WaypointID variable and store the resulting data inside WaypointInfo
        (bind _outrownames (DataTable|GetDataTableRowNames "/Game/MRPGT/Blueprints/DataTables/WorldWaypointsDataTable.WorldWaypointsDataTable"))
        (for _array_element _outrownames
          (if (Utilities|Name|Equal(Name) _array_element (Utilities|String|StringToName (Variables|MRPGT|Customizable|GetWaypointID)))
            (bind _returnvalue (Utilities|GetDataTableRow "/Game/MRPGT/Blueprints/DataTables/WorldWaypointsDataTable.WorldWaypointsDataTable" _array_element)
              (:then
                (Variables|MRPGT|ReferenceOnly|SetWaypointInfo _returnvalue)))))))
    (:then_1
      ;[1 1 1] Set the billboard sprite to be the Icon. For developer assistance only. Hidden in game.
      (Rendering|Components|Sprite|SetSprite (Variables|Default|GetBillboard) (.MInimapIconTexture (Utilities|Struct|BreakWaypointStruct (Variables|MRPGT|ReferenceOnly|GetWaypointInfo))))
      (Transformation|SetWorldScale3D (Variables|Default|GetBox) (Variables|MRPGT|Customizable|GetBoxCollisionScale))
      (Components|Sphere|SetSphereRadius (Variables|Default|GetSphere) (Variables|MRPGT|Customizable|GetCollisionSphereRadius) true))))

(fn UpdateMinimapIconPosition
  (bind _returnvalue (Game|GetPlayerCharacter 0))
  (bind _rootcomponent (Variables|/Script/Engine.Actor|GetRootComponent _returnvalue))
  (bind _returnvalue_2 (Transformation|GetWorldTransform _rootcomponent))
  (Utilities|IsValid (Game|GetPlayerCharacter 0)
    (:Is%20Valid
      (Transformation|SetWorldLocation (Variables|Default|GetCalcHelper) (Transformation|GetActorLocation) false false)
      (Default|UpdateIconLocation (Variables|Default|GetMinimapIcon) (Math|Conversions|ToVector2D(Vector) (Math|Vector|SelectVector (Variables|/Script/Engine.SceneComponent|GetRelativeLocation (Variables|Default|GetCalcHelper)) (Math|Transform|InverseTransformLocation (Math|Transform|MakeTransform (.location _returnvalue_2) "0, 0, 0" (.scale _returnvalue_2)) (Transformation|GetActorLocation)) (Variables|Default|GetbMinimapRotates))) (Math|Float|SelectFloat (.yaw (Transformation|GetActorRotation)) 0.0 (.bIconRotates (Utilities|Struct|BreakWaypointStruct (Variables|MRPGT|ReferenceOnly|GetWaypointInfo))))))))

(fn IsBehind
  (params (Camera :type Vector) (Objective :type Vector))
  (bind _returnvalue (Math|Vector|Normalize Objective))
  (bind _returnvalue_2 (Math|Vector|Normalize Camera))
  (bind _returnvalue_3 (Math|Vector|DotProduct _returnvalue_2 _returnvalue))
  (if (Variables|MRPGT|Customizable|GetDebug)
    (Development|PrintString (Utilities|String|Append "Dot == " (Utilities|String|ToString(Float) _returnvalue_3))))
  (return (< (Class|KismetMathLibrary|DegAcos _returnvalue_3) 1.5e+02)))

(fn UpdateCompassIconAppearance
  (bind _waypointinfo (Variables|MRPGT|ReferenceOnly|GetWaypointInfo))
  (bind _waypointinfo_2 (Variables|MRPGT|ReferenceOnly|GetWaypointInfo))
  (bind (_maxsizemultiplierforcompassicon _actordistancefornormalsizecompassicon _actordistanceformaxsizecompassicon) (Utilities|Struct|BreakWaypointStruct _waypointinfo_2))
  (bind (_minimumcompassiconalpha _maxactordistanceforcompassiconvisibility _actordistanceforopaquecompassicon) (Utilities|Struct|BreakWaypointStruct _waypointinfo))
  (bind _returnvalue (Utilities|LoadAssetBlocking (Variables|Default|GetPlayerCharacter)))
  (bind _asbp_character (Utilities|Casting|CastToBP_Character _returnvalue))
  (LocalVariables|SetLocalDistanceFromPlayerToWaypoint (Math|Vector|Distance(Vector) (Transformation|GetActorLocation) (Transformation|GetWorldLocation (Variables|/Script/Engine.Actor|GetRootComponent _asbp_character))))
  (Default|ChangeSize (Variables|Default|GetCompassIcon) (Math|Conversions|ToVector2D(Vector) (* (.CompassIconSize (Utilities|Struct|BreakWaypointStruct (Variables|MRPGT|ReferenceOnly|GetWaypointInfo))) (Math|Float|MapRangeClamped (LocalVariables|GetLocalDistanceFromPlayerToWaypoint) _actordistancefornormalsizecompassicon _actordistanceformaxsizecompassicon 1.0 _maxsizemultiplierforcompassicon))))
  (Default|ChangeIconAlpha (Variables|Default|GetCompassIcon) (Math|Float|SelectFloat 0.0 (Math|Float|MapRangeClamped (LocalVariables|GetLocalDistanceFromPlayerToWaypoint) _maxactordistanceforcompassiconvisibility _actordistanceforopaquecompassicon _minimumcompassiconalpha 1.0) (> (LocalVariables|GetLocalDistanceFromPlayerToWaypoint) _maxactordistanceforcompassiconvisibility))))

(fn InitializeIconandTextWidgetin3DSpace
  (bind _waypointinfo (Variables|MRPGT|ReferenceOnly|GetWaypointInfo))
  (bind _waypointinfo_2 (Variables|MRPGT|ReferenceOnly|GetWaypointInfo))
  (bind (_minimapicontexture _3diconsize) (Utilities|Struct|BreakWaypointStruct _waypointinfo))
  (bind (_minimapicontexture_2 _bdisplay3dicon _bdisplaydistancetowaypoint) (Utilities|Struct|BreakWaypointStruct _waypointinfo_2))
  (bind _aswbp_waypoint (Utilities|Casting|CastToWBP_Waypoint (UserInterface|GetWidget (Variables|Default|GetIconAndTextWidget))))
  (Variables|Default|SetWaypointWidgetIn3DSpace _aswbp_waypoint)
  (Utilities|FlowControl|Sequence
    (:then_0
      (if _bdisplay3dicon
        (Default|UpdateIcon (Variables|Default|GetWaypointWidgetIn3DSpace) _minimapicontexture _3diconsize)
        (Default|SetIconVisiblity (Variables|Default|GetWaypointWidgetIn3DSpace) "Visible")
        (else
          (Default|SetIconVisiblity (Variables|Default|GetWaypointWidgetIn3DSpace) "Hidden"))))
    (:then_1
      (if _bdisplaydistancetowaypoint
        (Default|SetDistanceVisibility (Variables|Default|GetWaypointWidgetIn3DSpace) "Visible")
        (else
          (Default|SetDistanceVisibility (Variables|Default|GetWaypointWidgetIn3DSpace) "Hidden"))))))

(fn Update3DIconDistance
  (if (.bDisplayDistanceToWaypoint (Utilities|Struct|BreakWaypointStruct (Variables|MRPGT|ReferenceOnly|GetWaypointInfo)))
    (Default|SetText (Variables|Default|GetWaypointWidgetIn3DSpace) (Utilities|Text|FormatText "{Distance}m" (Math|Float|Truncate (/ (Math|Vector|Distance(Vector) (Transformation|GetActorLocation) (Transformation|GetActorLocation (Game|GetPlayerCharacter 0))) 1e+02))))))

(fn GetXPositionOfCompassIcon
  (bind _returnvalue (Utilities|LoadAssetBlocking (Variables|Default|GetPlayerCharacter)))
  (bind _asbp_character (Utilities|Casting|CastToBP_Character _returnvalue))
  (return (* (/ (Math|Vector2D|DotProduct(2D) (Math|Conversions|ToVector2D(Vector) (Math|Vector|GetRightVector (Variables|/Script/Engine.Actor|GetRootComponent _asbp_character))) (Math|Vector2D|Normalize2D (Math|Conversions|ToVector2D(Vector) (Math|Rotator|GetRotationXVector (Math|Rotator|FindLookatRotation (Transformation|GetActorLocation) (Transformation|GetWorldLocation (Variables|/Script/Engine.Actor|GetRootComponent _asbp_character))))))) (Math|Vector2D|DotProduct(2D) (Math|Conversions|ToVector2D(Vector) (Math|Vector|GetForwardVector (Variables|/Script/Engine.Actor|GetRootComponent _asbp_character))) (Math|Vector2D|Normalize2D (Math|Conversions|ToVector2D(Vector) (Math|Rotator|GetRotationXVector (Math|Rotator|FindLookatRotation (Transformation|GetActorLocation) (Transformation|GetWorldLocation (Variables|/Script/Engine.Actor|GetRootComponent _asbp_character)))))))) 4.5e+02) (Math|Vector|GetForwardVector (Variables|/Script/Engine.Actor|GetRootComponent _asbp_character)) (Math|Rotator|GetRotationXVector (Math|Rotator|FindLookatRotation (Transformation|GetActorLocation) (Transformation|GetWorldLocation (Variables|/Script/Engine.Actor|GetRootComponent _asbp_character))))))

(fn UpdateCompassIconPosition
  (bind _compassicon (Variables|Default|GetCompassIcon))
  (bind _returnvalue (Class|WidgetLayoutLibrary|SlotasCanvasSlot _compassicon))
  (bind (_xpos _camera _objective) (CallFunction|GetXPositionOfCompassIcon))
  (if (CallFunction|IsBehind _camera _objective)
    (Class|CanvasPanelSlot|SetPosition _returnvalue (Math|Vector2D|MakeVector2D _xpos -2e+02)) ; Move the image off the screen
    (else
      (Class|CanvasPanelSlot|SetPosition _returnvalue (Math|Vector2D|MakeVector2D _xpos 0.0)))))

(fn HideIconandTextWidgetin3DSpace
  (Widget|SetVisibility (UserInterface|GetWidget (Variables|Default|GetIconAndTextWidget)) "Hidden"))

(fn GetIsVisibleonMainMap
  (return (.bIsVisibleOnMainMap (Utilities|Struct|BreakWaypointStruct (Variables|MRPGT|ReferenceOnly|GetWaypointInfo)))))

(fn GetMapIconData
  (bind _waypointinfo (Variables|MRPGT|ReferenceOnly|GetWaypointInfo))
  (bind (_name _minimapicontexture _minimapiconsize _biconrotates) (Utilities|Struct|BreakWaypointStruct _waypointinfo))
  (return (Transformation|GetActorLocation) _minimapicontexture _minimapiconsize _name (Math|Float|SelectFloat (.yaw (Transformation|GetActorRotation)) 0.0 _biconrotates) self 0.0 0.0 true))

(fn GetWaypointInfo
  (return (Variables|MRPGT|ReferenceOnly|GetWaypointInfo)))