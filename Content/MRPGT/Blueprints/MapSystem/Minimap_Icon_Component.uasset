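; Actor component that shows its owner as configurable minimap and compass icons.
; Creates the widgets once the player character exists; a fast timer, started only for minimap-visible owners, updates both.
; A helper scene component attached to the player yields rotating-map positions, with an unrotated inverse transform for fixed maps.
; Compass icons use dot-product ratios for placement, move off-strip when behind, and scale and fade by distance.
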(event Custom|CreateMinimapIconWidget
  ;[0 0 0] When the player character is available, create map icons
  (Utilities|IsValid (Game|GetPlayerCharacter 0)
    (:Is%20Valid
      (Utilities|Time|ClearandInvalidateTimerbyHandle (Variables|MRPGT|GetCreateMinimapIconTimer))
      (Utilities|FlowControl|Sequence
        (:then_0
          ;[0 0 0] Create the minimap icon for this actor component
          (if (Variables|MRPGT|Customizable|GetbIsVisibleOnMinimap)
            (bind _returnvalue (UserInterface|CreateWidget "/Game/MRPGT/Blueprints/MapSystem/WBP_Minimap_Icon.WBP_Minimap_Icon_C" 0 (Variables|MRPGT|Customizable|GetbPreventIconLeavingMinimap) (Variables|MRPGT|Customizable|GetDebug)))
            (bind _output_get (Variables|MRPGT|SetMinimapIcon _returnvalue))
            (Default|ChangeIcon _output_get (Variables|MRPGT|Customizable|GetMinimapIconTexture))
            (Default|ChangeSize (Variables|MRPGT|GetMinimapIcon) (Variables|MRPGT|Customizable|GetMinimapIconSize))
            (UserInterface|Viewport|AddtoViewport (Variables|MRPGT|GetMinimapIcon) 1)
            (bind _returnvalue_2 (Game|AddComponentbyClass (Components|GetOwner) "/Script/Engine.SceneComponent" false))
            (Variables|Default|SetCalcHelper _returnvalue_2)
            (Transformation|AttachComponentToComponent (Variables|Default|GetCalcHelper) (Variables|/Script/Engine.Actor|GetRootComponent (Game|GetPlayerCharacter 0)) "None" "KeepWorld" "KeepWorld" "KeepWorld" true)
            ;[0 0 0] Update the icon positions 60 times a second
            (Utilities|Time|SetTimerbyEvent (delegate Custom|UpdateIconPositionTimer) 0.015 true)))
        (:then_1
          ;[0 0 0] Create compass icon
          (if (Variables|MRPGT|Customizable|GetbIsVisibleOnCompass)
            (bind _asbp_character (Utilities|Casting|CastToBP_Character (Game|GetPlayerCharacter 0)))
            (Variables|MRPGT|SetPlayerCharacter _asbp_character)
            (bind _returnvalue_3 (UserInterface|CreateWidget "/Game/MRPGT/Blueprints/MapSystem/WBP_Compass_Icon.WBP_Compass_Icon_C"))
            (bind _output_get_2 (Variables|MRPGT|SetCompassIcon _returnvalue_3))
            (Default|ChangeIcon _output_get_2 (Variables|MRPGT|Customizable|GetCompassIconTexture))
            (Default|ChangeSize (Variables|MRPGT|GetCompassIcon) (Variables|MRPGT|Customizable|GetCompassIconSize))
            (bind _ashud_minimap (Utilities|Casting|CastToHUD_Minimap (HUD|GetHUD (Game|GetPlayerController 0))))
            (bind _returnvalue_4 (Class|CanvasPanel|AddChildtoCanvas (Variables|/Game/MRPGT/Blueprints/MapSystem/WBP_Compass.WBP_Compass_C|GetCanvasPanel_Inner2 (Variables|/Game/MRPGT/Blueprints/MapSystem/HUD_Minimap.HUD_Minimap_C|GetCompass _ashud_minimap)) (Variables|MRPGT|GetCompassIcon)))
            (Class|CanvasPanelSlot|SetAlignment _returnvalue_4 "(X=0.500000,Y=0.500000)")
            (Class|CanvasPanelSlot|SetAnchors _returnvalue_4 (Utilities|Struct|MakeAnchors "(X=0.500000,Y=0.500000)" "(X=0.500000,Y=0.500000)"))))))))

(event Custom|UpdateIconPositionTimer
  ;[0 0 0] Update the icon positions 60 times a second
  (Utilities|FlowControl|Sequence
    (:then_0
      ;[0 0 0] Update minimap icon position and appearance
      (Variables|MRPGT|GetMinimapIcon
        (:then
          (if (or (and (Variables|MRPGT|Customizable|GetHideMinimapIconWhenOwnerPossessed) (Variables|MRPGT|GetbOwnerIsPossessed)) (and (Variables|MRPGT|Customizable|GetHideMinimapIconWhenOwnerDead) (Variables|MRPGT|GetbOwnerIsDead)))
            (Widget|SetVisibility (Variables|MRPGT|GetMinimapIcon) "Hidden")
            (else
              (CallFunction|UpdateMinimapIconPosition)
              (Widget|SetVisibility (Variables|MRPGT|GetMinimapIcon) "HitTestInvisible"))))
        (:else)))
    (:then_1
      ;[0 0 0] Update compass icon position and appearance
      (Variables|MRPGT|GetCompassIcon
        (:then
          (if (and (Variables|MRPGT|GetbOwnerIsDead) (Variables|MRPGT|Customizable|GetHideCompassIconWhenOwnerDead))
            (Default|ChangeIconAlpha (Variables|MRPGT|GetCompassIcon) 0.0)
            (else
              (CallFunction|UpdateCompassIconPosition)
              (CallFunction|UpdateCompassIconAppearance))))
        (:else)))))

(event EventBeginPlay
  ;[0 0 0] When the player character is available, create map icons
  (bind _returnvalue (Utilities|Time|SetTimerbyEvent (delegate Custom|CreateMinimapIconWidget) 1.0 true))
  (Variables|MRPGT|SetCreateMinimapIconTimer _returnvalue))

(fn UpdateMinimapIconPosition
  (bind _returnvalue (Game|GetPlayerCharacter 0))
  (bind _returnvalue_2 (Game|GetPlayerCharacter 0))
  (bind _returnvalue_3 (Components|GetOwner))
  (bind _rootcomponent (Variables|/Script/Engine.Actor|GetRootComponent _returnvalue))
  (bind _returnvalue_4 (Transformation|GetWorldTransform _rootcomponent))
  ;[0 0 0] Update the 2D position of the minimap icon relative to the player character icon in the center of the minimap. The CalcHelper is a scene component that is attached to the PlayerCharacter. This provides a relative-to-the-player-character location. If it is desirable for the minimap not to rotate with the player charcter then this cannot be used. Instead, the InverseTransformLocation is used to get a relative location but with the player pointing north/not being rotated at all.
  (Utilities|IsValid (Game|GetPlayerCharacter 0)
    (:Is%20Valid
      (bind _calchelper (Variables|Default|GetCalcHelper)
        (:then
          (Transformation|SetWorldLocationAndRotation _calchelper (Transformation|GetActorLocation _returnvalue_3) (Transformation|GetActorRotation _returnvalue_3) false false)
          (Default|UpdateIconLocation (Variables|MRPGT|GetMinimapIcon) (Math|Conversions|ToVector2D(Vector) (Math|Vector|SelectVector (Variables|/Script/Engine.SceneComponent|GetRelativeLocation (Variables|Default|GetCalcHelper)) (Math|Transform|InverseTransformLocation (Math|Transform|MakeTransform (.location _returnvalue_4) "0, 0, 0" (.scale _returnvalue_4)) (Transformation|GetActorLocation (Components|GetOwner))) (Variables|MRPGT|Customizable|GetbMinimapRotates))) (Math|Float|SelectFloat (Math|Float|SelectFloat (.yaw (Transformation|GetActorRotation _returnvalue_2)) (Math|Float|SelectFloat (.yaw (Variables|/Script/Engine.SceneComponent|GetRelativeRotation (Variables|Default|GetCalcHelper))) (.yaw (Transformation|GetActorRotation (Components|GetOwner))) (Variables|MRPGT|Customizable|GetbMinimapRotates)) (== (Components|GetOwner) _returnvalue_2)) 0.0 (Variables|MRPGT|Customizable|GetbIconRotates))))
        (:else)))))

(fn UpdateCompassIconAppearance
  (LocalVariables|SetLocalDistanceFromPlayerToWaypoint (Math|Vector|Distance(Vector) (Transformation|GetActorLocation (Components|GetOwner)) (Transformation|GetWorldLocation (Variables|/Script/Engine.Actor|GetRootComponent (Variables|MRPGT|GetPlayerCharacter)))))
  (Default|ChangeSize (Variables|MRPGT|GetCompassIcon) (Math|Conversions|ToVector2D(Vector) (* (Variables|MRPGT|Customizable|GetCompassIconSize) (Math|Float|MapRangeClamped (LocalVariables|GetLocalDistanceFromPlayerToWaypoint) (Variables|MRPGT|Customizable|GetActorDistanceForNormalSizeCompassIcon) (Variables|MRPGT|Customizable|GetActorDistanceForMaxSizeCompassIcon) 1.0 (Variables|MRPGT|Customizable|GetMaxSizeMultiplierForCompassIcon)))))
  (Default|ChangeIconAlpha (Variables|MRPGT|GetCompassIcon) (Math|Float|SelectFloat 0.0 (Math|Float|MapRangeClamped (LocalVariables|GetLocalDistanceFromPlayerToWaypoint) (Variables|MRPGT|Customizable|GetMaxActorDistanceForCompassIconVisibility) (Variables|MRPGT|Customizable|GetActorDistanceForOpaqueCompassIcon) (Variables|MRPGT|Customizable|GetMinimumCompassIconAlpha) 1.0) (> (LocalVariables|GetLocalDistanceFromPlayerToWaypoint) (Variables|MRPGT|Customizable|GetMaxActorDistanceForCompassIconVisibility)))))

(fn UpdateCompassIconPosition
  (bind _compassicon (Variables|MRPGT|GetCompassIcon))
  (bind _returnvalue (Class|WidgetLayoutLibrary|SlotasCanvasSlot _compassicon))
  (bind (_xpos _camera _objective) (CallFunction|GetXPositionOfCompassIcon))
  (if (CallFunction|IsBehind _camera _objective)
    (Class|CanvasPanelSlot|SetPosition _returnvalue (Math|Vector2D|MakeVector2D _xpos -2e+02)) ; Move the image off the screen
    (else
      (Class|CanvasPanelSlot|SetPosition _returnvalue (Math|Vector2D|MakeVector2D _xpos 0.0)))))

(fn GetXPositionOfCompassIcon
  (bind _returnvalue (Components|GetOwner))
  (bind _playercharacter (Variables|MRPGT|GetPlayerCharacter))
  (bind _returnvalue_2 (Transformation|GetActorLocation _returnvalue))
  (bind _rootcomponent (Variables|/Script/Engine.Actor|GetRootComponent _playercharacter))
  (bind _rootcomponent_2 (Variables|/Script/Engine.Actor|GetRootComponent _playercharacter))
  (bind _returnvalue_3 (Transformation|GetWorldLocation _rootcomponent_2))
  (bind _returnvalue_4 (Math|Vector|GetForwardVector _rootcomponent))
  (bind _returnvalue_5 (Math|Rotator|FindLookatRotation _returnvalue_2 _returnvalue_3))
  (bind _returnvalue_6 (Math|Rotator|GetRotationXVector _returnvalue_5))
  (bind _returnvalue_7 (Math|Conversions|ToVector2D(Vector) _returnvalue_6))
  (bind _returnvalue_8 (Math|Vector2D|Normalize2D _returnvalue_7))
  (return (* (/ (Math|Vector2D|DotProduct(2D) (Math|Conversions|ToVector2D(Vector) (Math|Vector|GetRightVector (Variables|/Script/Engine.Actor|GetRootComponent _playercharacter))) _returnvalue_8) (Math|Vector2D|DotProduct(2D) (Math|Conversions|ToVector2D(Vector) _returnvalue_4) _returnvalue_8)) 4.5e+02) _returnvalue_4 _returnvalue_6))

(fn IsBehind
  (params (Camera :type Vector) (Objective :type Vector))
  (bind _returnvalue (Math|Vector|Normalize Objective))
  (bind _returnvalue_2 (Math|Vector|Normalize Camera))
  (bind _returnvalue_3 (Math|Vector|DotProduct _returnvalue_2 _returnvalue))
  (if (Variables|MRPGT|Customizable|GetDebug)
    (Development|PrintString (Utilities|String|Append "Dot == " (Utilities|String|ToString(Float) _returnvalue_3)) false false))
  (return (< (Class|KismetMathLibrary|DegAcos _returnvalue_3) 1.5e+02)))