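; SG_GameOptions is the save game object that holds the player's game options in a GameOptions struct.
; Setters update the item and spell UI column configurations, while UpdateInputMappings stores the Input Mapping Contexts from a Player Mappable Input Config after key rebinds.
; CopyInputConfigurationToPMIC, called by BP_MRPGT_GameInstance when loading options, writes saved key mappings back into the live contexts, matching them by array index.
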(fn UpdateItemsColumnConfig
  (params (ItemUIColumnConfiguration :type Array%20of%20Items%20Column%20Configuration%20Struct%20Structures))
  (bind _structout (Utilities|Struct|SetmembersinGameOptionsStruct (Variables|MRPGT|GetGameOptions) ItemUIColumnConfiguration))
  (Variables|MRPGT|SetGameOptions _structout))

(fn UpdateSpellsColumnConfig
  (params (SpellUIColumnConfiguration :type Array%20of%20Spells%20Column%20Configuration%20Struct%20Structures))
  (bind _structout (Utilities|Struct|SetmembersinGameOptionsStruct (Variables|MRPGT|GetGameOptions) SpellUIColumnConfiguration))
  (Variables|MRPGT|SetGameOptions _structout))

(fn UpdateInputMappings
  (params (PlayerMappableInputConfig :type Player%20Mappable%20Input%20Config%20Object%20Reference))
  ;[0 0 0] Copies all of the Input Mapping Contexts from our PMIC to this GameOptions save game object. Called after user assigns a new key to an input action. Then the game options can be saved to disk.
  (bind _keys (Utilities|Map|Keys (Class|PlayerMappableInputConfig|GetMappingContexts PlayerMappableInputConfig)))
  (for _array_element _keys
    (Utilities|Array|Add (LocalVariables|GetLocalInputMappingContexts) _array_element)
    (for _array_element_2 (Variables|/Script/EnhancedInput.InputMappingContext|GetMappings _array_element)
      (Utilities|IsValid (Class|EnhancedInputLibrary|GetPlayerMappableKeySettings _array_element_2)
        (:Is%20Valid
          (Development|PrintString 0 (Utilities|String|Append "[Update Input Mappings] Updated IMC " (Utilities|GetDisplayName _array_element) ", Input Mapping Name == " (Utilities|String|ToString(Name) (Variables|/Script/EnhancedInput.PlayerMappableKeySettings|GetName (Class|EnhancedInputLibrary|GetPlayerMappableKeySettings _array_element_2))) ", Key == " (Utilities|String|ToString(Text) (Class|KismetInputLibrary|KeyGetDisplayName (.Key (Utilities|Struct|BreakEnhancedActionKeyMapping _array_element_2)) true))) false)))))
  (bind _structout (Utilities|Struct|SetmembersinGameOptionsStruct (Variables|MRPGT|GetGameOptions) (LocalVariables|GetLocalInputMappingContexts)))
  (Variables|MRPGT|SetGameOptions _structout))

(fn CopyInputConfigurationtoPMIC
  (params (PlayerMappableInputConfig :type Player%20Mappable%20Input%20Config%20Object%20Reference))
  ;[0 0 0] Apply the loaded input configuration from the game options file to the game. Assign the input configuration that has been loaded into the GameOptions variable, to the IMCs within the passed in PMIC. Called by the LoadOptions custom event in BP_MRPGT_GameInstance at EventInit.
  (bind _keys (Utilities|Map|Keys (Class|PlayerMappableInputConfig|GetMappingContexts PlayerMappableInputConfig)))
  (for (_array_element _array_index) _keys ; ForEach IMC
    (for (_ _array_index_2) (Variables|/Script/EnhancedInput.InputMappingContext|GetMappings _array_element) ; ForEach Enhanced Key Mapping within the IMC
      (Utilities|Array|SetArrayElem (Variables|/Script/EnhancedInput.InputMappingContext|GetMappings _array_element) _array_index_2 (Utilities|Array|Get(acopy) (Variables|/Script/EnhancedInput.InputMappingContext|GetMappings (Utilities|Array|Get(acopy) (Utilities|Struct|BreakGameOptionsStruct (Variables|MRPGT|GetGameOptions)) _array_index)) _array_index_2)) ; Update the Enhanced Input Mapping within the IMC with the one from the save.
      (Utilities|IsValid (Class|EnhancedInputLibrary|GetPlayerMappableKeySettings (Utilities|Array|Get(acopy) (Variables|/Script/EnhancedInput.InputMappingContext|GetMappings (Utilities|Array|Get(acopy) (Utilities|Struct|BreakGameOptionsStruct (Variables|MRPGT|GetGameOptions)) _array_index)) _array_index_2))
        (:Is%20Valid
          (Development|PrintString 0 (Utilities|String|Append "[Copy Input Configuration To PMIC] Loaded IMC " (Utilities|GetDisplayName _array_element) ", Input Mapping Name == " (Utilities|String|ToString(Name) (Variables|/Script/EnhancedInput.PlayerMappableKeySettings|GetName (Class|EnhancedInputLibrary|GetPlayerMappableKeySettings (Utilities|Array|Get(acopy) (Variables|/Script/EnhancedInput.InputMappingContext|GetMappings (Utilities|Array|Get(acopy) (Utilities|Struct|BreakGameOptionsStruct (Variables|MRPGT|GetGameOptions)) _array_index)) _array_index_2)))) ", Key == " (Utilities|String|ToString(Text) (Class|KismetInputLibrary|KeyGetDisplayName (.Key (Utilities|Struct|BreakEnhancedActionKeyMapping (Utilities|Array|Get(acopy) (Variables|/Script/EnhancedInput.InputMappingContext|GetMappings (Utilities|Array|Get(acopy) (Utilities|Struct|BreakGameOptionsStruct (Variables|MRPGT|GetGameOptions)) _array_index)) _array_index_2))) true))) false false))))))