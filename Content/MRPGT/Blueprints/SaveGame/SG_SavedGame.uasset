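; SaveGame object for the RPG that holds the whole saved state in one SavedGame struct: level, character data, quests, perks, followers, waypoints and world changes.
; Setter functions overwrite individual struct members, and getters return some of them.
; Changed containers are upserted by UniqueActorID, while dropped items and interacted actor IDs are tracked in arrays.
; Followers are saved as the NPCInfo struct taken from each NPC actor.
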(fn UpdateLevel
  (params (Level :type Name))
  (bind _structout (Utilities|Struct|SetmembersinSavedGameStruct (Variables|MRPGT|GetSavedGame) Level))
  (Variables|MRPGT|SetSavedGame _structout))

(fn UpdateCharacterInfo
  (params (CharInfo :type Character%20Struct%20Structure))
  (bind _structout (Utilities|Struct|SetmembersinSavedGameStruct (Variables|MRPGT|GetSavedGame) CharInfo))
  (Variables|MRPGT|SetSavedGame _structout))

(fn UpdateCharacterTransform
  (params (Transform :type Transform))
  (bind _structout (Utilities|Struct|SetmembersinSavedGameStruct (Variables|MRPGT|GetSavedGame) Transform))
  (Variables|MRPGT|SetSavedGame _structout))

(fn UpdateCharacterItems
  (params (Items :type Array%20of%20Item%20Struct%20Structures))
  (bind _structout (Utilities|Struct|SetmembersinSavedGameStruct (Variables|MRPGT|GetSavedGame) Items))
  (Variables|MRPGT|SetSavedGame _structout))

(fn UpdateCharacterSpells
  (params (Spells :type Array%20of%20Spell%20Struct%20Structures))
  (bind _structout (Utilities|Struct|SetmembersinSavedGameStruct (Variables|MRPGT|GetSavedGame) Spells))
  (Variables|MRPGT|SetSavedGame _structout))

(fn UpdateCharacterQuests
  (params (Quests :type Array%20of%20Quest%20Struct%20Structures))
  (bind _structout (Utilities|Struct|SetmembersinSavedGameStruct (Variables|MRPGT|GetSavedGame) Quests))
  (Variables|MRPGT|SetSavedGame _structout))

(fn UpdateCharacterQuestObjectives
  (params (QuestObjectives :type Array%20of%20Quest%20Objective%20Struct%20Structures))
  (bind _structout (Utilities|Struct|SetmembersinSavedGameStruct (Variables|MRPGT|GetSavedGame) QuestObjectives))
  (Variables|MRPGT|SetSavedGame _structout))

(fn UpdateCharacterSkills
  (params (Skills :type Array%20of%20Skill%20Struct%20Structures))
  (bind _structout (Utilities|Struct|SetmembersinSavedGameStruct (Variables|MRPGT|GetSavedGame) Skills))
  (Variables|MRPGT|SetSavedGame _structout))

(fn UpdateCharacterSpellEffects
  (params (SpellEffects :type Array%20of%20Spell%20Effect%20Struct%20Structures))
  (bind _structout (Utilities|Struct|SetmembersinSavedGameStruct (Variables|MRPGT|GetSavedGame) SpellEffects))
  (Variables|MRPGT|SetSavedGame _structout))

(fn UpdateChangedContainer
  (params (ChangedContainer :type Changed%20Container%20Struct%20Structure))
  (bind (_array_element _array_index) (Utilities|Array|ForEachLoopwithBreak (.ChangedContainers (Utilities|Struct|BreakSavedGameStruct (Variables|MRPGT|GetSavedGame))) :!label _label)
    (:LoopBody
      (LocalVariables|SetLocalArrayIndex _array_index)
      (if (Utilities|Enum|Equal(Enum) (.UniqueActorID (Utilities|Struct|BreakChangedContainerStruct _array_element)) (.UniqueActorID (Utilities|Struct|BreakChangedContainerStruct ChangedContainer)))
        (LocalVariables|SetFoundChangedContainer true)
        (goto _label Break)))
    (:Completed
      (if (LocalVariables|GetFoundChangedContainer)
        (Utilities|Array|SetArrayElem (.ChangedContainers (Utilities|Struct|BreakSavedGameStruct (Variables|MRPGT|GetSavedGame))) (LocalVariables|GetLocalArrayIndex) ChangedContainer)
        (else
          (Utilities|Array|Add (.ChangedContainers (Utilities|Struct|BreakSavedGameStruct (Variables|MRPGT|GetSavedGame))) ChangedContainer))))))

(fn UpdateWorldItems
  (params (Items :type Array%20of%20Item%20Struct%20Structures))
  (bind _structout (Utilities|Struct|SetmembersinSavedGameStruct (Variables|MRPGT|GetSavedGame) Items))
  (Variables|MRPGT|SetSavedGame _structout))

(fn AddInteractedActorID
  (params (ID :type String))
  (Utilities|Array|AddUnique (.InteractedActorIDs (Utilities|Struct|BreakSavedGameStruct (Variables|MRPGT|GetSavedGame))) ID))

(fn RemoveDroppedItem
  (params (DroppedItemNowPickedUp :type Dropped%20Item%20Struct%20Structure))
  (bind (_array_element _array_index) (Utilities|Array|ForEachLoopwithBreak (.DroppedItems (Utilities|Struct|BreakSavedGameStruct (Variables|MRPGT|GetSavedGame))) :!label _label)
    (:LoopBody
      (LocalVariables|SetLocalArrayIndex _array_index)
      (if (Utilities|Enum|Equal(Enum) (.ItemID (Utilities|Struct|BreakDroppedItemStruct _array_element)) (.ItemID (Utilities|Struct|BreakDroppedItemStruct DroppedItemNowPickedUp)))
        (LocalVariables|SetFoundDroppedItem true)
        (goto _label Break)))
    (:Completed
      (if (LocalVariables|GetFoundDroppedItem)
        (Utilities|Array|RemoveIndex (.DroppedItems (Utilities|Struct|BreakSavedGameStruct (Variables|MRPGT|GetSavedGame))) (LocalVariables|GetLocalArrayIndex))))))

(fn AddDroppedItem
  (params (UniqueID :type String) (ItemID :type String) (Transform :type Transform))
  (Utilities|Array|AddUnique (.DroppedItems (Utilities|Struct|BreakSavedGameStruct (Variables|MRPGT|GetSavedGame))) (Utilities|Struct|MakeDroppedItemStruct UniqueID ItemID Transform)))

(fn GetCharacterInfo
  (return (.characterinfo (Variables|MRPGT|GetSavedGame))))

(fn GetItems
  (return (.charactersitems (Variables|MRPGT|GetSavedGame))))

(fn GetSpells
  (return (.charactersknownspells (Variables|MRPGT|GetSavedGame))))

(fn GetSkills
  (return (.charactersskills (Variables|MRPGT|GetSavedGame))))

(fn GetTransform
  (return (.charactertransform (Variables|MRPGT|GetSavedGame))))

(fn GetQuests
  (return (.charactersquests (Variables|MRPGT|GetSavedGame))))

(fn GetQuestObjectives
  (return (.charactersquestobjectives (Variables|MRPGT|GetSavedGame))))

(fn GetSpellEffects
  (return (.charactersspelleffects (Variables|MRPGT|GetSavedGame))))

(fn UpdateSaveGameID
  (params (NewID :type String))
  (bind _structout (Utilities|Struct|SetmembersinSavedGameStruct (Variables|MRPGT|GetSavedGame) NewID))
  (Variables|MRPGT|SetSavedGame _structout))

(fn AddChangedContainer
  (params (UniqueActorID :type String) (Items :type Array%20of%20Item%20Struct%20Structures))
  (bind _changedcontainerstruct (Utilities|Struct|MakeChangedContainerStruct UniqueActorID Items))
  (for (_array_element _array_index) (.ChangedContainers (Utilities|Struct|BreakSavedGameStruct (Variables|MRPGT|GetSavedGame)))
    (LocalVariables|SetLocalIndex _array_index)
    (if (Utilities|Enum|Equal(Enum) (.UniqueActorID (Utilities|Struct|BreakChangedContainerStruct _array_element)) UniqueActorID)
      (LocalVariables|SetContainerExistsInArrayAlready true)
      (LocalVariables|SetIndexWhereExists (LocalVariables|GetLocalIndex))))
  (if (LocalVariables|GetContainerExistsInArrayAlready)
    (Utilities|Array|SetArrayElem (.ChangedContainers (Utilities|Struct|BreakSavedGameStruct (Variables|MRPGT|GetSavedGame))) (LocalVariables|GetIndexWhereExists) _changedcontainerstruct)
    (Development|PrintString self (Utilities|String|Append "[AddChangedContainer] Container already added to ChangedContainers array in SaveGame. Updated existing element at array index " (Utilities|String|ToString(Integer) (LocalVariables|GetIndexWhereExists)) ", UniqueActorID = " UniqueActorID) false (LocalVariables|GetLocalDebugThisFunction))
    (else
      (Utilities|Array|Add (.ChangedContainers (Utilities|Struct|BreakSavedGameStruct (Variables|MRPGT|GetSavedGame))) _changedcontainerstruct)
      (Development|PrintString self (Utilities|String|Append "[AddChangedContainer] Container does not exist in ChangedContainers array in SaveGame. Added new array element. UniqueActorID = " UniqueActorID) false (LocalVariables|GetLocalDebugThisFunction)))))

(fn GetContainersItems
  (params (UniqueActorID :type String))
  (for _array_element (.changedcontainers (Variables|MRPGT|GetSavedGame))
    (if (Utilities|Enum|Equal(Enum) UniqueActorID (.UniqueActorID (Utilities|Struct|BreakChangedContainerStruct _array_element)))
      (return (.Items (Utilities|Struct|BreakChangedContainerStruct _array_element))))))

(fn IsDroppedIteminSaveGame
  (params (UniqueID :type String))
  (for _array_element (.DroppedItems (Utilities|Struct|BreakSavedGameStruct (Variables|MRPGT|GetSavedGame)))
    (if (Utilities|Enum|Equal(Enum) (.UniqueID (Utilities|Struct|BreakDroppedItemStruct _array_element)) UniqueID)
      (return true)))
  (return false))

(fn UpdateDroppedItemSavedTransform
  (params (UniqueID :type String) (Transform :type Transform))
  (bind _savedgame (Variables|MRPGT|GetSavedGame))
  (bind _droppeditems (Utilities|Struct|BreakSavedGameStruct _savedgame))
  (for (_array_element _array_index) _droppeditems
    (if (Utilities|Enum|Equal(Enum) (.UniqueID (Utilities|Struct|BreakDroppedItemStruct _array_element)) UniqueID)
      (bind _structout (Utilities|Struct|SetmembersinDroppedItemStruct _array_element Transform))
      (Utilities|Array|SetArrayElem _droppeditems _array_index _structout)
      (Development|PrintString 0 (Utilities|String|Append "[UpdateDroppedItemSavesTransform] Saved transform " (Utilities|String|ToString(Transform) (.Transform (Utilities|Struct|BreakDroppedItemStruct _structout))) " for item with UniqueID " (.UniqueID (Utilities|Struct|BreakDroppedItemStruct _structout)) " and ItemID " (.ItemID (Utilities|Struct|BreakDroppedItemStruct _structout))) false true "(R=0.000000,G=0.660000,B=1.000000,A=1.000000)" 1e+01))))

(fn UpdateCharactersPerks
  (params (CharactersPerks :type Array%20of%20Characters%20Perk%20Struct%20Structures))
  (bind _structout (Utilities|Struct|SetmembersinSavedGameStruct (Variables|MRPGT|GetSavedGame) CharactersPerks))
  (Variables|MRPGT|SetSavedGame _structout))

(fn UpdateFollowerInfo
  (params (Followers :type Array%20of%20Actor%20Object%20References))
  ;[1 1 1] Get the NPC info from each follower actor object and store it in a temporary NPCStruct array then store the array within the SaveGame struct. Everything we need to save regarding followers is inside the NPCInfo variable. When we load a game we'll spawn the NPC and then assign the saved NPCInfo to it
  (for _array_element Followers
    (bind _asbp_npc_master (Utilities|Casting|CastToBP_NPC_Master _array_element))
    (Utilities|Array|Add (LocalVariables|GetLocalNPCs) (Variables|/Game/MRPGT/Blueprints/NPCs/BP_NPC_Master.BP_NPC_Master_C|GetNPCInfo _asbp_npc_master)))
  (bind _structout (Utilities|Struct|SetmembersinSavedGameStruct (Variables|MRPGT|GetSavedGame) (LocalVariables|GetLocalNPCs)))
  (Variables|MRPGT|SetSavedGame _structout))

(fn UpdateVisitedWaypoints
  (params (VisitedWaypoints :type Array%20of%20Strings))
  (bind _structout (Utilities|Struct|SetmembersinSavedGameStruct (Variables|MRPGT|GetSavedGame) VisitedWaypoints))
  (Variables|MRPGT|SetSavedGame _structout))

(fn GetVisitedWaypoints
  (return (Utilities|Struct|BreakSavedGameStruct (Variables|MRPGT|GetSavedGame))))