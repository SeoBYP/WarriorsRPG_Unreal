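; BP_Trap is a one-shot trap that deals piercing damage to an overlapping BP_Character, with a screen message and sound.
; Triggering swaps it to the closed mesh, disables it and records its construction-generated GUID in the saved game.
; An event bound through the player controller restores the triggered state from that save.
; It also offers a timed emissive outline and damage-causer query functions such as CausesKnockback.
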(event Custom|EnableOutline
  (Rendering|Material|SetScalarParameterValueonMaterials (Variables|Default|GetStaticMesh) "EmissiveSpellEffectEnabled" 1.0)
  (Utilities|Time|SetTimerbyEvent (delegate Custom|CustomEvent_0) 3.0))

(event Custom|DisableOutline
  (Rendering|Material|SetScalarParameterValueonMaterials (Variables|Default|GetStaticMesh) "EmissiveSpellEffectEnabled" 0.0))

(event Custom|CustomEvent_0
  (CallFunction|DisableOutline))

(event Custom|CustomEvent_2
  (CallFunction|CheckifStateChanged))

(event EventBeginPlay
  (CallFunction|InitializeReferences)
  (EventDispatchers|BindEventtoInitializeTraps (Variables|MRPGT|ReferenceOnly|GetInGamePlayerController) (delegate Custom|CustomEvent_2)))

(event Collision|EventActorBeginOverlap
  (params (OtherActor :type Actor%20Object%20Reference))
  (if (Variables|MRPGT|ReferenceOnly|GetIsTrapTriggerable?)
    ;[1 1 1] Send a message to the screen to tell the player that s/he has entered this trap
    (bind _asbp_character (Utilities|Casting|CastToBP_Character OtherActor))
    (Default|SendMessagetoScreen (Variables|/Game/MRPGT/Blueprints/Controllers/BP_InGamePlayerController.BP_InGamePlayerController_C|GetMessagesWidget (Variables|MRPGT|ReferenceOnly|GetInGamePlayerController)) "Trap Triggered!" "NewEnumerator0")
    (Game|Damage|ApplyDamage _asbp_character (Variables|MRPGT|Customizable|GetTrapDamage) 0 self "/Game/MRPGT/Blueprints/DamageTypes/DT_Piercing.DT_Piercing_C")
    (Audio|PlaySoundatLocation (Variables|MRPGT|Customizable|GetTriggeredSoundEffect) (Transformation|GetWorldLocation (Variables|Default|GetStaticMesh)) "0, 0, 0" 1.0 1.0 0.0 0 0 0 0)
    (CallFunction|ChangeState)))

(event EventTick
  (params (DeltaSeconds :type Float%20%28single-precision%29)))

(event EventChangeState
  ;[1 1 1] When the trap is triggered we save this state so that if the game is saved and loaded later on then the trap remains triggered
  (Components|StaticMesh|SetStaticMesh (Variables|Default|GetStaticMesh) (Variables|MRPGT|Customizable|GetTrapClosedStaticMesh))
  (Variables|MRPGT|ReferenceOnly|SetIsTrapTriggerable? false)
  (Default|AddInteractedActorID (Variables|/Game/MRPGT/Blueprints/GameInstance/BP_MRPGT_GameInstance.BP_MRPGT_GameInstance_C|GetSavedGame (Variables|MRPGT|ReferenceOnly|GetGameInstance)) (Variables|MRPGT|ReferenceOnly|GetUniqueID)))

(fn ConstructionScript
  (CallFunction|GenerateUniqueID false))

(fn CheckifStateChanged
  (if (Default|GetSavedInteractableActorState (Variables|MRPGT|ReferenceOnly|GetGameInstance) (Variables|MRPGT|ReferenceOnly|GetUniqueID))
    (CallFunction|ChangeState)))

(fn InitializeReferences
  ;[1 1 1] Get a reference to the GameInstance and PlayerController
  (Utilities|FlowControl|Sequence
    (:then_0
      (bind _asbp_mrpgt_game_instance (Utilities|Casting|CastToBP_MRPGT_GameInstance (Game|GetGameInstance)))
      (Variables|MRPGT|ReferenceOnly|SetGameInstance _asbp_mrpgt_game_instance))
    (:then_1
      (bind _asbp_in_game_player_controller (Utilities|Casting|CastToBP_InGamePlayerController (Game|GetPlayerController 0)))
      (Variables|MRPGT|ReferenceOnly|SetInGamePlayerController _asbp_in_game_player_controller))))

(fn GenerateUniqueID
  (params (ForceGeneration :type Boolean))
  ;[0.25 0.25 0.25] Generate a unique ID for the SaveGames
  (if (or (Utilities|Array|IsEmpty (Variables|MRPGT|ReferenceOnly|GetUniqueID)) ForceGeneration)
    (Variables|MRPGT|ReferenceOnly|SetUniqueID (Guid|ToString(Guid) (Guid|NewGuid)))))

(fn CausesKnockback
  (return (Variables|MRPGT|Customizable|GetCausesKnockbackWhenTriggered)))

(fn GetID
  (return ""))

(fn GetLauncherActor
  (return 0))

(fn GetObjectName
  (return ""))

(fn IsProjectile
  (return false))