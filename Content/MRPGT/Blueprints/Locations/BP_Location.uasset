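; BP_Location is a trigger volume marking a named world location, with its collision box scaled in the construction script.
; When the character or horse overlaps it, it optionally shows the location name through the player controller's message widget.
; It then reports the location ID to the player controller as an entered waypoint so related quest objectives can update.
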(event EventBeginPlay
  ;[1 1 1] Get a reference to PlayerController
  (bind _asbp_in_game_player_controller (Utilities|Casting|CastToBP_InGamePlayerController (Game|GetPlayerController 0)))
  (Variables|MRPGT|ReferenceOnly|SetPlayerControllerReference _asbp_in_game_player_controller))

(event Collision|EventActorBeginOverlap
  (params (OtherActor :type Actor%20Object%20Reference))
  (bind _locationinfo (Variables|MRPGT|Customizable|GetLocationInfo))
  (bind (_id _name _displayonscreenwhenenter_) (Utilities|Struct|BreakLocationStruct _locationinfo))
  ;[0 0 0] Send a message to the screen to tell the player that s/he has entered this location
  (Utilities|Casting|CastToBP_Character OtherActor
    (:then
      _)
    (:CastFailed
      (Utilities|Casting|CastToBP_Horse OtherActor)))
  (if _displayonscreenwhenenter_
    (Default|SendMessagetoScreen (Variables|/Game/MRPGT/Blueprints/Controllers/BP_InGamePlayerController.BP_InGamePlayerController_C|GetMessagesWidget (Variables|MRPGT|ReferenceOnly|GetPlayerControllerReference)) (Utilities|Text|ToText(String) _name) "NewEnumerator2"))
  ;[1 1 1] Tell the player controller about the location that the player has entered in order to update any quest objectives in relation to it
  (Default|WaypointEntered (Variables|MRPGT|ReferenceOnly|GetPlayerControllerReference) (.ID (Utilities|Struct|BreakLocationStruct (Variables|MRPGT|Customizable|GetLocationInfo)))))

(event EventTick
  (params (DeltaSeconds :type Float%20%28single-precision%29)))

(fn ConstructionScript
  (Transformation|SetWorldScale3D (Variables|MRPGT|ReferenceOnly|GetCollisionBox) (Variables|MRPGT|Customizable|GetBoxCollisionScale)))