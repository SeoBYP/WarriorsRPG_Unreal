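; AI controller for combatant NPCs that runs the BT_NPC_Combatant behaviour tree on possess.
; On BeginPlay it stores the pawn's spawn location and max wander distance in the blackboard to limit wandering.
; Perception updates are forwarded to the BP_NPC_Combatant pawn, and Tick mirrors the pawn's dead state.
; Wrapper functions write target, sight, chase, dialogue and facing keys to the blackboard, and perception can be wiped on demand.
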(event OnTargetPerceptionUpdated(AIPerception)
  (params (Actor :type Actor%20Object%20Reference) (Stimulus :type AI%20Stimulus%20Structure))
  (bind _asbp_npc_combatant (Utilities|Casting|CastToBP_NPC_Combatant (Pawn|GetControlledPawn)))
  (Default|PerceptionUpdated _asbp_npc_combatant Actor Stimulus))

(event EventTick
  (params (DeltaSeconds :type Float%20%28single-precision%29))
  ;[1 1 1] Get Is Dead status from pawn object
  (bind _npcmaster (Variables|MRPGT|ReferenceOnly|GetNPCMaster)
    (:then
      _)
    (:else
      (bind _asbp_npc_master (Utilities|Casting|CastToBP_NPC_Master (Pawn|GetControlledPawn)))
      (Variables|MRPGT|ReferenceOnly|SetNPCMaster _asbp_npc_master)))
  (Variables|MRPGT|ReferenceOnly|SetIsDead (Default|GetIsDead _npcmaster)))

(event EventPossess
  (params (PossessedPawn :type Pawn%20Object%20Reference))
  (bind _debugthisblueprint_ (Variables|MRPGT|ReferenceOnly|GetDebugThisBlueprint?))
  (AI|RunBehaviorTree "/Game/MRPGT/ArtificialIntelligence/BehaviourTrees/BT_NPC_Combatant.BT_NPC_Combatant")
  (Development|PrintString "Running behaviour tree" _debugthisblueprint_ _debugthisblueprint_))

(event EventBeginPlay
  (bind _returnvalue (Pawn|GetControlledPawn))
  ;[1 1 1] Get a reference to pawn object
  (Utilities|IsValid _returnvalue
    (:Is%20Valid
      (bind _asbp_npc_master (Utilities|Casting|CastToBP_NPC_Master _returnvalue))
      (Variables|MRPGT|ReferenceOnly|SetNPCMaster _asbp_npc_master)
      ;[1 1 1] Record within the AI blackboard , the max wander distance and the initial location of the actor so that we can use it to make sure that it does not wander too far away from its spawn point in the behaviour tree.
      (bind _maxwanderdistance (Class|InterfaceNPCs1|GetMaxWanderDistance(Message) (Pawn|GetControlledPawn)))
      (AI|Components|Blackboard|SetValueasFloat (Variables|Default|GetBlackboard) (Variables|MRPGT|ReferenceOnly|GetMaxWanderDistanceName) _maxwanderdistance)
      (bind _output_get (Variables|MRPGT|ReferenceOnly|SetSpawnTransform (Transformation|GetActorTransform (Pawn|GetControlledPawn))))
      (AI|Components|Blackboard|SetValueasVector (Variables|Default|GetBlackboard) (Variables|MRPGT|ReferenceOnly|GetSpawnLocationName) (.Location (Math|Transform|BreakTransform _output_get))))
    (:Is%20Not%20Valid
      (Development|PrintString "Not valid" false (Variables|MRPGT|ReferenceOnly|GetDebugThisBlueprint?)))))

(event EventForgetAllTargets
  (Class|AIPerceptionComponent|ForgetAll (Variables|Default|GetAIPerception)))

(fn ConstructionScript)

(fn UpdateBlackboardTargetActor
  (params (TargetActor :type Object%20Object%20Reference))
  (AI|Components|Blackboard|SetValueasObject (Variables|Default|GetBlackboard) (Variables|MRPGT|ReferenceOnly|GetTargetActorName) TargetActor))

(fn UpdateBlackboardHasLineOfSight
  (params (HasLineOfSight :type Boolean))
  (AI|Components|Blackboard|SetValueasBool (Variables|Default|GetBlackboard) (Variables|MRPGT|ReferenceOnly|GetHasLineOfSightName) HasLineOfSight))

(fn UpdateBlackboardStillWantstoChase
  (params (StillWantsToChase :type Boolean))
  (AI|Components|Blackboard|SetValueasBool (Variables|Default|GetBlackboard) (Variables|MRPGT|ReferenceOnly|GetStillWantsToChaseName) StillWantsToChase))

(fn UpdateBlackboardLastKnownLocation
  (params (LastKnownLocation :type Vector))
  (AI|Components|Blackboard|SetValueasVector (Variables|Default|GetBlackboard) (Variables|MRPGT|ReferenceOnly|GetLastKnownLocationName) LastKnownLocation))

(fn UpdateBlackboardIsTargetStillAlive
  (params (BoolValue :type Boolean))
  (AI|Components|Blackboard|SetValueasBool (Variables|Default|GetBlackboard) (Variables|MRPGT|ReferenceOnly|GetIsTargetAliveName) BoolValue))

(fn UpdateBlackboardTargetAcquired
  (params (TargetAcquired :type Boolean))
  (AI|Components|Blackboard|SetValueasBool (Variables|Default|GetBlackboard) (Variables|MRPGT|ReferenceOnly|GetTargetAcquiredName) TargetAcquired))

(fn GetBlackboardTargetActor
  (bind _asactor (Utilities|Casting|CastToActor (AI|Components|Blackboard|GetValueasObject (Variables|Default|GetBlackboard) (Variables|MRPGT|ReferenceOnly|GetTargetActorName)))
    (:then
      (return _asactor))
    (:CastFailed
      (return 0))))

(fn UpdateBlackboardWantstoBeginDialogue
  (params (WantsToBeginDialogue :type Boolean))
  (AI|Components|Blackboard|SetValueasBool (Variables|Default|GetBlackboard) (Variables|MRPGT|ReferenceOnly|GetWantsToBeginDialogueName) WantsToBeginDialogue))

(fn UpdateBlackboardAttacksonSight
  (params (AttacksOnSight :type Boolean))
  (AI|Components|Blackboard|SetValueasBool (Variables|Default|GetBlackboard) (Variables|MRPGT|ReferenceOnly|GetAttacksOnSightName) AttacksOnSight))

(fn UpdateBlackboardShouldFaceActor
  (params (ShouldFaceActor :type Boolean))
  (AI|Components|Blackboard|SetValueasBool (Variables|Default|GetBlackboard) (Variables|MRPGT|ReferenceOnly|GetShouldFaceActorName) ShouldFaceActor))