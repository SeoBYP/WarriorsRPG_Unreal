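; Player controller for the main menu that creates the menu widget, focuses it in Game and UI input mode and flags it open on the game instance.
; On BeginPlay it also registers gameplay and UI input mapping contexts with Enhanced Input user settings so players can remap them in options.
; Completed menu input actions (directions, select, back/exit) are forwarded as enum-typed navigation requests.
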(event Input|EnhancedActionEvents|EnhancedInputActionIA_Menu_Left
  (params (ActionValue :type Boolean) (ElapsedSeconds :type Float%20%28double-precision%29) (TriggeredSeconds :type Float%20%28double-precision%29) (InputAction :type Input%20Action%20Object%20Reference :default "/Game/MRPGT/Input/IA_Menu_Left.IA_Menu_Left"))
  (:Completed
    (Default|CallNavigationRequest "NewEnumerator0")
    (Development|PrintString "Left" false)))

(event Input|EnhancedActionEvents|EnhancedInputActionIA_Menu_Right
  (params (ActionValue :type Boolean) (ElapsedSeconds :type Float%20%28double-precision%29) (TriggeredSeconds :type Float%20%28double-precision%29) (InputAction :type Input%20Action%20Object%20Reference :default "/Game/MRPGT/Input/IA_Menu_Right.IA_Menu_Right"))
  (:Completed
    (Default|CallNavigationRequest "NewEnumerator1")
    (Development|PrintString "Right" false)))

(event Input|EnhancedActionEvents|EnhancedInputActionIA_Menu_Back_Or_Exit
  (params (ActionValue :type Boolean) (ElapsedSeconds :type Float%20%28double-precision%29) (TriggeredSeconds :type Float%20%28double-precision%29) (InputAction :type Input%20Action%20Object%20Reference :default "/Game/MRPGT/Input/IA_Menu_Back_Or_Exit.IA_Menu_Back_Or_Exit"))
  (:Completed
    (Default|CallNavigationRequest "NewEnumerator7")
    (Development|PrintString "Back" false)))

(event Input|EnhancedActionEvents|EnhancedInputActionIA_Menu_Select
  (params (ActionValue :type Boolean) (ElapsedSeconds :type Float%20%28double-precision%29) (TriggeredSeconds :type Float%20%28double-precision%29) (InputAction :type Input%20Action%20Object%20Reference :default "/Game/MRPGT/Input/IA_Menu_Select.IA_Menu_Select"))
  (:Completed
    (Default|CallNavigationRequest "NewEnumerator6")
    (Development|PrintString "Select" false)))

(event Input|EnhancedActionEvents|EnhancedInputActionIA_Menu_Down
  (params (ActionValue :type Boolean) (ElapsedSeconds :type Float%20%28double-precision%29) (TriggeredSeconds :type Float%20%28double-precision%29) (InputAction :type Input%20Action%20Object%20Reference :default "/Game/MRPGT/Input/IA_Menu_Down.IA_Menu_Down"))
  (:Completed
    (Default|CallNavigationRequest "NewEnumerator5")
    (Development|PrintString "Down" false)))

(event Input|EnhancedActionEvents|EnhancedInputActionIA_Menu_Up
  (params (ActionValue :type Boolean) (ElapsedSeconds :type Float%20%28double-precision%29) (TriggeredSeconds :type Float%20%28double-precision%29) (InputAction :type Input%20Action%20Object%20Reference :default "/Game/MRPGT/Input/IA_Menu_Up.IA_Menu_Up"))
  (:Completed
    (Default|CallNavigationRequest "NewEnumerator4")
    (Development|PrintString "Up" false)))

(event EventBeginPlay
  (bind _debugthisblueprint (Variables|MRPGT|GetDebugThisBlueprint))
  (bind _asbp_mrpgt_game_instance (Utilities|Casting|CastToBP_MRPGT_GameInstance (Game|GetGameInstance)))
  (Variables|MRPGT|SetGameInstance _asbp_mrpgt_game_instance)
  (CallFunction|RegisterInputMappingContexts)
  (Development|PrintString (Utilities|String|Append "[BeginPlay] Creating MainMenuWidget" "") _debugthisblueprint _debugthisblueprint)
  (bind _returnvalue (UserInterface|CreateWidget "/Game/MRPGT/UserInterface/WidgetBlueprints/MainMenuWidget.MainMenuWidget_C" (Game|GetPlayerController 0)))
  (bind _output_get (Variables|MRPGT|SetMainMenu _returnvalue))
  (UserInterface|Viewport|AddtoViewport _output_get 0)
  (Input|SetInputModeGameandUI self (Variables|MRPGT|GetMainMenu) "DoNotLock" true false)
  (Variables|/Game/MRPGT/Blueprints/GameInstance/BP_MRPGT_GameInstance.BP_MRPGT_GameInstance_C|SetIsMainMenuOpen (Variables|MRPGT|GetGameInstance) true))

(fn ConstructionScript)

(fn RegisterInputMappingContexts
  ;[1 1 1] The IMCs need to be "registered" in order to be changeable by the user in the option widget. So here I registered all of them.
  (bind _returnvalue (Class|EnhancedInputSubsystemInterface|GetUserSettings(Message) (PlayerController|LocalPlayerSubsystems|GetEnhancedInputLocalPlayerSubsystem)))
  (bind _output_get (LocalVariables|SetUserInputSettings _returnvalue))
  (Utilities|IsValid _output_get
    (:Is%20Valid
      (Class|EnhancedInputUserSettings|RegisterInputMappingContext (LocalVariables|GetUserInputSettings) "/Game/MRPGT/Input/IMC_Buying.IMC_Buying")
      (Class|EnhancedInputUserSettings|RegisterInputMappingContext (LocalVariables|GetUserInputSettings) "/Game/MRPGT/Input/IMC_Crafting.IMC_Crafting")
      (Class|EnhancedInputUserSettings|RegisterInputMappingContext (LocalVariables|GetUserInputSettings) "/Game/MRPGT/Input/IMC_Enchanting.IMC_Enchanting")
      (Class|EnhancedInputUserSettings|RegisterInputMappingContext (LocalVariables|GetUserInputSettings) "/Game/MRPGT/Input/IMC_General_Game.IMC_General_Game")
      (Class|EnhancedInputUserSettings|RegisterInputMappingContext (LocalVariables|GetUserInputSettings) "/Game/MRPGT/Input/IMC_General_UI.IMC_General_UI")
      (Class|EnhancedInputUserSettings|RegisterInputMappingContext (LocalVariables|GetUserInputSettings) "/Game/MRPGT/Input/IMC_Inventory.IMC_Inventory")
      (Class|EnhancedInputUserSettings|RegisterInputMappingContext (LocalVariables|GetUserInputSettings) "/Game/MRPGT/Input/IMC_Mounted.IMC_Mounted")
      (Class|EnhancedInputUserSettings|RegisterInputMappingContext (LocalVariables|GetUserInputSettings) "/Game/MRPGT/Input/IMC_Selling.IMC_Selling")
      (Class|EnhancedInputUserSettings|RegisterInputMappingContext (LocalVariables|GetUserInputSettings) "/Game/MRPGT/Input/IMC_Storing.IMC_Storing")
      (Class|EnhancedInputUserSettings|RegisterInputMappingContext (LocalVariables|GetUserInputSettings) "/Game/MRPGT/Input/IMC_Taking.IMC_Taking")
      (Class|EnhancedInputUserSettings|RegisterInputMappingContext (LocalVariables|GetUserInputSettings) "/Game/MRPGT/Input/IMC_Reading.IMC_Reading")
      (Class|EnhancedInputUserSettings|RegisterInputMappingContext (LocalVariables|GetUserInputSettings) "/Game/MRPGT/Input/IMC_Lockpicking.IMC_Lockpicking"))))