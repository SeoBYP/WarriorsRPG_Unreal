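; Base harvestable world item, such as a plant, that the player gathers into their inventory.
; Construction script loads item info, mesh and enchantment FX from WorldItemsDataTable by ItemID.
; Interact adds a perk-adjusted quantity, notifies quest tracking, swaps to the harvested mesh and starts a regrowth timer that restores it.
; Empty Destroyed and ChangeState overrides keep harvests out of save games, so items reappear on load.
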(event Custom|Regrow
  ;[1 1 1] If the item was taken by the player then start a timer to regrow self after a specified amount of time (1 hour by default)
  (Components|StaticMesh|SetStaticMesh (Variables|Default|GetStaticMesh) (Utilities|Struct|BreakItemStruct (Variables|Default|GetItemInfo)))
  (Variables|Default|SetIsHarvested false))

(event EventDestroyed
  (Development|PrintString "Override inherited function. Do nothing. Harvested items will magically reappear upon save game being loaded. To add them to the save game instead, remove this override of the Event Destroyed event." false false))

(event EventChangeState
  (Development|PrintString "Override inherited function. Do nothing. Harvested items will magically reappear upon save game being loaded. To add them to the save game instead, remove this override of the Event Change State event." false false))

(event EventInteract
  (params (HitComponent :type Actor%20Component%20Object%20Reference) (InteractingActor :type Actor%20Object%20Reference))
  (bind _playercontroller (Variables|Default|GetPlayerController))
  (bind _playercontroller_2 (Variables|Default|GetPlayerController))
  (bind _gameinstance (Variables|Default|GetGameInstance))
  (bind _playercontroller_3 (Variables|Default|GetPlayerController))
  (bind _iteminfo (Variables|Default|GetItemInfo))
  (bind _iteminfo_2 (Variables|Default|GetItemInfo))
  (bind _name (Utilities|Struct|BreakItemStruct _iteminfo_2))
  (bind _harvestedmesh (Utilities|Struct|BreakItemStruct _iteminfo))
  (bind _charactersperks (Variables|/Game/MRPGT/Blueprints/Controllers/BP_InGamePlayerController.BP_InGamePlayerController_C|GetCharactersPerks _playercontroller_3))
  (bind _messageswidget (Variables|/Game/MRPGT/Blueprints/Controllers/BP_InGamePlayerController.BP_InGamePlayerController_C|GetMessagesWidget _playercontroller))
  (bind _returnvalue (Utilities|String|ToString(Text) _name))
  ;[1 1 1] Take item in the world and add it to the player's inventory. Called from the Character class
  (if (Variables|Default|GetInitialized)
    (if (not (Variables|Default|GetIsHarvested))
      (Development|PrintString (Utilities|String|Append "[EventInteract] Taking item, ID = " (Variables|Default|GetItemID)) false (Variables|Default|GetDebugEntireBlueprint))
      (bind _output_get (Variables|Default|SetQuantityHarvested (select (.Result (Default|HasPerkEffect _gameinstance _charactersperks "NewEnumerator6" "NewEnumerator18" "NewEnumerator9" "NewEnumerator9")) (Default|QuantityIngredientsHarvested _gameinstance _charactersperks) 1)))
      (bind _result (Default|AddItemtoInventory _playercontroller_2 (Variables|Default|GetItemInfo) (Variables|/Game/MRPGT/Blueprints/Controllers/BP_InGamePlayerController.BP_InGamePlayerController_C|GetCharactersItems _playercontroller_2) _output_get))
      ;[1 1 1] If the item was taken by the player then start a timer to regrow self after a specified amount of time (1 hour by default)
      (if _result
        (Utilities|Time|SetTimerbyEvent (delegate Custom|Regrow) (Variables|Default|GetRegrowthTimeSecs))
        ;[1 1 1] Send message to screen
        (if (== (Variables|Default|GetQuantityHarvested) 1)
          (Default|SendMessagetoScreen _messageswidget (Utilities|Text|ToText(String) (Utilities|String|Append "You harvested a " _returnvalue)) "NewEnumerator0")
          (else
            (Default|SendMessagetoScreen _messageswidget (Utilities|Text|ToText(String) (Utilities|String|Append "You harvested " (Utilities|String|ToString(Integer) (Variables|Default|GetQuantityHarvested)) " x " _returnvalue)) "NewEnumerator0")))
        ;[1 1 1] Tell the PlayerController that we took an item which might be a quest item
        (Default|QuestItemTaken (Variables|Default|GetPlayerController) (Variables|Default|GetItemInfo))
        (Audio|PlaySound2D "/Game/MRPGT/Audio/SoundCues/SC_PluckFlower_A.SC_PluckFlower_A" 1.0 1.0 0.0 0 0)
        (Variables|Default|SetIsHarvested true)
        ;[1 1 1] Change the look of the harvested plant by replacing the static mesh with a different one
        (Utilities|IsValid _harvestedmesh
          (:Is%20Valid
            (Components|StaticMesh|SetStaticMesh (Variables|Default|GetStaticMesh) _harvestedmesh))
          (:Is%20Not%20Valid
            (Components|StaticMesh|SetStaticMesh (Variables|Default|GetStaticMesh) 0)))))))

(fn ConstructionScript
  ;[1 1 1] Change the static mesh of the blueprint to the harvestablemesh for the row in the WorldItemsDataTable which corresponds to the ItemID value that the user has just changed in the Unreal Editor
  (Utilities|FlowControl|Sequence
    (:then_0
      (bind _outrownames (DataTable|GetDataTableRowNames "/Game/MRPGT/Blueprints/DataTables/WorldItemsDataTable.WorldItemsDataTable"))
      (for _array_element _outrownames
        (if (Utilities|Name|Equal(Name) _array_element (Utilities|String|StringToName (Variables|Default|GetItemID)))
          (bind _returnvalue (Utilities|GetDataTableRow "/Game/MRPGT/Blueprints/DataTables/WorldItemsDataTable.WorldItemsDataTable" _array_element)
            (:then
              (bind _output_get (LocalVariables|SetLocalItem _returnvalue))
              (bind _output_get_2 (Variables|Default|SetItemInfo _output_get))
              (if (Utilities|IsValid (.HarvestableMesh (Utilities|Struct|BreakItemStruct _output_get_2)))
                (Components|StaticMesh|SetStaticMesh (Variables|Default|GetStaticMesh) (.HarvestableMesh (Utilities|Struct|BreakItemStruct _output_get_2)))
                (if (.IsEnchanted (Utilities|Struct|BreakItemStruct (LocalVariables|GetLocalItem)))
                  (CallFunction|SetupNiagaraSystem (.EnchantmentFX (Utilities|Struct|BreakItemStruct (LocalVariables|GetLocalItem)))))))))))
    (:then_1
      (CallFunction|GenerateUniqueID false))))

(fn GetObjectName
  (return (Utilities|String|SelectString "" (Utilities|String|ToString(Text) (Utilities|Text|FormatText "Gather the {Name}" (.Name (Utilities|Struct|BreakItemStruct (Variables|Default|GetItemInfo))))) (Variables|Default|GetIsHarvested))))