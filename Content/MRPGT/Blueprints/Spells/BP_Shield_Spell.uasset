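; BP_Shield_Spell is a magic shield spell actor that drives the shield's material and Niagara visuals.
; On BeginPlay it writes color, opacity, fresnel depth fade and WPO settings to the MPC_MagicShield parameter collection and passes the color to Niagara.
; Each tick, a float spring interpolation moves StartSize toward TargetSize and feeds it to Niagara's User.SpringFloat for a springy size animation.
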(event EventBeginPlay
  (|CallParentFunction)
  (Rendering|Material|SetVectorParameterValue "/Game/MRPGT/FX/MagicShield/MPC_MagicShield.MPC_MagicShield" "Shield Color" (Variables|MRPGT|Customizable|GetShield%20Color) :!class /Script/Engine.KismetMaterialLibrary)
  (Rendering|Material|SetScalarParameterValue "/Game/MRPGT/FX/MagicShield/MPC_MagicShield.MPC_MagicShield" "Shield Opacity" (Variables|MRPGT|Customizable|GetShield%20Opacity) :!class /Script/Engine.KismetMaterialLibrary)
  (Rendering|Material|SetScalarParameterValue "/Game/MRPGT/FX/MagicShield/MPC_MagicShield.MPC_MagicShield" "Fresnel Depth Fade Opacity" (Variables|MRPGT|Customizable|GetFresnel%20Depth%20Fade%20Opacity) :!class /Script/Engine.KismetMaterialLibrary)
  (Rendering|Material|SetScalarParameterValue "/Game/MRPGT/FX/MagicShield/MPC_MagicShield.MPC_MagicShield" "Fresnel Depth Fade Distance" (Variables|MRPGT|Customizable|GetFresnel%20Depth%20Fade%20Distance) :!class /Script/Engine.KismetMaterialLibrary)
  (Rendering|Material|SetScalarParameterValue "/Game/MRPGT/FX/MagicShield/MPC_MagicShield.MPC_MagicShield" "WPO Multiplier" (Variables|MRPGT|Customizable|GetWPO%20Multiplier) :!class /Script/Engine.KismetMaterialLibrary)
  (Niagara|SetNiagaraVariable(LinearColor) (Variables|Default|GetNiagara) "User.Color" (Variables|MRPGT|Customizable|GetShield%20Color)))

(event Collision|EventActorBeginOverlap
  (params (OtherActor :type Actor%20Object%20Reference))
  (|CallParentFunction OtherActor) ; This node is disabled and will not be called.\nDrag off pins to build functionality.
)

(event EventTick
  (params (DeltaSeconds :type Float%20%28single-precision%29))
  (|CallParentFunction DeltaSeconds)
  (bind _returnvalue (Class|KismetMathLibrary|FloatSpringInterp (Variables|MRPGT|ReferenceOnly|GetStart%20Size) (Variables|MRPGT|ReferenceOnly|GetTarget%20Size) (Variables|MRPGT|ReferenceOnly|GetSpringState) (Variables|MRPGT|ReferenceOnly|GetSpring%20Stiffness) (Variables|MRPGT|ReferenceOnly|GetSpring%20Critical%20Damping%20Factor) DeltaSeconds (Variables|MRPGT|ReferenceOnly|GetMass) 1.0))
  (bind _output_get (Variables|MRPGT|ReferenceOnly|SetStart%20Size _returnvalue))
  (Development|PrintString (Utilities|String|ToString(Float) _output_get) false false)
  (Niagara|SetNiagaraVariable(Float) (Variables|Default|GetNiagara) "User.SpringFloat" (Variables|MRPGT|ReferenceOnly|GetStart%20Size)))

(fn ConstructionScript
  (|CallParentFunction))