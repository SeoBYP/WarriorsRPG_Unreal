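; Conjured light spell actor that displays a Niagara light orb with trails.
; The construction script pushes the orb, light and trail colors and the light radius into the Niagara component's user parameters.
; A Loop flag selects between repeating playback with fixed timings and a single run lasting the configurable Duration.
; The event graph has no logic, so all behavior comes from the Niagara system.
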(event EventBeginPlay)

(event Collision|EventActorBeginOverlap
  (params (OtherActor :type Actor%20Object%20Reference)))

(event EventTick
  (params (DeltaSeconds :type Float%20%28single-precision%29)))

(fn ConstructionScript
  (Niagara|SetNiagaraVariable(LinearColor) (Variables|Default|GetNPS_Light) "User.OrbColor" (Variables|MRPGT|GetOrbColor))
  (Niagara|SetNiagaraVariable(LinearColor) (Variables|Default|GetNPS_Light) "User.LightColor" (Variables|MRPGT|GetLightColor))
  (Niagara|SetNiagaraVariable(LinearColor) (Variables|Default|GetNPS_Light) "User.TrailsColor" (Variables|MRPGT|GetTrailsColor))
  (Niagara|SetNiagaraVariable(Float) (Variables|Default|GetNPS_Light) "User.LightRadius" (Variables|MRPGT|GetLightRadius))
  (if (Variables|MRPGT|GetLoop)
    (Niagara|SetNiagaraVariable(Float) (Variables|Default|GetNPS_Light) "User.NextLoopDuration" 1e+01)
    (Class|NiagaraComponent|SetNiagaraVariableInt (Variables|Default|GetNPS_Light) "User.MaxLoopCount")
    (Niagara|SetNiagaraVariable(Float) (Variables|Default|GetNPS_Light) "User.Duration" 9.0)
    (else
      (Niagara|SetNiagaraVariable(Float) (Variables|Default|GetNPS_Light) "User.NextLoopDuration" 0.0)
      (Class|NiagaraComponent|SetNiagaraVariableInt (Variables|Default|GetNPS_Light) "User.MaxLoopCount" 1)
      (Niagara|SetNiagaraVariable(Float) (Variables|Default|GetNPS_Light) "User.Duration" (Variables|MRPGT|GetDuration)))))