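; Master arrow projectile for RPG ranged combat that doubles as an inventory item, initialized from GameInstance item data.
; Launch ignores a launcher-dependent collision channel, then drives ProjectileMovement along local X.
; Fast hits on Enemy or Player actors apply typed damage from projectile, weapon, enchantments and the higher perk or stealth critical multiplier, then attach the arrow to the mesh temporarily.
; Interact moves it into the player's inventory.
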(event OnComponentHit(BoxCollision)
  (params (HitComponent :type Primitive%20Component%20Object%20Reference) (OtherActor :type Actor%20Object%20Reference) (OtherComp :type Primitive%20Component%20Object%20Reference) (NormalImpulse :type Vector :default "0, 0, 0") (Hit :type Hit%20Result%20Structure%20%28by%20ref%29))
  ;[1 1 1] Apply damage to target if its in BoxCollision during flight
  (Variables|MRPGT|ReferenceOnly|SetOtherActor OtherActor)
  (Development|PrintString (Utilities|String|Append "Hit a " (Utilities|GetDisplayName (Variables|MRPGT|ReferenceOnly|GetOtherActor))) false (Variables|MRPGT|ReferenceOnly|GetDebugThisGraph) "(R=1.000000,G=0.000000,B=0.014395,A=1.000000)" 5.0)
  (if (and (or (Actor|ActorHasTag (Variables|MRPGT|ReferenceOnly|GetOtherActor) "Enemy") (Actor|ActorHasTag (Variables|MRPGT|ReferenceOnly|GetOtherActor) "Player")) (not (Math|Float|NearlyEqual(Float) (Math|Vector|VectorLength (Transformation|GetVelocity)) 0.0 1e+03)))
    (Collision|SetCollisionResponsetoChannel (Variables|Default|GetBoxCollision) "ECC_Visibility" "ECR_Overlap")
    (Utilities|CalculateandApplyDamage)
    (Components|Activation|SetActive (Variables|Default|GetProjectileMovement) false true)
    (Collision|SetCollisionEnabled (Variables|Default|GetBoxCollision) "NoCollision")
    (Transformation|AttachComponentToComponent (Variables|/Script/Engine.Character|GetMesh (.AsCharacter (Utilities|Casting|CastToCharacter (Variables|MRPGT|ReferenceOnly|GetOtherActor)))) "headSocket" "KeepWorld" "KeepWorld" "KeepWorld" true)
    (Utilities|Time|SetTimerbyEvent (delegate Custom|CustomEvent_0) (Variables|MRPGT|ReferenceOnly|GetArrowLifeDuration))
    (bind _result (Class|InterfaceGeneralCharacter|IsthePlayerCharacter(Message) (Variables|MRPGT|ReferenceOnly|GetLauncherActor)))
    (if _result
      (if (Variables|MRPGT|ReferenceOnly|GetWasLastHitACritical?)
        (Class|InterfaceMessaging|SendShortMessage(Message) (Game|GetPlayerController 0) (Utilities|Text|FormatText "Critical hit! {1} x damage!" (Variables|MRPGT|ReferenceOnly|GetFinalCriticalHitDamageMultiplier)))
        (Class|InterfaceCombat|ResetCriticalHitMultiplier(Message) (Game|GetPlayerController 0))))
    (else
      (Development|PrintString "Actor does not have tag Enemy. It has the following tags " false (or (Variables|MRPGT|ReferenceOnly|GetDebugThisBlueprint) (Variables|MRPGT|ReferenceOnly|GetDebugThisGraph)))
      (for _array_element (Variables|/Script/Engine.Actor|GetTags (Variables|MRPGT|ReferenceOnly|GetOtherActor))
        (Development|PrintString (Utilities|String|ToString(Name) _array_element) false (or (Variables|MRPGT|ReferenceOnly|GetDebugThisBlueprint) (Variables|MRPGT|ReferenceOnly|GetDebugThisGraph)))))))

(event Custom|Launch
  (params (Speed :type Float%20%28double-precision%29) (ProjectileRotation :type Rotator))
  ;[1 1 1] Launch arrow into the air
  (Development|PrintString (Utilities|String|Append "[Launch] Current rotation == " (Utilities|String|ToString(Rotator) (Transformation|GetActorRotation)) ", New rotation == " (Utilities|String|ToString(Rotator) ProjectileRotation)) false true "(R=0.000000,G=0.660000,B=1.000000,A=1.000000)" 1e+01)
  (bind _result (Class|InterfaceGeneralCharacter|IsthePlayerCharacter(Message) (Variables|MRPGT|ReferenceOnly|GetLauncherActor)))
  (if _result
    (Collision|SetCollisionResponsetoChannel (Variables|Default|GetBoxCollision) "ECC_GameTraceChannel2" "ECR_Ignore")
    (Variables|MRPGT|Customizable|SetArrowSpeed Speed)
    (Transformation|SetActorRotation ProjectileRotation true)
    (else
      (Collision|SetCollisionResponsetoChannel (Variables|Default|GetBoxCollision) "ECC_GameTraceChannel3" "ECR_Ignore")
      (Variables|MRPGT|Customizable|SetArrowSpeed Speed)
      (Transformation|SetActorRotation ProjectileRotation true)))
  (Game|Components|ProjectileMovement|SetVelocityinLocalSpace (Variables|Default|GetProjectileMovement) (Math|Vector|MakeVector (Variables|MRPGT|Customizable|GetArrowSpeed) 0.0 0.0))
  (Development|PrintString (Utilities|String|Append "[Launch] New arrow rotation = " (Utilities|String|ToString(Rotator) (Transformation|GetActorRotation))) false)
  (Components|Activation|SetActive (Variables|Default|GetProjectileMovement) true false)
  (Collision|SetCollisionEnabled (Variables|Default|GetBoxCollision) "QueryAndPhysics")
  (Utilities|Time|SetTimerbyEvent (delegate Custom|DestroySelf) 6e+02))

(event Custom|DestroySelf
  ;[1 1 1] Launch arrow into the air
  (Actor|DestroyActor))

(event Custom|CustomEvent_0
  ;[1 1 1] Apply damage to target if its in BoxCollision during flight
  (CallFunction|DestroySelf))

(event EventInteract
  (params (HitComponent :type Actor%20Component%20Object%20Reference) (InteractingActor :type Actor%20Object%20Reference))
  ;[1 1 1] Take item in the world and add it to the player's inventory. Called from the FirstPersonCharacter class
  (if (and (Variables|MRPGT|ReferenceOnly|GetInitialized) (not (Variables|MRPGT|ReferenceOnly|GetIsVisuallyEquipped)))
    (Development|PrintString (Utilities|String|Append "Taking item, ID = " (Variables|MRPGT|ReferenceOnly|GetItemID)) false (Variables|MRPGT|ReferenceOnly|GetDebugEntireBlueprint))
    (bind _success (Class|InterfaceInventory1|AddItem(Message) (Game|GetPlayerController 0) (Variables|MRPGT|ReferenceOnly|GetItemInfo)))
    ;[1 1 1] If the item was taken by the player then destroy self (remove the Actor from the Level)
    (if _success
      (Actor|DestroyActor)
      ;[1 1 1] Send message to screen
      (Class|InterfaceMessaging|SendShortMessage(Message) (Game|GetPlayerController 0) (Utilities|Text|ToText(String) (Utilities|String|Append "You take the " (Utilities|String|ToString(Text) (.Name (Utilities|Struct|BreakItemStruct (Variables|MRPGT|ReferenceOnly|GetItemInfo)))))))
      ;[1 1 1] Calculate the initial carry weight of the player and update the UI
      (Class|InterfaceCharStats|UpdateWeightUI(Message) (Game|GetPlayerController 0))
      ;[1 1 1] Tell the PlayerController that we took an item which might be a quest item
      (Class|InterfaceQuests|ItemWasTaken(Message) (Game|GetPlayerController 0) (Variables|MRPGT|ReferenceOnly|GetItemInfo)))))

(event EventTick
  (params (DeltaSeconds :type Float%20%28single-precision%29))
  ;[1 1 1] Some debug stuff
  (Development|PrintString (Utilities|String|Append "Location: " (Utilities|String|ToString(Vector) (Transformation|GetActorLocation))) false false))

(fn ConstructionScript
  (|CallParentFunction))

(fn Initialize
  (params (ItemIn :type Item%20Struct%20Structure) (IsVisuallyEquipped :type Boolean) (IsSpawnedByNPC? :type Boolean))
  ;[1 1 1] To initialize this blueprint, get the data about this item from the WorldItems array and assign it to a local variable, only once
  (Utilities|FlowControl|Sequence
    (:then_0
      (Development|PrintString (Utilities|String|Append "[Initialize] Item ID = " (.ID (Utilities|Struct|BreakItemStruct ItemIn))) false (Variables|MRPGT|ReferenceOnly|GetDebugEntireBlueprint) "(R=0.000000,G=0.660000,B=1.000000,A=1.000000)" 5.0)
      (bind _item (Class|InterfaceItems|GetItembyID(Message) (Game|GetGameInstance) (.ID (Utilities|Struct|BreakItemStruct ItemIn))))
      (bind _output_get (LocalVariables|SetLocalItem _item))
      (bind _structout (Utilities|Struct|SetmembersinItemStruct _output_get (* (.Quantity (Utilities|Struct|BreakItemStruct _output_get)) (.UnitWeight (Utilities|Struct|BreakItemStruct _output_get))) (Math|Conversions|ToFloat(Integer) (* (.Quantity (Utilities|Struct|BreakItemStruct _output_get)) (.UnitValue (Utilities|Struct|BreakItemStruct _output_get)))) (Math|Conversions|ToFloat(Integer) (Math|Float|Round (/ (Math|Conversions|ToFloat(Integer) (.UnitValue (Utilities|Struct|BreakItemStruct _output_get))) (.UnitWeight (Utilities|Struct|BreakItemStruct _output_get)))))))
      (bind _output_get_2 (Variables|MRPGT|ReferenceOnly|SetItemInfo _structout))
      (Development|PrintString (Utilities|String|Append "[Initialize] This item is a " (Utilities|String|ToString(Text) (.Name (Utilities|Struct|BreakItemStruct _output_get_2)))) false (Variables|MRPGT|ReferenceOnly|GetDebugEntireBlueprint) "(R=0.000000,G=0.660000,B=1.000000,A=1.000000)" 5.0))
    (:then_1
      (Variables|MRPGT|ReferenceOnly|SetIsVisuallyEquipped IsVisuallyEquipped)
      (if IsSpawnedByNPC?
        (Collision|SetCollisionResponsetoChannel (Variables|Default|GetBoxCollision) "ECC_GameTraceChannel2" "ECR_Block")
        (Collision|SetCollisionResponsetoChannel (Variables|Default|GetBoxCollision) "ECC_GameTraceChannel3" "ECR_Overlap")
        (Development|PrintString (Utilities|String|Append "[Initialize] Set CollisionResponseToChannel Player to Block" "") false (Variables|MRPGT|ReferenceOnly|GetDebugEntireBlueprint))))
    (:then_2
      (Variables|MRPGT|ReferenceOnly|SetInitialized true)
      (Development|PrintString (Utilities|String|Append "[Initialize] END" "") false (Variables|MRPGT|ReferenceOnly|GetDebugEntireBlueprint)))))

(fn GetDesiredRotationOfSelf
  (params (Camera :type Scene%20Component%20Object%20Reference))
  (bind _returnvalue (Transformation|GetActorLocation))
  (bind _returnvalue_2 (Transformation|GetWorldLocation Camera))
  (bind _returnvalue_3 (Math|Vector|GetForwardVector Camera))
  (bind _arrowlinetracedistance (Variables|MRPGT|Customizable|GetArrowLineTraceDistance))
  (bind _returnvalue_4 (* _returnvalue_3 _arrowlinetracedistance))
  (bind _returnvalue_5 (+ _returnvalue_4 _returnvalue_2))
  ;[1 1 1] Get the desired rotation of the arrow after it has been fired. It is pointing in the Y axis so the rotation is calculated to be the vector from the arrow to a point in space 10 metres in front of the camera. The camera can be passed into the function so that the third person camera or the first person camera can be the parameter and result in a different rotation being output.
  (Development|PrintString (Utilities|String|Append "[Get Desired Rotation Of Self] Initial arrow rotation = " (Utilities|String|ToString(Rotator) (Transformation|GetActorRotation))) false (LocalVariables|GetLocalDebugThisFunction))
  (Collision|LineTraceByChannel _returnvalue _returnvalue_5 "TraceTypeQuery1" false 0 "None")
  (return (Math|Rotator|MakeRotfromY (Math|Vector|Normalize (- _returnvalue_5 _returnvalue)))))

(fn GetProjectileDamage
  (bind _iteminfo (Variables|MRPGT|ReferenceOnly|GetItemInfo))
  (bind (_name _weapondamage) (Utilities|Struct|BreakItemStruct _iteminfo))
  (Development|PrintString (Utilities|String|Append "[GetProjectileDamage] Projectile Base Damage == " (Utilities|String|ToString(Integer) _weapondamage) ", Projectile Name == " (Utilities|String|ToString(Text) _name)) false false)
  (return (Math|Conversions|ToFloat(Integer) _weapondamage)))

(fn GetProjectileEnchantmentDamage
  (bind _iteminfo (Variables|MRPGT|ReferenceOnly|GetItemInfo))
  (bind (_name _weapondamage _staticmesh _skeletalmesh _enchantmenttype _enchantmentvalue) (Utilities|Struct|BreakItemStruct _iteminfo))
  (bind _returnvalue (Utilities|Select :Index _enchantmenttype :NewEnumerator10 0 :NewEnumerator0 0 :NewEnumerator1 0 :NewEnumerator2 0 :NewEnumerator3 0 :NewEnumerator4 0 :NewEnumerator5 0 :NewEnumerator12 0 :NewEnumerator11 0 :NewEnumerator13 0 :NewEnumerator14 0 :NewEnumerator6 0 :NewEnumerator7 0 :NewEnumerator15 _enchantmentvalue :NewEnumerator16 _enchantmentvalue :NewEnumerator17 _enchantmentvalue))
  (Development|PrintString (Utilities|String|Append "[GetProjectileDamage] Projectile Enchantment Damage == " (Utilities|String|ToString(Integer) _returnvalue)) false false)
  (return (Math|Conversions|ToFloat(Integer) _returnvalue)))

(fn GetID
  (return ""))

(fn GetLauncherActor
  (return (Variables|MRPGT|ReferenceOnly|GetLauncherActor)))

(fn GetObjectName
  (if (not (Variables|MRPGT|ReferenceOnly|GetIsVisuallyEquipped))
    (return (Utilities|String|ToString(Text) (.Name (Utilities|Struct|BreakItemStruct (Variables|MRPGT|ReferenceOnly|GetItemInfo)))))))

(fn IsProjectile
  (return true))