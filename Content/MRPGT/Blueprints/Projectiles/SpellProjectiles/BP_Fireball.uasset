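; BP_Fireball is a fireball spell projectile that adds color setup to the behavior it inherits from its parent.
; On BeginPlay, after the parent call, it passes its Color and LightColor variables to the Niagara effect's user parameters.
; It also writes Color to the shared MPC_Fireball material parameter collection, so that color is global rather than per projectile.
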(event EventBeginPlay
  (|CallParentFunction)
  (Niagara|SetNiagaraVariable(LinearColor) (Variables|Default|GetNiagara) "User.Color" (Variables|Default|GetColor))
  (Niagara|SetNiagaraVariable(LinearColor) (Variables|Default|GetNiagara) "User.LightColor" (Variables|Default|GetLightColor))
  (Rendering|Material|SetVectorParameterValue "/Game/MRPGT/Materials/MaterialParameterCollections/MPC_Fireball.MPC_Fireball" "Fireball Color" (Variables|Default|GetColor) :!class /Script/Engine.KismetMaterialLibrary))

(event Collision|EventActorBeginOverlap
  (params (OtherActor :type Actor%20Object%20Reference))
  (|CallParentFunction OtherActor) ; This node is disabled and will not be called.\nDrag off pins to build functionality.
)

(event EventTick
  (params (DeltaSeconds :type Float%20%28single-precision%29))
  (|CallParentFunction DeltaSeconds) ; This node is disabled and will not be called.\nDrag off pins to build functionality.
)

(fn ConstructionScript
  (|CallParentFunction))