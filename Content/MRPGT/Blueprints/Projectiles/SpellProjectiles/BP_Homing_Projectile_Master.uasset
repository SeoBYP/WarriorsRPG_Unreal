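; Master homing spell projectile that steers itself toward an enemy combatant NPC.
; BeginPlay applies the spell's release Niagara effect, picks the nearest tagged enemy if no target is set, and opens a Tick-fed gate.
; The gate plays a timeline that lerps rotation toward the target and rebuilds velocity along the new facing with slight acceleration per update.
; An uncalled line-trace finder ignores its trace result and also picks the nearest enemy.
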(event EventBeginPlay
  (bind _returnvalue (Transformation|GetActorRotation))
  (|CallParentFunction)
  (CallFunction|Initialize)
  (Variables|Default|GetHomingTarget
    (:then
      (Utilities|FlowControl|Gate true) ; enters at Open
    )
    (:else
      (CallFunction|FindNearestHomingTarget)
      (Utilities|FlowControl|Gate true) ; enters at Open
    )))

(event Collision|EventActorBeginOverlap
  (params (OtherActor :type Actor%20Object%20Reference))
  (|CallParentFunction OtherActor) ; This node is disabled and will not be called.\nDrag off pins to build functionality.
)

(event EventTick
  (params (DeltaSeconds :type Float%20%28single-precision%29))
  (bind _returnvalue (Transformation|GetActorRotation))
  (|CallParentFunction DeltaSeconds)
  (Utilities|FlowControl|Gate true
    (:Exit
      (bind _lerpalpha (Timeline|Timeline_0 Play)
        (:Update
          (Transformation|SetActorRotation (Math|Rotator|Lerp(Rotator) (Transformation|GetActorRotation) (Math|Rotator|FindLookatRotation (Transformation|GetActorLocation) (Transformation|GetActorLocation (Variables|Default|GetHomingTarget))) _lerpalpha))
          (Variables|/Script/Engine.MovementComponent|SetVelocity (Variables|Default|GetProjectileMovement) (* (Class|KismetMathLibrary|CreateVectorfromYawPitch (.yaw _returnvalue) (.pitch _returnvalue) (Math|Vector|VectorLength (Transformation|GetVelocity))) 1.01)))))))

(fn ConstructionScript
  (|CallParentFunction))

(fn FindNearestHomingTarget
  ;[1 1 1] Finds the nearest enemy NPC. Might be undesirable as it can choose an unintended NPC.
  (bind _outactors (Actor|GetAllActorsOfClasswithTag "/Game/MRPGT/Blueprints/NPCs/BP_NPC_Combatant_Enemy.BP_NPC_Combatant_Enemy_C" "Enemy"))
  (bind _array_element (Utilities|Array|ForEachLoopwithBreak _outactors)
    (:LoopBody
      (if (< (Math|Vector|VectorLength (- (Transformation|GetActorLocation _array_element) (Transformation|GetActorLocation))) (Variables|Default|GetClosestDistance))
        (Variables|Default|SetClosestDistance (Math|Vector|VectorLength (- (Transformation|GetActorLocation _array_element) (Transformation|GetActorLocation))))
        (Variables|Default|SetHomingTarget _array_element)))
    (:Completed
      (Development|PrintString (Utilities|String|Append "[Find Nearest Homing Target] Homing Target == " (Utilities|GetDisplayName (Variables|Default|GetHomingTarget))) false)
      (return (Actor|GetComponentbyClass (Variables|Default|GetHomingTarget) "/Script/Engine.SceneComponent")))))

(fn FindHomingTargetwithLineTrace
  (Collision|LineTraceByChannel (Transformation|GetActorLocation) (* (Math|Vector|GetForwardVector (Transformation|GetActorRotation)) 1e+04) "TraceTypeQuery1" false 0 "Persistent")
  ;[1 1 1] Finds the nearest enemy NPC using a line trace method.
  (bind _outactors (Actor|GetAllActorsOfClasswithTag "/Game/MRPGT/Blueprints/NPCs/BP_NPC_Combatant_Enemy.BP_NPC_Combatant_Enemy_C" "Enemy"))
  (bind _array_element (Utilities|Array|ForEachLoopwithBreak _outactors)
    (:LoopBody
      (if (< (Math|Vector|VectorLength (- (Transformation|GetActorLocation _array_element) (Transformation|GetActorLocation))) (Variables|Default|GetClosestDistance))
        (Variables|Default|SetClosestDistance (Math|Vector|VectorLength (- (Transformation|GetActorLocation _array_element) (Transformation|GetActorLocation))))
        (Variables|Default|SetHomingTarget _array_element)))
    (:Completed
      (Development|PrintString (Utilities|String|Append "Homing Target == " (Utilities|GetDisplayName (Variables|Default|GetHomingTarget))))
      (return (Actor|GetComponentbyClass (Variables|Default|GetHomingTarget) "/Script/Engine.SceneComponent")))))

(fn Initialize
  (Class|NiagaraComponent|SetAsset (Variables|Default|GetNiagara) (.NiagaraSystemOnRelease (Utilities|Struct|BreakSpellStruct (Variables|Default|GetSpellInfo))) true)
  (Niagara|ResetSystem (Variables|Default|GetNiagara)))