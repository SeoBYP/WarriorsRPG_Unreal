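; BP_SpellRenderToTexture is a retired (since v2.11) spell preview stage that uses a SceneCaptureComponent2D, kept as a render-to-texture reference.
; It swaps in a Cascade template or a spell's Niagara preview, optionally overriding a user static mesh parameter with a custom mesh.
; Activate and Deactivate toggle per-frame capture, lights and post-process intensity, with Deactivate also clearing the effects.
; Capture and effect components keep ticking while the game is paused.
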(event OnComponentActivated(SceneCaptureComponent2D)
  (params (Component :type Actor%20Component%20Object%20Reference) (bReset :type Boolean))
  ;[1 0 0] Since v2.11 this blueprint is no longer used. I left it here for reference in case you want to implement some kind of render to texture using a SceneCaptureComponent2D.
  (Development|PrintString "[EventGraph] SceneCaptureComponent2D activated" false (Variables|MRPGT|GetDebugThisEventGraph)))

(event EventBeginPlay
  ;[1 0 0] Since v2.11 this blueprint is no longer used. I left it here for reference in case you want to implement some kind of render to texture using a SceneCaptureComponent2D.
  (Class|ActorComponent|SetTickablewhenPaused (Variables|Default|GetSceneCaptureComponent2D) true))

(fn ConstructionScript)

(fn SetNewParticleSystem
  (params (ParticleSystemIn :type Particle%20System%20Object%20Reference))
  (Effects|Components|ParticleSystem|SetTemplate (Variables|Default|GetParticleSystem) ParticleSystemIn))

(fn ClearParticleSystem
  (Effects|Components|ParticleSystem|SetTemplate (Variables|Default|GetParticleSystem) 0)
  (Class|NiagaraComponent|SetAsset (Variables|Default|GetNiagara) 0 true))

(fn SetNewNiagaraSystem
  (params (Spell :type Spell%20Struct%20Structure))
  (bind (_spellpreview _projectilespellclass _assignniagaracustommesh _niagaracustommesh _niagaracustommeshparametername) (Utilities|Struct|BreakSpellStruct Spell))
  (Components|Activation|SetActive (Variables|Default|GetNiagara) false true)
  (Class|NiagaraComponent|SetAsset (Variables|Default|GetNiagara) _spellpreview true)
  (if _assignniagaracustommesh
    (Components|StaticMesh|SetStaticMesh (Variables|Default|GetCustomStaticMesh) _niagaracustommesh)
    (Class|NiagaraFunctionLibrary|OverrideSystemUserVariableStaticMeshComponent (Variables|Default|GetNiagara) _niagaracustommeshparametername (Variables|Default|GetCustomStaticMesh)))
  (Components|Activation|SetActive (Variables|Default|GetNiagara) true true)
  (Rendering|SetVisibility (Variables|Default|GetNiagara) true false)
  (Class|ActorComponent|SetTickablewhenPaused (Variables|Default|GetNiagara) true))

(fn Activate
  (bind _postprocess1 (Variables|Default|GetPostProcess1))
  (Variables|/Script/Engine.SceneCaptureComponent|SetbCaptureEveryFrame (Variables|Default|GetSceneCaptureComponent2D) true)
  (bind _structout (Utilities|Struct|SetmembersinPostProcessSettings (Variables|/Script/Engine.PostProcessComponent|GetSettings _postprocess1) 2.0))
  (Variables|/Script/Engine.PostProcessComponent|SetSettings _postprocess1 _structout)
  (Rendering|SetVisibility (Variables|Default|GetSpotLight) true false))

(fn Deactivate
  (bind _postprocess1 (Variables|Default|GetPostProcess1))
  (Variables|/Script/Engine.SceneCaptureComponent|SetbCaptureEveryFrame (Variables|Default|GetSceneCaptureComponent2D) false)
  (bind _structout (Utilities|Struct|SetmembersinPostProcessSettings (Variables|/Script/Engine.PostProcessComponent|GetSettings _postprocess1) 0.0))
  (Variables|/Script/Engine.PostProcessComponent|SetSettings _postprocess1 _structout)
  (Rendering|SetVisibility (Variables|Default|GetSpotLight) false false)
  (CallFunction|ClearParticleSystem))