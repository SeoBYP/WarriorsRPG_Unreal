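; Unused since v2.11 and kept for reference, this actor renders an item mesh, optionally with Niagara effects, through a SceneCaptureComponent2D for an interactive preview.
; SetNewMesh scales the mesh to fit a desired extent and re-centers it on its bounds for rotation.
; Mouse input rotates MeshRoot and wheel-zooms it within limits by moving it, not the camera.
; Activate and Deactivate toggle per-frame capture and lights; deactivation also clears mesh and effect.
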(event OnComponentActivated(SceneCaptureComponent2D)
  (params (Component :type Actor%20Component%20Object%20Reference) (bReset :type Boolean))
  ;[1 0 0] Since v2.11 this blueprint is no longer used. I left it here for reference in case you want to implement some kind of render to texture using a SceneCaptureComponent2D.
  (Development|PrintString "SceneCaptureComponent2D activated" false (Variables|MRPGT|ReferenceOnly|GetDebugThisEntireBlueprint)))

(event Custom|UpdatePivotAndScale
  (bind _debugthiseventgraph (Variables|MRPGT|ReferenceOnly|GetDebugThisEventGraph))
  (bind _debugthisentireblueprint (Variables|MRPGT|ReferenceOnly|GetDebugThisEntireBlueprint))
  (bind _desiredextend (Variables|MRPGT|ReferenceOnly|GetDesiredExtend))
  (bind _returnvalue (or _debugthisentireblueprint _debugthiseventgraph))
  ;[1 0 0] Since v2.11 this blueprint is no longer used. I left it here for reference in case you want to implement some kind of render to texture using a SceneCaptureComponent2D.
  ;;[1 1 1] When viewing a new object set its pivot in the centre of the object so that it rotates around its centre point
  (Variables|MRPGT|ReferenceOnly|SetCurrentMeshExtend (.BoxExtent (Collision|GetComponentBounds (Variables|Default|GetMesh))))
  (Transformation|SetWorldScale3D (Variables|Default|GetMesh) (* (Transformation|GetWorldScale (Variables|Default|GetMesh)) (Math|Float|Min(Float) (/ (.x _desiredextend) (.x (Variables|MRPGT|ReferenceOnly|GetCurrentMeshExtend))) (/ (.y _desiredextend) (.y (Variables|MRPGT|ReferenceOnly|GetCurrentMeshExtend))) (/ (.z _desiredextend) (.z (Variables|MRPGT|ReferenceOnly|GetCurrentMeshExtend))))))
  (Transformation|AddLocalOffset (Variables|Default|GetMesh) (- (Transformation|GetWorldLocation (Variables|Default|GetMesh)) (.Origin (Collision|GetComponentBounds (Variables|Default|GetMesh)))) false false)
  (Transformation|SetRelativeRotation (Variables|Default|GetMeshRoot) "1.000000,1.000000,1.000000" false false) ; Resets the rotation of the mesh root. I set to 1, 1, 1 rotation to workaround a bug whereby the mesh turns black
  (Development|PrintString "UpdatePivotAndScale fired" _returnvalue _returnvalue))

(event Custom|OnClickedStart
  (params (MouseLocation :type Vector%202D%20Structure))
  (bind _debugthisentireblueprint (Variables|MRPGT|ReferenceOnly|GetDebugThisEntireBlueprint))
  (bind _debugthiseventgraph (Variables|MRPGT|ReferenceOnly|GetDebugThisEventGraph))
  (bind _returnvalue (or _debugthisentireblueprint _debugthiseventgraph))
  ;[1 0 0] Since v2.11 this blueprint is no longer used. I left it here for reference in case you want to implement some kind of render to texture using a SceneCaptureComponent2D.
  ;;[1 1 1] Enable rotation of the object when holding mouse button down
  (Variables|MRPGT|ReferenceOnly|SetOnStartRotateLocation MouseLocation)
  (Variables|MRPGT|ReferenceOnly|SetbRotateEnabled true)
  (Development|PrintString "OnClickedStart fired" _returnvalue _returnvalue))

(event Custom|OnMouseMove
  (params (MouseLocation :type Vector%202D%20Structure))
  (bind _debugthisentireblueprint (Variables|MRPGT|ReferenceOnly|GetDebugThisEntireBlueprint))
  (bind _debugthiseventgraph (Variables|MRPGT|ReferenceOnly|GetDebugThisEventGraph))
  (bind _returnvalue (or _debugthisentireblueprint _debugthiseventgraph))
  ;[1 0 0] Since v2.11 this blueprint is no longer used. I left it here for reference in case you want to implement some kind of render to texture using a SceneCaptureComponent2D.
  ;;[1 1 1] Rotate the object with the mouse
  (if (Variables|MRPGT|ReferenceOnly|GetbRotateEnabled)
    (Transformation|AddWorldRotation (Variables|Default|GetMeshRoot) (Math|Rotator|MakeRotator 0.0 (.y (- MouseLocation (Variables|MRPGT|ReferenceOnly|GetOnStartRotateLocation))) (* (.x (- MouseLocation (Variables|MRPGT|ReferenceOnly|GetOnStartRotateLocation))) -1.0)) false false)
    (Variables|MRPGT|ReferenceOnly|SetOnStartRotateLocation MouseLocation)
    (Development|PrintString "OnMouseMove fired" _returnvalue _returnvalue)))

(event Custom|OnClickedEnd
  (params (MouseLocation :type Vector%202D%20Structure))
  (bind _debugthisentireblueprint (Variables|MRPGT|ReferenceOnly|GetDebugThisEntireBlueprint))
  (bind _debugthiseventgraph (Variables|MRPGT|ReferenceOnly|GetDebugThisEventGraph))
  (bind _returnvalue (or _debugthisentireblueprint _debugthiseventgraph))
  ;[1 0 0] Since v2.11 this blueprint is no longer used. I left it here for reference in case you want to implement some kind of render to texture using a SceneCaptureComponent2D.
  ;;[1 1 1] Disable rotation of the object when mouse button released
  (Variables|MRPGT|ReferenceOnly|SetbRotateEnabled false)
  (Development|PrintString "OnClickedEnd fired" _returnvalue _returnvalue))

(event Custom|OnMouseWheel
  (params (WheelDelta :type Float%20%28double-precision%29))
  (bind _returnvalue (* WheelDelta 2.0))
  (bind _debugthiseventgraph (Variables|MRPGT|ReferenceOnly|GetDebugThisEventGraph))
  (bind _debugthisentireblueprint (Variables|MRPGT|ReferenceOnly|GetDebugThisEntireBlueprint))
  (bind _debugthiseventgraph_2 (Variables|MRPGT|ReferenceOnly|GetDebugThisEventGraph))
  (bind _meshroot (Variables|Default|GetMeshRoot))
  (bind _debugthisentireblueprint_2 (Variables|MRPGT|ReferenceOnly|GetDebugThisEntireBlueprint))
  (bind _returnvalue_2 (Transformation|GetRelativeTransform _meshroot))
  (bind _returnvalue_3 (Math|Float|Clamp(Float) _returnvalue -2.0 2.0))
  (bind _returnvalue_4 (or _debugthisentireblueprint_2 _debugthiseventgraph))
  (bind _returnvalue_5 (or _debugthisentireblueprint _debugthiseventgraph_2))
  (bind _x (Math|Vector|BreakVector (.location _returnvalue_2)))
  ;[1 0 0] Since v2.11 this blueprint is no longer used. I left it here for reference in case you want to implement some kind of render to texture using a SceneCaptureComponent2D.
  ;;[1 1 1] Zoom in and out with the mouse wheel
  (Development|PrintString (Utilities|String|Append "Zooming " (Utilities|String|ToString(Float) _returnvalue_3) ", " (Utilities|String|Append "Distance = " (Utilities|String|ToString(Float) (Math|Float|Absolute(Float) (.X (Math|Vector|BreakVector (- (.location (Variables|MRPGT|ReferenceOnly|GetStartingMeshRootTransform)) (.location _returnvalue_2)))))) ", Relative X Location = " (Utilities|String|ToString(Float) _x))) _returnvalue_4 _returnvalue_4)
  (if (> _returnvalue_3 0.0)
    (Development|PrintString "Mouse delta > 0" _returnvalue_5 _returnvalue_5)
    (if (< (+ _x _returnvalue_3) (Variables|MRPGT|ReferenceOnly|GetMaxCameraZoom))
      (Transformation|AddRelativeLocation (Variables|Default|GetMeshRoot) (Math|Vector|MakeVector _returnvalue_3 (/ _returnvalue_3 2.0) 0.0) false false :!label _label))
    (else
      (Development|PrintString "Mouse delta < 0" _returnvalue_5 _returnvalue_5)
      (if (> (- _x (Math|Float|Absolute(Float) _returnvalue_3)) (* (Variables|MRPGT|ReferenceOnly|GetMaxCameraZoom) -1.0))
        (goto _label)))))

(event EventBeginPlay
  ;[1 0 0] Since v2.11 this blueprint is no longer used. I left it here for reference in case you want to implement some kind of render to texture using a SceneCaptureComponent2D.
  (Class|ActorComponent|SetTickablewhenPaused (Variables|Default|GetSceneCaptureComponent2D) true))

(fn ConstructionScript
  (bind _scenecapturecomponent2d (Variables|Default|GetSceneCaptureComponent2D))
  (bind _hiddenactors (Variables|/Script/Engine.SceneCaptureComponent|GetHiddenActors _scenecapturecomponent2d))
  (Utilities|FlowControl|Sequence
    (:then_0
      (Variables|/Script/Engine.SceneCaptureComponent|SetPrimitiveRenderMode _scenecapturecomponent2d "PRM_LegacySceneCapture")
      (Utilities|Array|Add _hiddenactors 0)
      (bind _outactors (Actor|GetAllActorsOfClass "/Engine/EngineSky/BP_Sky_Sphere.BP_Sky_Sphere_C"))
      (if (> (Utilities|Array|Length _outactors) 0)
        (Utilities|Array|Add _hiddenactors (Utilities|Array|Get(acopy) _outactors))))
    (:then_1
      (Variables|MRPGT|ReferenceOnly|SetStartingMeshRootTransform (Transformation|GetRelativeTransform (Variables|Default|GetMeshRoot))))))

(fn SetNewMesh
  (params (Mesh :type Static%20Mesh%20Object%20Reference))
  (bind _debugthiseventgraph (Variables|MRPGT|ReferenceOnly|GetDebugThisEventGraph))
  (bind _debugthisentireblueprint (Variables|MRPGT|ReferenceOnly|GetDebugThisEntireBlueprint))
  (bind _returnvalue (or _debugthisentireblueprint _debugthiseventgraph))
  (Development|PrintString "SetNewMesh fired" _returnvalue _returnvalue)
  (Components|StaticMesh|SetStaticMesh (Variables|Default|GetMesh) Mesh)
  (Transformation|SetRelativeLocation (Variables|Default|GetMesh) "0, 0, 0" false false) ; Resets the location to the root location
  (Transformation|SetRelativeRotation (Variables|Default|GetMeshRoot) "0, 0, 0" false false) ; Resets the rotation of the mesh root
  (CallFunction|UpdatePivotandScale)
  (Variables|MRPGT|ReferenceOnly|SetStartingMeshRootTransform (Transformation|GetRelativeTransform (Variables|Default|GetMeshRoot))))

(fn ClearMesh
  (bind _debugthiseventgraph (Variables|MRPGT|ReferenceOnly|GetDebugThisEventGraph))
  (bind _debugthisentireblueprint (Variables|MRPGT|ReferenceOnly|GetDebugThisEntireBlueprint))
  (bind _returnvalue (or _debugthisentireblueprint _debugthiseventgraph))
  (Development|PrintString "ClearMesh fired" _returnvalue _returnvalue)
  (Components|StaticMesh|SetStaticMesh (Variables|Default|GetMesh) 0))

(fn Activate
  (Variables|/Script/Engine.SceneCaptureComponent|SetbCaptureEveryFrame (Variables|Default|GetSceneCaptureComponent2D) true)
  (Rendering|SetVisibility (Variables|Default|GetPointLight1) true false)
  (Rendering|SceneCapture|ShowOnlyActorComponents (Variables|Default|GetSceneCaptureComponent2D) self false))

(fn Deactivate
  (Variables|/Script/Engine.SceneCaptureComponent|SetbCaptureEveryFrame (Variables|Default|GetSceneCaptureComponent2D) false)
  (CallFunction|StopNiagaraSystem)
  (Rendering|SetVisibility (Variables|Default|GetPointLight1) false false)
  (CallFunction|ClearMesh))

(fn SetupNiagaraSystem
  (params (NiagaraSystemIn :type Niagara%20System%20Object%20Reference))
  (if (Utilities|IsValid NiagaraSystemIn)
    (Class|NiagaraComponent|SetAsset (Variables|Default|GetNiagara) NiagaraSystemIn true)
    (Class|NiagaraFunctionLibrary|OverrideSystemUserVariableStaticMesh (Variables|Default|GetNiagara) "User.StaticMesh" (Variables|/Script/Engine.StaticMeshComponent|GetStaticMesh (Variables|Default|GetMesh)))
    (Components|Activation|SetActive (Variables|Default|GetNiagara) true true)
    (Rendering|SetVisibility (Variables|Default|GetNiagara) true false)))

(fn StopNiagaraSystem
  (Components|Activation|SetActive (Variables|Default|GetNiagara) false false)
  (Rendering|SetVisibility (Variables|Default|GetNiagara) false false))