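; Sandbox actor for dragging into a level and tuning enchantment effect parameters to find new item looks.
; It applies a custom static mesh to the Mesh and to the Niagara system's StaticMesh user parameter.
; Exposed colors, noise, spawn rate and acceleration drive the Niagara system, while a third color and opacity set the mesh materials' parameters.
; The construction script and BeginPlay run identical setup, so values apply both on construction and at play start.
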(event EventBeginPlay
  ;[1 1 1] The purpose of this blueprint is only for you to drag it into the world and play with the parameters for the enchantment effects in order to discover a new effect that you like
  (Utilities|FlowControl|Sequence
    (:then_0
      (Components|StaticMesh|SetStaticMesh (Variables|Default|GetMesh) (Variables|MRPGT|GetCustomStaticMesh))
      (Class|NiagaraFunctionLibrary|OverrideSystemUserVariableStaticMesh (Variables|Default|GetNiagaraSys) "User.StaticMesh" (Variables|MRPGT|GetCustomStaticMesh)))
    (:then_1
      (Niagara|SetNiagaraVariable(LinearColor) (Variables|Default|GetNiagaraSys) "User.EnchantmentColor1" (Variables|ParticleParams|GetEnchantmentColor1))
      (Niagara|SetNiagaraVariable(LinearColor) (Variables|Default|GetNiagaraSys) "User.EnchantmentColor2" (Variables|ParticleParams|GetEnchantmentColor2))
      (Niagara|SetNiagaraVariable(Float) (Variables|Default|GetNiagaraSys) "User.CurlNoiseStrength" (Variables|ParticleParams|GetCurlNoiseStrength))
      (Niagara|SetNiagaraVariable(Float) (Variables|Default|GetNiagaraSys) "User.CurlNoiseFrequency" (Variables|ParticleParams|GetCurlNoiseFrequency))
      (Niagara|SetNiagaraVariable(Float) (Variables|Default|GetNiagaraSys) "User.SpawnRate" (Variables|ParticleParams|GetSpawnRate))
      (Class|NiagaraComponent|SetNiagaraVariableVec3 (Variables|Default|GetNiagaraSys) "User.Acceleration" (Variables|ParticleParams|GetAcceleration))
      (Niagara|SetNiagaraVariable(Float) (Variables|Default|GetNiagaraSys) "User.RandomNoiseForceAmount" (Variables|ParticleParams|GetRandomNoiseForceAmount))
      (Niagara|SetNiagaraVariable(Float) (Variables|Default|GetNiagaraSys) "User.RandomNoiseTimeInterval" (Variables|ParticleParams|GetRandomNoiseTimeInterval)))
    (:then_2
      (Rendering|Material|SetVectorParameterValueonMaterials (Variables|Default|GetMesh) "EmissiveColor" (Math|Conversions|ToVector(LinearColor) (Variables|MaterialParams|GetEnchantmentColor3)))
      (Rendering|Material|SetScalarParameterValueonMaterials (Variables|Default|GetMesh) "Opacity" (Variables|MaterialParams|GetOpacity)))))

(event Collision|EventActorBeginOverlap
  (params (OtherActor :type Actor%20Object%20Reference))
  ;[1 1 1] The purpose of this blueprint is only for you to drag it into the world and play with the parameters for the enchantment effects in order to discover a new effect that you like
)

(event EventTick
  (params (DeltaSeconds :type Float%20%28single-precision%29))
  ;[1 1 1] The purpose of this blueprint is only for you to drag it into the world and play with the parameters for the enchantment effects in order to discover a new effect that you like
)

(fn ConstructionScript
  (Utilities|FlowControl|Sequence
    (:then_0
      (Components|StaticMesh|SetStaticMesh (Variables|Default|GetMesh) (Variables|MRPGT|GetCustomStaticMesh))
      (Class|NiagaraFunctionLibrary|OverrideSystemUserVariableStaticMesh (Variables|Default|GetNiagaraSys) "User.StaticMesh" (Variables|MRPGT|GetCustomStaticMesh)))
    (:then_1
      (Niagara|SetNiagaraVariable(LinearColor) (Variables|Default|GetNiagaraSys) "User.EnchantmentColor1" (Variables|ParticleParams|GetEnchantmentColor1))
      (Niagara|SetNiagaraVariable(LinearColor) (Variables|Default|GetNiagaraSys) "User.EnchantmentColor2" (Variables|ParticleParams|GetEnchantmentColor2))
      (Niagara|SetNiagaraVariable(Float) (Variables|Default|GetNiagaraSys) "User.CurlNoiseStrength" (Variables|ParticleParams|GetCurlNoiseStrength))
      (Niagara|SetNiagaraVariable(Float) (Variables|Default|GetNiagaraSys) "User.CurlNoiseFrequency" (Variables|ParticleParams|GetCurlNoiseFrequency))
      (Niagara|SetNiagaraVariable(Float) (Variables|Default|GetNiagaraSys) "User.SpawnRate" (Variables|ParticleParams|GetSpawnRate))
      (Class|NiagaraComponent|SetNiagaraVariableVec3 (Variables|Default|GetNiagaraSys) "User.Acceleration" (Variables|ParticleParams|GetAcceleration))
      (Niagara|SetNiagaraVariable(Float) (Variables|Default|GetNiagaraSys) "User.RandomNoiseForceAmount" (Variables|ParticleParams|GetRandomNoiseForceAmount))
      (Niagara|SetNiagaraVariable(Float) (Variables|Default|GetNiagaraSys) "User.RandomNoiseTimeInterval" (Variables|ParticleParams|GetRandomNoiseTimeInterval)))
    (:then_2
      (Rendering|Material|SetVectorParameterValueonMaterials (Variables|Default|GetMesh) "EmissiveColor" (Math|Conversions|ToVector(LinearColor) (Variables|MaterialParams|GetEnchantmentColor3)))
      (Rendering|Material|SetScalarParameterValueonMaterials (Variables|Default|GetMesh) "Opacity" (Variables|MaterialParams|GetOpacity)))))