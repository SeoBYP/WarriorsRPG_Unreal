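; Trader NPC that lets the player buy and sell items through a trading menu and doubles as an item container.
; On interaction, a looping timer polls until dialogue ends, then opens the trader UI if no other UI is open and inventory is initialized.
; Stock is recorded in the SaveGame by unique ID on that opening and on inventory changes, so it persists across loads.
; Trader gold lives in the NPC info struct, with functions to check affordability and adjust it.
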(event Custom|CheckDialogueEnded
  ;[1 1 1] Open trading UI (player trades with the NPC Trader which has an item container functionality)
  (if (not (Variables|/Game/MRPGT/Blueprints/GameInstance/BP_MRPGT_GameInstance.BP_MRPGT_GameInstance_C|GetIsDialogueMenuOpen (Variables|Default|GetGameInstance)))
    (Utilities|Time|ClearandInvalidateTimerbyHandle (Variables|MRPGT|ReferenceOnly|GetCheckDialogueEndedHandle))
    (if (not (Default|IsAnyUIOpen (Variables|Default|GetGameInstance)))
      (if (Variables|Default|GetInventoryInitialized)
        (CallFunction|OpenTradingUI)
        ;[1 1 1] Once you interact with an NPC Trader and see what they have in stock you want to see the same stock the next time you interact with them, even if you save the game and come back another day, so here we add this NPC to the SaveGame so that if the game is saved then loaded at a later point in time, the trader has the same items as during the previous interaction with him/her
        (Default|AddChangedContainer (Variables|/Game/MRPGT/Blueprints/GameInstance/BP_MRPGT_GameInstance.BP_MRPGT_GameInstance_C|GetSavedGame (Variables|Default|GetGameInstance)) (Variables|Default|GetUniqueID) (Variables|Default|GetNPCItems))))))

(event EventInteract
  (params (HitComponent :type Actor%20Component%20Object%20Reference) (InteractingActor :type Actor%20Object%20Reference))
  ;[1 1 1] Open trading UI (player trades with the NPC Trader which has an item container functionality)
  (|CallParentFunction 0 0)
  (bind _returnvalue (Utilities|Time|SetTimerbyEvent (delegate Custom|CheckDialogueEnded) 0.1 true))
  (Variables|MRPGT|ReferenceOnly|SetCheckDialogueEndedHandle _returnvalue))

(event Collision|EventActorBeginOverlap
  (params (OtherActor :type Actor%20Object%20Reference)))

(event EventTick
  (params (DeltaSeconds :type Float%20%28single-precision%29)))

(event EventBeginPlay
  (|CallParentFunction) ; This node is disabled and will not be called.\nDrag off pins to build functionality.
)

(event EventSetInventory
  (params (InventoryIn :type Array%20of%20Item%20Struct%20Structures))
  ;[1 1 1] Here we implemented the SetInventory function for Container interface. When the Container inventory has changed (the player may have taken some or all items out of the container) then make a note of this in the SaveGame object
  (Variables|Default|SetNPCItems InventoryIn)
  (Default|AddChangedContainer (Variables|/Game/MRPGT/Blueprints/GameInstance/BP_MRPGT_GameInstance.BP_MRPGT_GameInstance_C|GetSavedGame (Variables|Default|GetGameInstance)) (Variables|Default|GetUniqueID) (Variables|Default|GetNPCItems)))

(event EventAddGold
  (params (Amount :type Integer))
  (bind _structout (Utilities|Struct|SetmembersinNPCStruct1 (Variables|Default|GetNPCInfo) (+ (.Gold (Utilities|Struct|BreakNPCStruct1 (Variables|Default|GetNPCInfo))) Amount)))
  (Variables|Default|SetNPCInfo _structout))

(event EventDeductGold
  (params (Amount :type Integer))
  (bind _structout (Utilities|Struct|SetmembersinNPCStruct1 (Variables|Default|GetNPCInfo) (- (.Gold (Utilities|Struct|BreakNPCStruct1 (Variables|Default|GetNPCInfo))) Amount)))
  (Variables|Default|SetNPCInfo _structout))

(event EventInitializeTrading
  (params (HideEquippedItems :type Boolean))
  (CallFunction|OpenTradingUI))

(fn ConstructionScript
  (|CallParentFunction))

(fn AddGoldtoTraderforItem
  (params (ItemSold :type Item%20Struct%20Structure))
  (bind _structout (Utilities|Struct|SetmembersinNPCStruct1 (Variables|Default|GetNPCInfo) (+ (.Gold (Utilities|Struct|BreakNPCStruct1 (Variables|Default|GetNPCInfo))) (.UnitValue (Utilities|Struct|BreakItemStruct ItemSold)))))
  (Variables|Default|SetNPCInfo _structout))

(fn DeductGoldfromTraderforItem
  (params (ItemBought :type Item%20Struct%20Structure))
  (bind _structout (Utilities|Struct|SetmembersinNPCStruct1 (Variables|Default|GetNPCInfo) (- (.Gold (Utilities|Struct|BreakNPCStruct1 (Variables|Default|GetNPCInfo))) (.UnitValue (Utilities|Struct|BreakItemStruct ItemBought)))))
  (Variables|Default|SetNPCInfo _structout))

(fn CanBuyItem
  (params (ItemIn :type Item%20Struct%20Structure))
  (return (>= (.Gold (Utilities|Struct|BreakNPCStruct1 (Variables|Default|GetNPCInfo))) (.UnitValue (Utilities|Struct|BreakItemStruct ItemIn)))))

(fn GetInventory
  (return (Variables|Default|GetNPCItems)))

(fn OpenTradingUI
  (Default|OpenTraderMenu (Variables|Default|GetPlayerController) false)
  (Default|LoadTraderInventory0 (Variables|/Game/MRPGT/Blueprints/Controllers/BP_InGamePlayerController.BP_InGamePlayerController_C|GetItemMainWidget (Variables|Default|GetPlayerController)) self)
  (Default|UpdateNavigationAppearance (Variables|/Game/MRPGT/Blueprints/Controllers/BP_InGamePlayerController.BP_InGamePlayerController_C|GetItemMainWidget (Variables|Default|GetPlayerController)))
  (Class|InterfaceGeneralCharacter|SetIsInteractingwithObject(Message) (Game|GetPlayerCharacter 0) true))

(fn GetGold
  (return (.Gold (Utilities|Struct|BreakNPCStruct1 (Variables|Default|GetNPCInfo)))))

(fn GetNPCInfo
  (return ""))