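; Quest-giver NPC that offers the player a quest when interacted with, provided no other UI is open.
; On first interaction it caches GameInstance WorldQuests whose start NPC matches its ID.
; GetApplicableQuest returns the first listed quest already in the player's progress (started, completed, finished or failed) or meeting the level requirement.
; That quest opens the quest-giver HUD; otherwise a localized "no quests available" message appears.
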(event EventBeginPlay
  (|CallParentFunction) ; This node is disabled and will not be called.\nDrag off pins to build functionality.
)

(event Collision|EventActorBeginOverlap
  (params (OtherActor :type Actor%20Object%20Reference)))

(event EventTick
  (params (DeltaSeconds :type Float%20%28single-precision%29)))

(event EventInteract
  (params (HitComponent :type Actor%20Component%20Object%20Reference) (InteractingActor :type Actor%20Object%20Reference))
  (bind _questout (CallFunction|GetApplicableQuest))
  ;[1 1 1] If the other menus arent currently open
  (if (not (Default|IsAnyUIOpen (Variables|Default|GetGameInstance)))
    (if (Variables|MRPGT|GetAreQuestsInitialized)
      _
      (else
        (CallFunction|InitializeQuests)))
    (|CallParentFunction 0 0)
    (if (not (Utilities|Enum|Equal(Enum) (Utilities|Struct|BreakQuestStruct _questout) "UNSET"))
      (if (not (Variables|/Game/MRPGT/Blueprints/GameInstance/BP_MRPGT_GameInstance.BP_MRPGT_GameInstance_C|GetIsQuestMenuOpen (Variables|Default|GetGameInstance)))
        (Default|OpenQuestGiverHUD (Variables|Default|GetPlayerController) _questout self))
      (else
        (Default|SendMessagetoScreen (Variables|/Game/MRPGT/Blueprints/Controllers/BP_InGamePlayerController.BP_InGamePlayerController_C|GetMessagesWidget (Variables|Default|GetPlayerController)) (.OutText (Class|KismetTextLibrary|FindTextinLocalizationTable "Messages" "NoQuestsAvailable")) "NewEnumerator0")))))

(fn ConstructionScript
  (|CallParentFunction))

(fn InitializeQuests
  ;[1 1 1] Get all quests for this NPC from the WorldQuests array and add them to the Quests array within this NPC object
  (for _array_element (Variables|/Game/MRPGT/Blueprints/GameInstance/BP_MRPGT_GameInstance.BP_MRPGT_GameInstance_C|GetWorldQuests (Variables|Default|GetGameInstance))
    (if (Utilities|Enum|Equal(Enum) (.StartNPCID (Utilities|Struct|BreakQuestStruct _array_element)) (.ID (Utilities|Struct|BreakNPCStruct1 (Variables|Default|GetNPCInfo))))
      (Utilities|Array|Add (Variables|MRPGT|GetNPCQuests) _array_element)))
  (Variables|MRPGT|SetAreQuestsInitialized true))

(fn GetApplicableQuest
  (bind _playercontroller (Variables|Default|GetPlayerController))
  ;[1 1 1] Get the most applicable quest from this NPC. It will either be a) the first already started, completed, finished or failed quest from the CharactersQuests array that has a StartingNPCID matching that of this NPC or b) the first unstarted quest from the NPCQuests array
  (for _array_element (Variables|MRPGT|GetNPCQuests)
    (LocalVariables|SetLocalQuest _array_element)
    (if (Math|Boolean|ORBoolean (Default|IsQuestStarted _playercontroller (.ID (Utilities|Struct|BreakQuestStruct (LocalVariables|GetLocalQuest)))) (Default|IsQuestCompleted _playercontroller (.ID (Utilities|Struct|BreakQuestStruct (LocalVariables|GetLocalQuest)))) (Default|IsQuestFinished _playercontroller (.ID (Utilities|Struct|BreakQuestStruct (LocalVariables|GetLocalQuest)))) (Default|IsQuestFailed _playercontroller (.ID (Utilities|Struct|BreakQuestStruct (LocalVariables|GetLocalQuest))))) ; Return the quest that the player has already started or completed for this NPC to make it finish that one first
      (return (Default|GetQuestbyQuestID (Variables|Default|GetPlayerController) (.ID (Utilities|Struct|BreakQuestStruct (LocalVariables|GetLocalQuest)))))
      (elif (>= (Utilities|Struct|BreakCharacterStruct (Variables|/Game/MRPGT/Blueprints/Controllers/BP_InGamePlayerController.BP_InGamePlayerController_C|GetCharacterInfo (Variables|Default|GetPlayerController))) (.MinimumCharacterLevel (Utilities|Struct|BreakQuestStruct (LocalVariables|GetLocalQuest)))) ; Return the first quest that the player can do for this NPC
        (return (LocalVariables|GetLocalQuest)))))
  (return "") ; If none of the quests that this NPC has can be done by the player then return UNSET which means that the NPC has no valid quests for the player
)