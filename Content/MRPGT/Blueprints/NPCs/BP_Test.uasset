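; Test actor in the NPCs folder that classifies which side of itself the player is on, every Tick.
; It dots the normalized direction to the player with its forward and right vectors.
; Forward thresholds separate front and back, the right dot's sign splits the sides, and nested selects pick a side enum name.
; The resulting message goes to a keyed PrintString with screen and log output both disabled.
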(event EventBeginPlay)

(event Collision|EventActorBeginOverlap
  (params (OtherActor :type Actor%20Object%20Reference)))

(event EventTick
  (params (DeltaSeconds :type Float%20%28single-precision%29))
  (Variables|Default|SetForwardDotProduct (Math|Vector|DotProduct (Math|Vector|Normalize (- (Transformation|GetActorLocation (Game|GetPlayerCharacter 0)) (Transformation|GetActorLocation self))) (Transformation|GetActorForwardVector)))
  (Variables|Default|SetRightDotProduct (Math|Vector|DotProduct (Math|Vector|Normalize (- (Transformation|GetActorLocation (Game|GetPlayerCharacter 0)) (Transformation|GetActorLocation self))) (Transformation|GetActorRightVector)))
  (Development|PrintString (Utilities|String|Append "Player is to the " (Utilities|String|SelectString (Utilities|String|EnumtoString (Utilities|Enum|LiteralenumSideEnum "NewEnumerator0")) (Utilities|String|SelectString (Utilities|String|EnumtoString (Utilities|Enum|LiteralenumSideEnum "NewEnumerator3")) (Utilities|String|SelectString (Utilities|String|EnumtoString (Utilities|Enum|LiteralenumSideEnum "NewEnumerator1")) (Utilities|String|EnumtoString (Utilities|Enum|LiteralenumSideEnum "NewEnumerator2")) (< (Variables|Default|GetForwardDotProduct) -0.5)) (and (> (Variables|Default|GetForwardDotProduct) -0.5) (> (Variables|Default|GetRightDotProduct) 0.0))) (> (Variables|Default|GetForwardDotProduct) 0.5)) " of the BP_Test actor") false false "(R=0.000000,G=0.660000,B=1.000000,A=1.000000)" 2.0 "PlayerDirection"))

(fn ConstructionScript)