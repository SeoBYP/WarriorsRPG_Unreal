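; Actor component that makes its owner lockpickable and launches the lockpicking minigame.
; It turns a difficulty into a randomly placed sweet spot and surrounding proximity region, sized exponentially by level and clamped.
; On interaction it spawns BP_Minigame_Lockpicking below the owner, passes it those bounds, and updates its lockpick count HUD.
; On success it clears the locked flag and notifies the owner through message calls.
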(event Custom|Event%20Lockpicking
  (params (Interacting%20Actor :type Actor%20Object%20Reference))
  (bind _returnvalue (Components|GetOwner))
  (bind _returnvalue_2 (Transformation|GetActorLocation _returnvalue))
  ;[1 0.2578 0] Spawn Lockpicking Minigame
  (Utilities|IsValid Interacting%20Actor
    (:Is%20Valid
      (Variables|Mechanism|SetOwner _returnvalue)
      (bind _returnvalue_3 (Game|SpawnActorfromClass "/Game/MRPGT/Lockpicking_Minigame/Blueprints/BP_Minigame_Lockpicking.BP_Minigame_Lockpicking_C" (Math|Transform|MakeTransform (Math|Vector|MakeVector (.x _returnvalue_2) (.y _returnvalue_2) (- (.z _returnvalue_2) (Variables|UserDefined|GetSpawn_Location_Z))) "0.000000,0.000000,90.000000") "Undefined" "MultiplyWithRoot" (Variables|Mechanism|GetOwner) 0))
      (CallFunction|StoreLockSettings _returnvalue_3)
      (Class|InterfaceLockpickingCharacter|SetLockpickMinigame(Message) Interacting%20Actor _returnvalue_3)
      (Variables|/Game/MRPGT/Lockpicking_Minigame/Blueprints/BP_Minigame_Lockpicking.BP_Minigame_Lockpicking_C|SetAC_Owner _returnvalue_3 self)
      (bind _numlockpicks (Class|InterfaceInventory1|GetNumLockpicks(Message) (Game|GetPlayerController 0)))
      (Default|UpdateLockpickHUD _returnvalue_3 _numlockpicks)
      (Variables|Default|SetbLockpickingInProgress true))))

(event Custom|Event%20Generate%20Lock%20Settings
  (params (Lock%20Difficulty :type E_Lock_Difficulties%20Enum :default "NewEnumerator0"))
  ;[1 0 0.07031] Lock Settings Generation
  (Variables|Mechanism|SetDifficulty_Level (.Value (Utilities|Map|Find (Variables|UserDefined|GetDifficulty_Levels) Lock%20Difficulty)))
  (CallFunction|GenerateLockSettings))

(event Custom|Event%20Successful%20Lockpicking
  ;[0.7344 0 1] Successful Lockpicking
  (Game|AddComponentbyClass (Variables|Mechanism|GetOwner) "/Game/MRPGT/Lockpicking_Minigame/Blueprints/Actor_Components/AC_Lockpicking_Successful.AC_Lockpicking_Successful_C")
  (Variables|Default|SetbIsLocked false)
  (Class|InterfaceLockable|Unlocked(Message) (Variables|Mechanism|GetOwner)))

(fn GenerateLockSettings
  ;[1 0 0.4219] Lock Settings - Sweet Spot Size
  (Variables|Mechanism|SetSweet_Spot_Size (* (Math|Float|Clamp(Float) (* (Math|Float|Power (Variables|UserDefined|GetDifficulty_Multiplier) (Math|Conversions|ToFloat(Integer) (- (- (Utilities|Map|Length (Variables|UserDefined|GetDifficulty_Levels)) (Variables|Mechanism|GetDifficulty_Level)) 1))) (/ (Variables|UserDefined|GetSmallest_Sweet_Spot_%28%25%29) 1e+02)) (Variables|UserDefined|GetMin_Sweet_Spot_Size) (Variables|UserDefined|GetMax_Sweet_Spot_Size)) 1.8e+02))
  ;[0 1 0.25] Lock Settings - Sweet Spot Location
  (bind _output_get (Variables|Mechanism|SetSweet_Spot_Location (Math|Random|RandomFloatinRange -9e+01 9e+01)))
  ;[0.2422 0 1] Lock Settings - Sweet Spot Boundaries
  (Variables|Mechanism|SetSweet_Spot_LB (Math|Float|Clamp(Float) (- _output_get (/ (Variables|Mechanism|GetSweet_Spot_Size) 2.0)) -9e+01 9e+01))
  (Variables|Mechanism|SetSweet_Spot_UB (Math|Float|Clamp(Float) (+ _output_get (/ (Variables|Mechanism|GetSweet_Spot_Size) 2.0)) -9e+01 9e+01))
  ;[0 1 0.4375] Lock Settings - Proximity Region Boundaries
  (Variables|Mechanism|SetProximity_Region_LB (Math|Float|Clamp(Float) (- (Variables|Mechanism|GetSweet_Spot_LB) (* (Variables|Mechanism|GetSweet_Spot_Size) (Variables|UserDefined|GetProximity_Region_Multiplier))) -9e+01 9e+01))
  (Variables|Mechanism|SetProximity_Region_UB (Math|Float|Clamp(Float) (+ (Variables|Mechanism|GetSweet_Spot_UB) (* (Variables|Mechanism|GetSweet_Spot_Size) (Variables|UserDefined|GetProximity_Region_Multiplier))) -9e+01 9e+01)))

(fn StoreLockSettings
  (params (Lockpick%20Minigame :type BP%20Minigame%20Lockpicking%20Object%20Reference))
  (Utilities|FlowControl|Sequence
    (:then_0
      (Variables|/Game/MRPGT/Lockpicking_Minigame/Blueprints/BP_Minigame_Lockpicking.BP_Minigame_Lockpicking_C|SetSweet_Spot_LB Lockpick%20Minigame (Variables|Mechanism|GetSweet_Spot_LB)))
    (:then_1
      (Variables|/Game/MRPGT/Lockpicking_Minigame/Blueprints/BP_Minigame_Lockpicking.BP_Minigame_Lockpicking_C|SetSweet_Spot_UB Lockpick%20Minigame (Variables|Mechanism|GetSweet_Spot_UB)))
    (:then_2
      (Variables|/Game/MRPGT/Lockpicking_Minigame/Blueprints/BP_Minigame_Lockpicking.BP_Minigame_Lockpicking_C|SetProximity_Region_LB Lockpick%20Minigame (Variables|Mechanism|GetProximity_Region_LB)))
    (:then_3
      (Variables|/Game/MRPGT/Lockpicking_Minigame/Blueprints/BP_Minigame_Lockpicking.BP_Minigame_Lockpicking_C|SetProximity_Region_UB Lockpick%20Minigame (Variables|Mechanism|GetProximity_Region_UB)))))