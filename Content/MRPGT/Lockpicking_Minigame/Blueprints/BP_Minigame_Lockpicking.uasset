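; Lockpicking minigame actor that swaps input contexts, shows a HUD and renders only its own meshes through a scene capture to a render target.
; The pick's angle relative to a sweet spot and proximity region limits how far the lock turns; a full turn notifies the owning lockpicking component.
; Jamming starts looping timers for shake, sound, rumble and difficulty-scaled damage.
; Broken picks fly off with physics, then reset, until attempts run out.
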(event Custom|Event%20Lock
  (bind _reset_rotation_timeline (Variables|Default|GetReset%20Rotation%20Timeline))
  (bind _lockpick_01_pivot (Variables|Default|GetLockpick_01_Pivot))
  ;[1 1 1] Rotate Lock (Left)
  (Variables|Mechanism|SetControl_Continuous_Unlock false)
  (if (Variables|Mechanism|GetIsUnlocking)
    (Variables|Mechanism|SetIsLocking true)
    (Variables|Mechanism|SetIsUnlocking false)
    (CallFunction|StopLockpickingFeedback)
    (Variables|Mechanism|SetTemp%20Lockpick%20Rotation%20Z (.yaw (Variables|/Script/Engine.SceneComponent|GetRelativeRotation (Variables|Default|GetLockpick_01_Pivot))))
    (bind _output_get (Variables|Mechanism|SetCurrent%20Lock%20Rotation%20Z (.yaw (Variables|/Script/Engine.SceneComponent|GetRelativeRotation (Variables|Default|GetLock)))))
    (Components|Timeline|SetPlayRate _reset_rotation_timeline (/ (Components|Timeline|GetTimelineLength _reset_rotation_timeline) (/ (* _output_get (Variables|UserDefined|GetLock_Rotation_Time)) 9e+01)))
    (bind _alpha_for_rotation_z (Timeline|Reset%20Rotation%20Timeline PlayFromStart)
      (:Update
        (Transformation|SetRelativeRotation (Variables|Default|GetLock) (Math|Rotator|MakeRotator 0.0 0.0 (Math|Float|Lerp (Variables|Mechanism|GetCurrent%20Lock%20Rotation%20Z) 0.0 _alpha_for_rotation_z)) false false)
        (if (not (Variables|UserDefined|GetIs_LockPick_Rotating_With_Lock))
          (Transformation|SetRelativeRotation (Variables|Default|GetLockpick_01_Pivot) (Math|Rotator|MakeRotator 0.0 0.0 (Math|Float|Lerp (Variables|Mechanism|GetTemp%20Lockpick%20Rotation%20Z) (Variables|Mechanism|GetCurrent%20Lockpick%20Rotation%20Z) _alpha_for_rotation_z)) false false))
        (if (not (and (not (Variables|Mechanism|GetIsUnlocking)) (> (.yaw (Variables|/Script/Engine.SceneComponent|GetRelativeRotation (Variables|Default|GetLock))) 0.0)))
          (Timeline|Reset%20Rotation%20Timeline Stop)))
      (:Finished
        (Transformation|SetRelativeRotation (Variables|Default|GetLockpick_01_Pivot) (Math|Rotator|MakeRotator 0.0 0.0 (Variables|Mechanism|GetCurrent%20Lockpick%20Rotation%20Z)) false false)
        (Variables|Mechanism|SetIsLocking false)))
    (else
      (CallFunction|StopLockpickingFeedback)
      (Transformation|SetRelativeRotation _lockpick_01_pivot (Math|Rotator|MakeRotator 0.0 0.0 (.yaw (Variables|/Script/Engine.SceneComponent|GetRelativeRotation _lockpick_01_pivot))) false false))))

(event Custom|Event%20Rotate%20Lockpick
  (params (X-Axis%20Value :type Float%20%28double-precision%29))
  ;[1 0.9844 0] Rotate Lockpick
  (if (and (not (Variables|Mechanism|GetIsUnlocking)) (not (Variables|Mechanism|GetIsLocking)))
    (Transformation|SetRelativeRotation (Variables|Default|GetLockpick_01_Pivot) (Math|Rotator|MakeRotator 0.0 0.0 (Math|Float|Clamp(Float) (+ (* X-Axis%20Value (Variables|UserDefined|GetLockpick_Rotation_Speed)) (.yaw (Variables|/Script/Engine.SceneComponent|GetRelativeRotation (Variables|Default|GetLockpick_01_Pivot)))) -9e+01 9e+01)) false false)
    (Variables|Mechanism|SetCurrent%20Lockpick%20Rotation%20Z (.yaw (Variables|/Script/Engine.SceneComponent|GetRelativeRotation (Variables|Default|GetLockpick_01_Pivot))))))

(event Custom|Event%20Unlock
  (bind _unlock_rotation_speed (Variables|UserDefined|GetUnlock_Rotation_Speed))
  (bind _proximity_max_rotation (Variables|Mechanism|GetProximity_Max_Rotation))
  (bind _lock (Variables|Default|GetLock))
  (bind _current_lockpick_rotation_z (Variables|Mechanism|GetCurrent%20Lockpick%20Rotation%20Z))
  (bind _returnvalue (* _proximity_max_rotation 9e+01))
  (bind _relativerotation (Variables|/Script/Engine.SceneComponent|GetRelativeRotation _lock))
  (bind _returnvalue_2 (+ _unlock_rotation_speed (.yaw _relativerotation)))
  (bind _returnvalue_3 (/ _returnvalue_2 _returnvalue))
  (bind _returnvalue_4 (Math|Float|Clamp(Float) _returnvalue_3))
  (bind _returnvalue_5 (Math|Float|Lerp 0.0 _returnvalue _returnvalue_4))
  ;[0.4766 1 0] Rotate Lock (Right)
  (Variables|Mechanism|SetControl_Continuous_Unlock true)
  (Variables|Mechanism|SetIsUnlocking true)
  (CallFunction|DetermineMaximumUnlockRotation)
  (if (> (Variables|Mechanism|GetProximity_Max_Rotation) 0.0)
    (Transformation|SetRelativeRotation (Variables|Default|GetLock) (Math|Rotator|MakeRotator 0.0 0.0 _returnvalue_5) false false)
    (if (not (Variables|UserDefined|GetIs_LockPick_Rotating_With_Lock))
      (Transformation|SetRelativeRotation (Variables|Default|GetLockpick_01_Pivot) (Math|Rotator|MakeRotator 0.0 0.0 (Math|Float|Lerp _current_lockpick_rotation_z (- _current_lockpick_rotation_z 9e+01) (/ (.yaw (Variables|/Script/Engine.SceneComponent|GetRelativeRotation (Variables|Default|GetLock))) 9e+01))) false false))
    (if (and (== (Variables|Mechanism|GetProximity_Max_Rotation) 1.0) (== _returnvalue_5 9e+01))
      (CallFunction|EventSuccessfulLockpicking)
      (elif (== _returnvalue_4 1.0)
        (CallFunction|EventLockpickingFeedback)))
    (else
      (Variables|Mechanism|SetIsUnlocking false)
      (CallFunction|EventLockpickingFeedback))))

(event Custom|Event%20Successful%20Lockpicking
  ;[1 0.8438 0] Successful Lockpicking
  (Default|EventSuccessfulLockpicking (Variables|Mechanism|GetAC_Owner))
  (CallFunction|EventInterruptLockpicking)
  (Variables|Mechanism|SetControl_Continuous_Unlock false))

(event Custom|Event%20Interrupt%20Lockpicking
  (bind _returnvalue (Game|GetPlayerController 0))
  (bind _returnvalue_2 (PlayerController|LocalPlayerSubsystems|GetEnhancedInputLocalPlayerSubsystem _returnvalue))
  ;[0.4531 1 0] Interrupt Lockpicking
  (Utilities|IsValid _returnvalue_2
    (:Is%20Valid
      (Input|RemoveMappingContext _returnvalue_2 (Variables|UserDefined|GetLockpick_Controls) "(bIgnoreAllPressedKeysUntilRelease=True,bForceImmediately=False,bNotifyUserSettings=False)")
      (Input|AddMappingContext _returnvalue_2 (Variables|UserDefined|GetPlayer_Default_Controls) 0 "(bIgnoreAllPressedKeysUntilRelease=True,bForceImmediately=False,bNotifyUserSettings=False)")
      (Widget|RemovefromParent (Variables|Mechanism|GetLockpick_Hud))
      (Variables|/Game/MRPGT/Lockpicking_Minigame/Blueprints/Actor_Components/AC_Lockpicking.AC_Lockpicking_C|SetbLockpickingInProgress (Actor|GetComponentbyClass (Components|GetOwner) "/Game/MRPGT/Lockpicking_Minigame/Blueprints/Actor_Components/AC_Lockpicking.AC_Lockpicking_C") false)
      (Utilities|IsValid self
        (:Is%20Valid
          (CallFunction|StopLockpickingFeedback)
          (Actor|DestroyActor)
          (Variables|Mechanism|SetControl_Continuous_Unlock false))))))

(event Custom|Event%20Lockpicking%20Feedback
  ;[1 0.6094 0] Feedback Lockpicking
  (Game|Feedback|ClientPlayForceFeedback (Game|GetPlayerController 0) "/Game/MRPGT/Lockpicking_Minigame/Feedback_Effects/FFE_Lockpicking.FFE_Lockpicking" "None" true false false)
  (if (not (Class|KismetSystemLibrary|TimerExists 0 "Shake Meshes"))
    (Utilities|Time|SetTimerbyFunctionName 0 "Shake Meshes" 0.025 true)
    (Utilities|Time|SetTimerbyFunctionName 0 "Damage Lockpick" 0.1 true)
    (Utilities|Time|SetTimerbyFunctionName 0 "Lockpick Feedback Sound" 0.085 true)))

(event Custom|Update%20Lockpick%20HUD
  (params (Number_Attempts :type Integer))
  ;[1 0 0.3516] Update Lockpick HUD information (e.g., lock difficulty)
  (Default|EventUpdateLockpickData (Variables|Mechanism|GetLockpick_Hud) (Variables|/Game/MRPGT/Lockpicking_Minigame/Blueprints/Actor_Components/AC_Lockpicking.AC_Lockpicking_C|GetDifficulty_Level (Variables|Mechanism|GetAC_Owner)) Number_Attempts))

(event Custom|Event%20Break%20Lockpick
  (bind _returnvalue (Game|GetPlayerController 0))
  (bind _returnvalue_2 (Game|GetPlayerController 0))
  (bind _returnvalue_3 (Math|Random|RandomFloatinRange 4e+01 6e+01))
  (bind _lockpick_01_top (Variables|Default|GetLockpick_01_Top))
  (bind _returnvalue_4 (PlayerController|LocalPlayerSubsystems|GetEnhancedInputLocalPlayerSubsystem _returnvalue_2))
  (bind _returnvalue_5 (PlayerController|LocalPlayerSubsystems|GetEnhancedInputLocalPlayerSubsystem _returnvalue))
  ;[0.1016 1 0] Remove Lockpick control, stop Lockpick feedback and reset Lock rotation
  (Utilities|IsValid _returnvalue_5
    (:Is%20Valid
      (Input|RemoveMappingContext _returnvalue_5 (Variables|UserDefined|GetLockpick_Controls) "(bIgnoreAllPressedKeysUntilRelease=True,bForceImmediately=False,bNotifyUserSettings=False)")
      (CallFunction|StopLockpickingFeedback)
      (CallFunction|EventLock)
      ;[0.4062 0 1] Apply Physics to broken Lockpick part
      (if (< (Variables|Mechanism|GetCurrent%20Lockpick%20Rotation%20Z) 0.0)
        (Variables|Mechanism|SetImpulse_Towards_Side (* -1.0 _returnvalue_3))
        (else
          (Variables|Mechanism|SetImpulse_Towards_Side _returnvalue_3)))
      (Physics|SetSimulatePhysics _lockpick_01_top true)
      (Physics|AddImpulse _lockpick_01_top (Math|Vector|MakeVector (Variables|Mechanism|GetImpulse_Towards_Side) (Math|Random|RandomFloatinRange 5e+01 75.0) (Math|Random|RandomFloatinRange 75.0 1e+02)) "None" true)
      (Class|PrimitiveComponent|AddAngularImpulseinDegrees (Variables|Default|GetLockpick_01_Top) (Math|Vector|MakeVector (Math|Random|RandomFloatinRange 6e+02 1e+03) 2.5e+02 5e+02) "None" true)
      ;[1 0 0.8437] Play breaking sound
      (Audio|PlaySound2D (Variables|Mechanism|GetLockpick_Break_Sound) 1.0 1.0 0.0 0 0)
      ;[0 1 0.3871] Timer to reset Lockpick
      (Utilities|FlowControl|Delay (Variables|UserDefined|GetBroken_Lockpick_Wait_Timer))
      ;[0 0.3672 1] Reset broken pockpick part location and rotation
      (Physics|SetSimulatePhysics (Variables|Default|GetLockpick_01_Top) false)
      (Transformation|AttachComponentToComponent (Variables|Default|GetLockpick_01_Top) (Variables|Default|GetLockpick_01_Pivot) "None" "SnapToTarget" "SnapToTarget" "KeepRelative" false)
      (Transformation|SetRelativeTransform (Variables|Default|GetLockpick_01_Top) (Variables|Mechanism|GetLockpick_01_Top_Base_Transform) false false)
      (Transformation|SetRelativeRotation (Variables|Default|GetLockpick_01_Pivot) "0, 0, 0" false false)
      (Variables|Mechanism|SetCurrent%20Lockpick%20Rotation%20Z 0.0)
      ;[1 0.4003 0.572] Add back Lockpick control
      (Variables|Mechanism|SetControl_Continuous_Unlock false)
      (Utilities|IsValid _returnvalue_4
        (:Is%20Valid
          (Input|AddMappingContext _returnvalue_4 (Variables|UserDefined|GetLockpick_Controls) 0 "(bIgnoreAllPressedKeysUntilRelease=True,bForceImmediately=False,bNotifyUserSettings=False)"))))))

(event EventBeginPlay
  (bind _returnvalue (Game|GetPlayerController 0))
  (bind _returnvalue_2 (PlayerController|LocalPlayerSubsystems|GetEnhancedInputLocalPlayerSubsystem _returnvalue))
  ;[1 0.265 0.1352] Change Player's Controls
  (Utilities|IsValid _returnvalue_2
    (:Is%20Valid
      (Input|RemoveMappingContext _returnvalue_2 (Variables|UserDefined|GetPlayer_Default_Controls) "(bIgnoreAllPressedKeysUntilRelease=True,bForceImmediately=False,bNotifyUserSettings=False)")
      (Input|AddMappingContext _returnvalue_2 (Variables|UserDefined|GetLockpick_Controls) 1 "(bIgnoreAllPressedKeysUntilRelease=True,bForceImmediately=False,bNotifyUserSettings=False)")
      ;[0 0.1562 1] Show lockpick minigame in Viewport
      (bind _returnvalue_3 (UserInterface|CreateWidget "/Game/MRPGT/Lockpicking_Minigame/Blueprints/Widget/WBP_Minigame_Lockpicking.WBP_Minigame_Lockpicking_C"))
      (bind _output_get (Variables|Mechanism|SetLockpick_Hud _returnvalue_3))
      (UserInterface|Viewport|AddtoViewport _output_get 0)
      ;[1 0 0.7031] Restrict rendering to Actor Components in this BP
      (Rendering|SceneCapture|ShowOnlyActorComponents (Variables|Default|GetSceneCaptureComponent2D) self false))))

(fn ConstructionScript
  (Utilities|FlowControl|Sequence
    (:then_0
      ;[0.2188 0 1] Texture Render Target - Camera
      (bind _returnvalue (Utilities|LoadAssetBlocking (Variables|UserDefined|GetSoft_Camera)))
      (bind _astexture_render_target_2d (Utilities|Casting|CastToTextureRenderTarget2D _returnvalue))
      (Variables|/Script/Engine.SceneCaptureComponent2D|SetTextureTarget (Variables|Default|GetSceneCaptureComponent2D) _astexture_render_target_2d))
    (:then_1
      ;[0.9453 0 1] Mesh - Housing
      (bind _returnvalue_2 (Utilities|LoadAssetBlocking (Variables|UserDefined|GetSoft_Mesh_Housing)))
      (bind _asstatic_mesh (Utilities|Casting|CastToStaticMesh _returnvalue_2))
      (Components|StaticMesh|SetStaticMesh (Variables|Default|GetHousing) _asstatic_mesh))
    (:then_2
      ;[0 0.7187 1] Mesh - Lock
      (bind _returnvalue_3 (Utilities|LoadAssetBlocking (Variables|UserDefined|GetSoft_Mesh_Lock)))
      (bind _asstatic_mesh_2 (Utilities|Casting|CastToStaticMesh _returnvalue_3))
      (Components|StaticMesh|SetStaticMesh (Variables|Default|GetLock) _asstatic_mesh_2))
    (:then_3
      ;[1 0 0.2344] Mesh - Lockpick 01 (Bottom)
      (bind _returnvalue_4 (Utilities|LoadAssetBlocking (Variables|UserDefined|GetSoft_Mesh_Lockpick_01_Bottom)))
      (bind _asstatic_mesh_3 (Utilities|Casting|CastToStaticMesh _returnvalue_4))
      (Components|StaticMesh|SetStaticMesh (Variables|Default|GetLockpick_01_Bottom) _asstatic_mesh_3))
    (:then_4
      ;[1 1 1] Mesh - Lockpick 01 (Top)
      (bind _returnvalue_5 (Utilities|LoadAssetBlocking (Variables|UserDefined|GetSoft_Mesh_Lockpick_01_Top)))
      (bind _asstatic_mesh_4 (Utilities|Casting|CastToStaticMesh _returnvalue_5))
      (Components|StaticMesh|SetStaticMesh (Variables|Default|GetLockpick_01_Top) _asstatic_mesh_4)
      (Variables|Mechanism|SetLockpick_01_Top_Base_Transform (Transformation|GetRelativeTransform (Variables|Default|GetLockpick_01_Top))))
    (:then_5
      ;[0.4766 0 1] Mesh - Lockpick 02
      (bind _returnvalue_6 (Utilities|LoadAssetBlocking (Variables|UserDefined|GetSoft_Mesh_Lockpick_02)))
      (bind _asstatic_mesh_5 (Utilities|Casting|CastToStaticMesh _returnvalue_6))
      (Components|StaticMesh|SetStaticMesh (Variables|Default|GetLockpick_02) _asstatic_mesh_5))
    (:then_6
      ;[0 1 0.6953] Sound - Lockpick feedback
      (bind _returnvalue_7 (Utilities|LoadAssetBlocking (Variables|UserDefined|GetSoft_Lockpick_Feedback_Sound)))
      (bind _assound_base (Utilities|Casting|CastToSoundBase _returnvalue_7))
      (Variables|Mechanism|SetLockpick_Feedback_Sound _assound_base))
    (:then_7
      ;[0.9997 1 0] Sound - Lockpick break
      (bind _returnvalue_8 (Utilities|LoadAssetBlocking (Variables|UserDefined|GetSoft_Lockpick_Break_Sound)))
      (bind _assound_base_2 (Utilities|Casting|CastToSoundBase _returnvalue_8))
      (Variables|Mechanism|SetLockpick_Break_Sound _assound_base_2))))

(fn DamageLockpick
  ;[0 1 0.3672] Check Lockpick Health after Damage
  (bind _lockpickhealth (Class|InterfaceInventory1|GetLockpickHealth(Message) (Game|GetPlayerController 0)))
  (if (<= (- _lockpickhealth (* (Variables|UserDefined|GetLockpick_Damage) (+ (Variables|/Game/MRPGT/Lockpicking_Minigame/Blueprints/Actor_Components/AC_Lockpicking.AC_Lockpicking_C|GetDifficulty_Level (Variables|Mechanism|GetAC_Owner)) 1))) 0.0)
    ;[0.03125 1 0] Reduce Player's Amount of Lockpicks / Attempts
    (Class|InterfaceInventory1|DestroyLockpick(Message) (Game|GetPlayerController 0))
    (bind _numlockpicks (Class|InterfaceInventory1|GetNumLockpicks(Message) (Game|GetPlayerController 0)))
    (if (<= _numlockpicks 0)
      (CallFunction|EventBreakLockpick)
      ;[0 0.4609 1] Player ran out of Lockpicks / Attempts
      (CallFunction|EventInterruptLockpicking)
      (else
        ;[0 1 0.1094] Refresh HUD
        (CallFunction|UpdateLockpickHUD _numlockpicks)
        (CallFunction|EventBreakLockpick)))
    ;[0.7813 0 1] Reset Lockpick's health
    (Class|InterfaceInventory1|SetLockpickHealth(Message) (Game|GetPlayerController 0) 1e+02)
    (else
      ;[1 0.5391 0] Define Lockpick New Health
      (Class|InterfaceInventory1|SetLockpickHealth(Message) (Game|GetPlayerController 0) (Math|Float|Clamp(Float) (- _lockpickhealth (* (Variables|UserDefined|GetLockpick_Damage) (+ (Variables|/Game/MRPGT/Lockpicking_Minigame/Blueprints/Actor_Components/AC_Lockpicking.AC_Lockpicking_C|GetDifficulty_Level (Variables|Mechanism|GetAC_Owner)) 1))) 0.0 1e+02)))))

(fn DetermineDistancetoSweetSpot
  (params (Lockpick%20Rotation%20Z :type Float%20%28double-precision%29) (Sweet%20Spot%20Bound :type Float%20%28double-precision%29) (Proximity%20Region%20Bound :type Float%20%28double-precision%29))
  (return (- 1.0 (/ (Math|Float|Absolute(Float) (- Lockpick%20Rotation%20Z Sweet%20Spot%20Bound)) (Math|Float|Absolute(Float) (- Sweet%20Spot%20Bound Proximity%20Region%20Bound))))))

(fn DetermineMaximumUnlockRotation
  (if (and (>= (Variables|Mechanism|GetCurrent%20Lockpick%20Rotation%20Z) (Variables|Mechanism|GetProximity_Region_LB)) (< (Variables|Mechanism|GetCurrent%20Lockpick%20Rotation%20Z) (Variables|Mechanism|GetSweet_Spot_LB)))
    ;[0 1 0.1094] Within Proximity Region (Left)
    (Variables|Mechanism|SetProximity_Max_Rotation (CallFunction|DetermineDistancetoSweetSpot (Variables|Mechanism|GetCurrent%20Lockpick%20Rotation%20Z) (Variables|Mechanism|GetSweet_Spot_LB) (Variables|Mechanism|GetProximity_Region_LB)))
    (elif (and (<= (Variables|Mechanism|GetCurrent%20Lockpick%20Rotation%20Z) (Variables|Mechanism|GetProximity_Region_UB)) (> (Variables|Mechanism|GetCurrent%20Lockpick%20Rotation%20Z) (Variables|Mechanism|GetSweet_Spot_UB)))
      ;[0 1 0.3672] Within Proximity Region (Right)
      (Variables|Mechanism|SetProximity_Max_Rotation (CallFunction|DetermineDistancetoSweetSpot (Variables|Mechanism|GetCurrent%20Lockpick%20Rotation%20Z) (Variables|Mechanism|GetSweet_Spot_UB) (Variables|Mechanism|GetProximity_Region_UB)))
      (elif (and (<= (Variables|Mechanism|GetCurrent%20Lockpick%20Rotation%20Z) (Variables|Mechanism|GetSweet_Spot_UB)) (>= (Variables|Mechanism|GetCurrent%20Lockpick%20Rotation%20Z) (Variables|Mechanism|GetSweet_Spot_LB)))
        ;[0.3359 1 0] Within Sweet Spot
        (Variables|Mechanism|SetProximity_Max_Rotation 1.0)
        (else
          ;[1 0 0.375] Outside Proximity Region and Sweet Spot
          (Variables|Mechanism|SetProximity_Max_Rotation 0.0))))))

(fn LockpickFeedbackSound
  (Audio|PlaySound2D (Variables|Mechanism|GetLockpick_Feedback_Sound) 1.0 1.0 0.0 0 0))

(fn ShakeMeshes
  (bind _shake_mesh_max (Variables|UserDefined|GetShake_Mesh_Max))
  (bind _lockpick_01_pivot (Variables|Default|GetLockpick_01_Pivot))
  (bind _shake_mesh_min (Variables|UserDefined|GetShake_Mesh_Min))
  (bind _shake_mesh_max_2 (Variables|UserDefined|GetShake_Mesh_Max))
  (bind _shake_mesh_min_2 (Variables|UserDefined|GetShake_Mesh_Min))
  (bind _returnvalue (Math|Random|RandomFloatinRange _shake_mesh_min_2 _shake_mesh_max))
  (bind _returnvalue_2 (Math|Random|RandomFloatinRange _shake_mesh_min _shake_mesh_max_2))
  (bind _relativerotation (Variables|/Script/Engine.SceneComponent|GetRelativeRotation _lockpick_01_pivot))
  ;[0 1 0.6484] Rotation - X-axis
  (if (Math|Random|RandomBool)
    (LocalVariables|SetShake_X_axis _returnvalue)
    (else
      (LocalVariables|SetShake_X_axis (* _returnvalue -1.0))))
  ;[1 0.3281 0] Rotation - Y-axis
  (if (Math|Random|RandomBool)
    (LocalVariables|SetShake_Y_axis _returnvalue_2)
    (else
      (LocalVariables|SetShake_Y_axis (* _returnvalue_2 -1.0))))
  ;[0 0.1797 1] Rotation - Mesh
  (Transformation|SetRelativeRotation _lockpick_01_pivot (Math|Rotator|MakeRotator (Math|Float|Clamp(Float) (+ (LocalVariables|GetShake_X_axis) (.roll _relativerotation)) -5.0 5.0) (Math|Float|Clamp(Float) (+ (.pitch _relativerotation) (LocalVariables|GetShake_Y_axis)) -5.0 5.0) (.yaw _relativerotation)) false false))

(fn StopLockpickingFeedback
  (Game|Feedback|ClientStopForceFeedback (Game|GetPlayerController 0) "/Game/MRPGT/Lockpicking_Minigame/Feedback_Effects/FFE_Lockpicking.FFE_Lockpicking" "None")
  (Utilities|Time|ClearTimerbyFunctionName 0 "Shake Meshes")
  (Utilities|Time|ClearTimerbyFunctionName 0 "Damage Lockpick")
  (Utilities|Time|ClearTimerbyFunctionName 0 "Lockpick Feedback Sound"))