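; Interactable door for the lockpicking minigame that can be locked, picked and toggled open or closed.
; Interacting with a locked, pickable door checks the player's lockpick count, then starts AC_Lockpicking, or unlocks if an AC_Lockpicking_Successful marker component exists.
; A timeline swings the door with sounds, and the construction script synchronously loads soft-referenced meshes and sounds.
; ResetLock relocks with random difficulty, and GetObjectName supplies lock-status text.
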(event Custom|Event%20Inspect%20Door
  (bind _returnvalue (Actor|GetComponentbyClass "/Game/MRPGT/Lockpicking_Minigame/Blueprints/Actor_Components/AC_Lockpicking_Successful.AC_Lockpicking_Successful_C"))
  (bind _returnvalue_2 (Actor|GetComponentbyClass "/Game/MRPGT/Lockpicking_Minigame/Blueprints/Actor_Components/AC_Lockpicking.AC_Lockpicking_C"))
  ;[0 1 0.7422] Check if the door is locked
  (if (not (Variables|UserDefined|GetIsLocked))
    (CallFunction|EventOpenDoor :!label _label)
    (else
      ;[0 0.3203 1] Check if the door can be lockpicked
      (if (Variables|UserDefined|GetIsUnlockable)
        (bind _numlockpicks (Class|InterfaceInventory1|GetNumLockpicks(Message) (Game|GetPlayerController 0)))
        (if (> _numlockpicks 0)
          ;[1 1 1] Check if door has been lockpicked
          (Utilities|IsValid _returnvalue
            (:Is%20Valid
              (Variables|UserDefined|SetIsLocked false)
              (Components|DestroyComponent _returnvalue)
              (goto _label))
            (:Is%20Not%20Valid
              ;[1 0 0.5859] Lockpicking
              (Utilities|IsValid _returnvalue_2
                (:Is%20Valid
                  (Default|EventGenerateLockSettings _returnvalue_2 (Variables|UserDefined|GetLock%20Difficulty))
                  (Default|EventLockpicking _returnvalue_2 (Variables|Interaction|GetInteracting%20Actor))))))
          (else
            (Class|InterfaceMessaging|SendShortMessage(Message) (Game|GetPlayerController 0) "You do not have any lockpicks")))
        (else
          (Development|PrintString "Door cannot be lockpicked.")
          (Class|InterfaceMessaging|SendShortMessage(Message) (Game|GetPlayerController 0) "This door cannot be lockpicked"))))))

(event Custom|Event%20Reset%20Lock
  (bind _returnvalue (Actor|GetComponentbyClass "/Game/MRPGT/Lockpicking_Minigame/Blueprints/Actor_Components/AC_Lockpicking_Successful.AC_Lockpicking_Successful_C"))
  ;[0.00045 0.3125 0] Reset door lock
  (Utilities|IsValid _returnvalue
    (:Is%20Valid
      (Components|DestroyComponent _returnvalue))
    (:Is%20Not%20Valid
      _))
  (Variables|UserDefined|SetLock%20Difficulty (Utilities|Enum|ByteToEnumE_Lock_Difficulties (Math|Conversions|ToByte(Integer) (Math|Random|RandomInteger 5))))
  (Variables|UserDefined|SetIsLocked true))

(event Custom|Event%20Open%20Door
  (bind _original_door_rotation (Variables|Interaction|GetOriginal%20Door%20Rotation))
  ;[0 1 0.1328] Rotate door to open it
  (bind _isa (Utilities|FlowControl|FlipFlop)
    (:A
      _)
    (:B
      _))
  (if _isa
    (if (<= (Components|Timeline|GetPlaybackPosition (Variables|Default|GetDoor%20Rotation)) 0.0)
      (CallFunction|EventOpenDoorSound)
      (bind _rotation (Timeline|Door%20Rotation Play)
        (:Update
          (Transformation|SetWorldRotation (Variables|Default|GetDoor) (Math|Rotator|MakeRotator (.roll _original_door_rotation) (.pitch _original_door_rotation) (+ (* _rotation (Variables|UserDefined|GetOpen%20Door%20Angle)) (.yaw _original_door_rotation))) false false)
          (if (<= (Components|Timeline|GetPlaybackPosition (Variables|Default|GetDoor%20Rotation)) 0.1)
            (Utilities|FlowControl|DoOnce false :!label _label
              (:Completed
                (CallFunction|EventCloseDoorSound)))
            (else
              (goto _label Reset))))
        (:Finished
          (goto _label Reset)))
      (else
        (Timeline|Door%20Rotation Play)))
    (else
      (Timeline|Door%20Rotation Reverse))))

(event Custom|Event%20Open%20Door%20Sound
  ;[0 0.6953 1] Play opening sound at door
  (Audio|PlaySoundatLocation (Variables|Interaction|GetOpen%20Sound) (Transformation|GetWorldLocation (Variables|Default|GetDoor)) "0, 0, 0" 1.0 1.0 0.0 0 0 0 0))

(event Custom|Event%20Close%20Door%20Sound
  ;[1 0.6711 0] Play closing sound at door
  (Audio|PlaySoundatLocation (Variables|Interaction|GetClose%20Sound) (Transformation|GetWorldLocation (Variables|Default|GetDoor)) "0, 0, 0" 1.0 1.0 0.0 0 0 0 0))

(event EventInteract
  (params (HitComponent :type Actor%20Component%20Object%20Reference) (InteractingActor :type Actor%20Object%20Reference))
  ;[0.7344 0 1] Interaction with door
  (Variables|Interaction|SetInteracting%20Actor InteractingActor)
  (CallFunction|EventInspectDoor))

(fn ConstructionScript
  (Utilities|FlowControl|Sequence
    (:then_0
      ;[1 0.9609 0] Define door's world rotation
      (Variables|Interaction|SetOriginal%20Door%20Rotation (Transformation|GetWorldRotation (Variables|Default|GetDoor))))
    (:then_1
      ;[0.3359 0 1] Mesh - Door
      (bind _returnvalue (Utilities|LoadAssetBlocking (Variables|UserDefined|GetSoft%20Door%20SM)))
      (bind _asstatic_mesh (Utilities|Casting|CastToStaticMesh _returnvalue))
      (Components|StaticMesh|SetStaticMesh (Variables|Default|GetDoor) _asstatic_mesh))
    (:then_2
      ;[1 0 0] Mesh - Door Frame
      (bind _returnvalue_2 (Utilities|LoadAssetBlocking (Variables|UserDefined|GetSoft%20DoorFrame%20SM)))
      (bind _asstatic_mesh_2 (Utilities|Casting|CastToStaticMesh _returnvalue_2))
      (Components|StaticMesh|SetStaticMesh (Variables|Default|GetDoorFrame) _asstatic_mesh_2))
    (:then_3
      ;[0 0.6953 1] Sound - Open
      (bind _returnvalue_3 (Utilities|LoadAssetBlocking (Variables|UserDefined|GetSoft%20Open%20Sound)))
      (bind _assound_base (Utilities|Casting|CastToSoundBase _returnvalue_3))
      (Variables|Interaction|SetOpen%20Sound _assound_base))
    (:then_4
      ;[1 0.3331 0] Sound - Close
      (bind _returnvalue_4 (Utilities|LoadAssetBlocking (Variables|UserDefined|GetSoft%20Close%20Sound)))
      (bind _assound_base_2 (Utilities|Casting|CastToSoundBase _returnvalue_4))
      (Variables|Interaction|SetClose%20Sound _assound_base_2))))

(fn GetID
  (return ""))

(fn GetLauncherActor
  (return 0))

(fn GetObjectName
  (bind _ac_lockpicking (Variables|Default|GetAC_Lockpicking)
    (:then
      (if (Variables|UserDefined|GetIsLocked)
        (if (Variables|UserDefined|GetIsUnlockable)
          (bind _numlockpicks (Class|InterfaceInventory1|GetNumLockpicks(Message) (Game|GetPlayerController 0)))
          (if (> _numlockpicks 0)
            (return (Utilities|String|SelectString "Locked (Try to pick the lock)" "" (and (Variables|/Game/MRPGT/Lockpicking_Minigame/Blueprints/Actor_Components/AC_Lockpicking.AC_Lockpicking_C|GetbIsLocked _ac_lockpicking) (not (Variables|/Game/MRPGT/Lockpicking_Minigame/Blueprints/Actor_Components/AC_Lockpicking.AC_Lockpicking_C|GetbLockpickingInProgress _ac_lockpicking)))))
            (else
              (return (Utilities|String|SelectString "Locked (No lockpicks)" "" (and (Variables|/Game/MRPGT/Lockpicking_Minigame/Blueprints/Actor_Components/AC_Lockpicking.AC_Lockpicking_C|GetbIsLocked _ac_lockpicking) (not (Variables|/Game/MRPGT/Lockpicking_Minigame/Blueprints/Actor_Components/AC_Lockpicking.AC_Lockpicking_C|GetbLockpickingInProgress _ac_lockpicking)))))))
          (else
            (return "Locked (Cannot be picked)")))
        (else
          (return ""))))
    (:else)))

(fn IsInteractable
  (return true))

(fn IsProjectile
  (return false))