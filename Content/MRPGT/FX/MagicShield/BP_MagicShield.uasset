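; BP_MagicShield is a magic shield effect actor driven by a Niagara system and a material parameter collection.
; On BeginPlay it writes color, opacity, Fresnel depth fade and WPO settings into MPC_MagicShield, and passes color and lifetime to Niagara.
; Each tick a float spring interpolation eases the size toward its target and feeds it to Niagara as User.SpringFloat, giving a springy scale motion.
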(event EventBeginPlay
  (Rendering|Material|SetVectorParameterValue "/Game/MRPGT/FX/MagicShield/MPC_MagicShield.MPC_MagicShield" "Shield Color" (Variables|Default|GetShield%20Color) :!class /Script/Engine.KismetMaterialLibrary)
  (Rendering|Material|SetScalarParameterValue "/Game/MRPGT/FX/MagicShield/MPC_MagicShield.MPC_MagicShield" "Shield Opacity" (Variables|Default|GetShield%20Opacity) :!class /Script/Engine.KismetMaterialLibrary)
  (Rendering|Material|SetScalarParameterValue "/Game/MRPGT/FX/MagicShield/MPC_MagicShield.MPC_MagicShield" "Fresnel Depth Fade Opacity" (Variables|Default|GetFresnel%20Depth%20Fade%20Opacity) :!class /Script/Engine.KismetMaterialLibrary)
  (Rendering|Material|SetScalarParameterValue "/Game/MRPGT/FX/MagicShield/MPC_MagicShield.MPC_MagicShield" "Fresnel Depth Fade Distance" (Variables|Default|GetFresnel%20Depth%20Fade%20Distance) :!class /Script/Engine.KismetMaterialLibrary)
  (Rendering|Material|SetScalarParameterValue "/Game/MRPGT/FX/MagicShield/MPC_MagicShield.MPC_MagicShield" "WPO Multiplier" (Variables|Default|GetWPO%20Multiplier) :!class /Script/Engine.KismetMaterialLibrary)
  (Niagara|SetNiagaraVariable(LinearColor) (Variables|Default|GetNiagara) "User.Color" (Variables|Default|GetShield%20Color))
  (Niagara|SetNiagaraVariable(Float) (Variables|Default|GetNiagara) "User.Lifetime" (Variables|Default|GetLifetime)))

(event Collision|EventActorBeginOverlap
  (params (OtherActor :type Actor%20Object%20Reference)))

(event EventTick
  (params (DeltaSeconds :type Float%20%28single-precision%29))
  (bind _returnvalue (Class|KismetMathLibrary|FloatSpringInterp (Variables|Default|GetStart%20Size) (Variables|Default|GetTarget%20Size) (Variables|Default|GetSpringState) (Variables|Default|GetSpring%20Stiffness) (Variables|Default|GetSpring%20Critical%20Damping%20Factor) DeltaSeconds (Variables|Default|GetMass) 1.0))
  (bind _output_get (Variables|Default|SetStart%20Size _returnvalue))
  (Development|PrintString (Utilities|String|ToString(Float) _output_get) false false)
  (Niagara|SetNiagaraVariable(Float) (Variables|Default|GetNiagara) "User.SpringFloat" (Variables|Default|GetStart%20Size)))

(fn ConstructionScript)