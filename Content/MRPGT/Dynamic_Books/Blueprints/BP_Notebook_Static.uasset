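; BP_Notebook_Static is a readable world notebook whose mesh, text and cover come from a data table row matched by ItemID.
; Interact switches the player to book-reading mode, spawns a BP_Notebook_Dynamic, eases it before the camera on a timeline, then opens it.
; A construction-time GUID tracks it in save games: already-taken books destroy themselves on load, and dropped books store their transform after a settling delay.
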(event Custom|AddBookToSaveGame
  (Utilities|FlowControl|Delay 3.0) ; Allow for the book to fall to ground before getting its transform
  (Physics|SetSimulatePhysics (Variables|Default|GetBook) false)
  (if (Default|IsDroppedIteminSaveGame (Variables|/Game/MRPGT/Blueprints/GameInstance/BP_MRPGT_GameInstance.BP_MRPGT_GameInstance_C|GetSavedGame (Variables|Default|GetGameInstance)) (Variables|Default|GetUniqueID))
    (Default|UpdateDroppedItemSavedTransform (Variables|/Game/MRPGT/Blueprints/GameInstance/BP_MRPGT_GameInstance.BP_MRPGT_GameInstance_C|GetSavedGame (Variables|Default|GetGameInstance)) (Variables|Default|GetUniqueID) (Transformation|GetActorTransform))
    (Development|PrintString "[AddBookToSaveGame] Updated book's transform within the savegame" false)
    (else
      (Default|AddDroppedItem (Variables|/Game/MRPGT/Blueprints/GameInstance/BP_MRPGT_GameInstance.BP_MRPGT_GameInstance_C|GetSavedGame (Variables|Default|GetGameInstance)) (Variables|Default|GetUniqueID) (Variables|Default|GetItemID) (Transformation|GetActorTransform))
      (Development|PrintString "[AddBookToSaveGame] Added book to savegame" false))))

(event Custom|CustomEvent_0
  (CallFunction|CheckifStateChanged))

(event EventInteract
  (params (HitComponent :type Actor%20Component%20Object%20Reference) (InteractingActor :type Actor%20Object%20Reference))
  (bind _returnvalue (Game|GetPlayerCharacter 0))
  ;[1 0 0.04687] Define Variables + Controlling for Character Movement and Camera
  (bind _viewmode (Class|InterfaceGeneralCharacter|GetViewMode(Message) (Game|GetPlayerCharacter 0)))
  (Variables|Default|SetOriginalViewMode _viewmode)
  (Class|InterfacePlayerInput|EnableBookReadingMode(Message) (Game|GetPlayerController 0) true)
  (bind _bookreadingcamera (Class|InterfaceGeneralCharacter|GetBookReadingCamera(Message) (Game|GetPlayerCharacter 0)))
  (Variables|Default|SetPlayer%20Camera _bookreadingcamera)
  (Class|InterfaceGeneralCharacter|ActivateCamera(Message) (Game|GetPlayerCharacter 0) "NewEnumerator3")
  ;[0 0.7891 1] Spawn dynamic book
  (bind _returnvalue_2 (Game|SpawnActorfromClass "/Game/MRPGT/Dynamic_Books/Blueprints/BP_Notebook_Dynamic.BP_Notebook_Dynamic_C" (Math|Transform|MakeTransform (+ (.Location (Math|Transform|BreakTransform (Transformation|GetWorldTransform (Variables|Default|GetPlayer%20Camera)))) (* (Math|Vector|GetForwardVector (Variables|Default|GetPlayer%20Camera)) 1e+02)) (.Rotation (Math|Transform|BreakTransform (Transformation|GetWorldTransform (Variables|Default|GetPlayer%20Camera)))) (.Scale (Math|Transform|BreakTransform (Transformation|GetWorldTransform (Variables|Default|GetPlayer%20Camera))))) "AlwaysSpawn" "MultiplyWithRoot" 0 (Utilities|Struct|BreakItemStruct (Variables|Default|GetItemInfo)) "" (Variables|Default|GetOriginalViewMode) 0))
  (bind _output_get (Variables|Other|SetSpawned%20Book _returnvalue_2))
  (Variables|/Game/MRPGT/Dynamic_Books/Blueprints/BP_Book_Template_Dynamic.BP_Book_Template_Dynamic_C|SetAnimation%20Is%20Playing? _output_get true)
  (bind _moving___rotation_speed (Timeline|Reposition%20Book%20Speed PlayFromStart)
    (:Update
      (Transformation|SetActorLocationAndRotation (Variables|Other|GetSpawned%20Book) (Math|Vector|Lerp(Vector) (Transformation|GetActorLocation (Variables|Other|GetSpawned%20Book)) (+ (Transformation|GetWorldLocation (Variables|Default|GetPlayer%20Camera)) (* (Math|Vector|GetForwardVector (Variables|Default|GetPlayer%20Camera)) (Variables|UserDefined|GetDistance%20from%20Camera))) _moving___rotation_speed) (Math|Rotator|Lerp(Rotator) (Transformation|GetActorRotation _returnvalue) (Pawn|GetControlRotation _returnvalue :!class /Script/Engine.Pawn) _moving___rotation_speed true)))
    (:Finished
      ;[1 0.4922 0] Initialize the opening of the book and indicate it to the player controller
      (Default|OpenBook (Variables|Other|GetSpawned%20Book) (.BookText (Utilities|Struct|BreakItemStruct (Variables|Default|GetItemInfo))))
      (Class|InterfacePlayerInput|SetNewOpenBook(Message) (Game|GetPlayerController 0) (Variables|Other|GetSpawned%20Book) self))))

(event EventChangeState
  ;[1 1 1] When a save game loads and this ItemPickup actor is found to be stored within the save game (InteractedActorIDs array) then it means that this actor was taken (picked up) by the player therefore it should be destroyed immediately
  (Actor|DestroyActor))

(event EventBeginPlay
  (CallFunction|InitializeReferences)
  (EventDispatchers|BindEventtoInitializeItemPickups (Variables|Default|GetPlayerController) (delegate Custom|CustomEvent_0)))

(event EventDestroyed
  ;[1 1 1] When this actor is destroyed, either by the player when picking it up or when the save game is loaded within which this itempickup was already picked up then add it to the savegame object for storage within future save games
  (if (not (Variables|Default|GetWasSpawnedByThePlayer))
    (bind _gameinstance (Variables|Default|GetGameInstance)
      (:then
        (Default|AddInteractedActorID (Variables|/Game/MRPGT/Blueprints/GameInstance/BP_MRPGT_GameInstance.BP_MRPGT_GameInstance_C|GetSavedGame _gameinstance) (Variables|Default|GetUniqueID)))
      (:else))))

(fn ConstructionScript
  (Utilities|FlowControl|Sequence
    (:then_0
      (bind _outrownames (DataTable|GetDataTableRowNames "/Game/MRPGT/Blueprints/DataTables/WorldItemsDataTable.WorldItemsDataTable"))
      (for _array_element _outrownames
        (if (Utilities|Name|Equal(Name) _array_element (Utilities|String|StringToName (Variables|Default|GetItemID)))
          (bind _returnvalue (Utilities|GetDataTableRow "/Game/MRPGT/Blueprints/DataTables/WorldItemsDataTable.WorldItemsDataTable" _array_element)
            (:then
              (bind _output_get (LocalVariables|SetLocalItem _returnvalue))
              (bind _output_get_2 (Variables|Default|SetItemInfo _output_get))
              (if (Utilities|IsValidSoftObjectReference (.StaticMesh (Utilities|Struct|BreakItemStruct _output_get_2)))
                (bind _returnvalue_2 (Utilities|LoadAssetBlocking (.StaticMesh (Utilities|Struct|BreakItemStruct _output_get_2))))
                (Components|StaticMesh|SetStaticMesh (Variables|Default|GetBook) (.AsStatic%20Mesh (Utilities|Casting|CastToStaticMesh _returnvalue_2)))))))))
    (:then_1
      (CallFunction|GenerateUniqueID false))))

(fn Enable/DisableMovementandLook
  (params (Character :type Character%20Object%20Reference) (Enable? :type Boolean))
  (bind _returnvalue (Pawn|GetController Character))
  (bind _charactermovement (Variables|/Script/Engine.Character|GetCharacterMovement Character))
  (if Enable?
    (Pawn|Components|CharacterMovement|SetMovementMode _charactermovement "MOVE_Walking" 0)
    (Input|SetIgnoreLookInput _returnvalue false)
    (else
      (Pawn|Components|CharacterMovement|SetMovementMode _charactermovement "MOVE_None" 0)
      (Input|SetIgnoreLookInput _returnvalue true))))

(fn GenerateUniqueID
  (params (ForceGeneration :type Boolean))
  ;[0.25 0.25 0.25] Generate a unique ID for the SaveGames
  (if (or (Utilities|Array|IsEmpty (Variables|Default|GetUniqueID)) ForceGeneration)
    (Variables|Default|SetUniqueID (Guid|ToString(Guid) (Guid|NewGuid)))))

(fn InitializeReferences
  (Utilities|FlowControl|Sequence
    (:then_0
      (Variables|Default|SetPlayerController (.AsBP%20in%20Game%20Player%20Controller (Utilities|Casting|CastToBP_InGamePlayerController (Game|GetPlayerController 0))))
      (Variables|Default|SetPlayerCharacter (.AsBP%20Character (Utilities|Casting|CastToBP_Character (Game|GetPlayerCharacter 0)))))
    (:then_1
      (Variables|Default|SetGameInstance (.AsBP%20MRPGT%20Game%20Instance (Utilities|Casting|CastToBP_MRPGT_GameInstance (Game|GetGameInstance)))))))

(fn CheckifStateChanged
  (if (Default|GetSavedInteractableActorState (Variables|Default|GetGameInstance) (Variables|Default|GetUniqueID))
    (CallFunction|ChangeState)))

(fn GetID
  (return ""))

(fn GetLauncherActor
  (return 0))

(fn GetObjectName
  (return (Utilities|String|ToString(Text) (.Name (Utilities|Struct|BreakItemStruct (Variables|Default|GetItemInfo))))))

(fn IsProjectile
  (return false))