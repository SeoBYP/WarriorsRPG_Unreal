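; Static, interactable book that spawns a BP_Book_Template_Dynamic copy for reading when a character interacts with it.
; Interaction disables the character's movement and look input, then spawns the copy at the book mesh's transform.
; A timeline lerps the copy to a set distance in front of the camera, rotated toward the control rotation.
; When finished, it opens the copy with BookText and stores it on BP_PlayerCharacter as OpenBook.
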(event EventOnInteract
  (params (InteractingActor :type Character%20Object%20Reference) (ActorCamera :type Camera%20Component%20Object%20Reference))
  ;[1 0 0.04687] Define Variables + Controlling for Character Movement and Camera
  (bind _output_get (Variables|Other|SetInteracting%20Actor InteractingActor))
  (CallFunction|Enable/DisableMovementandLook _output_get false)
  (Variables|Default|SetPlayer%20Camera ActorCamera)
  ;[0 0.7891 1] Spawn dynamic book
  (bind _returnvalue (Game|SpawnActorfromClass "/Game/MRPGT/Dynamic_Books/Blueprints/BP_Book_Template_Dynamic.BP_Book_Template_Dynamic_C" (Transformation|GetWorldTransform (Variables|Default|GetBook self)) "AlwaysSpawn" "MultiplyWithRoot" 0 0 "" "NewEnumerator0" 0))
  (bind _output_get_2 (Variables|Other|SetSpawned%20Book _returnvalue))
  (Variables|/Game/MRPGT/Dynamic_Books/Blueprints/BP_Book_Template_Dynamic.BP_Book_Template_Dynamic_C|SetAnimation%20Is%20Playing? _output_get_2 true)
  (bind _moving___rotation_speed (Timeline|Reposition%20Book%20Speed PlayFromStart)
    (:Update
      (Transformation|SetActorLocationAndRotation (Variables|Other|GetSpawned%20Book) (Math|Vector|Lerp(Vector) (Transformation|GetActorLocation (Variables|Other|GetSpawned%20Book)) (+ (Transformation|GetWorldLocation (Variables|Default|GetPlayer%20Camera)) (* (Math|Vector|GetForwardVector (Variables|Default|GetPlayer%20Camera)) (Variables|UserDefined|GetDistance%20from%20Camera))) _moving___rotation_speed) (Math|Rotator|Lerp(Rotator) (Transformation|GetActorRotation (Variables|Other|GetInteracting%20Actor)) (Pawn|GetControlRotation (Variables|Other|GetInteracting%20Actor) :!class /Script/Engine.Pawn) _moving___rotation_speed true)))
    (:Finished
      ;[1 0.4922 0] Initialize the opening of the book and indicate it to the Interacting Actor
      (Default|OpenBook (Variables|Other|GetSpawned%20Book) (Variables|UserDefined|GetBook%20Text))
      (bind _asbp_player_character (Utilities|Casting|CastToBP_PlayerCharacter (Variables|Other|GetInteracting%20Actor)))
      (Variables|/Game/MRPGT/Dynamic_Books/Demo/BP_PlayerCharacter.BP_PlayerCharacter_C|SetOpenBook _asbp_player_character (Variables|Other|GetSpawned%20Book)))))

(fn ConstructionScript)

(fn Enable/DisableMovementandLook
  (params (Character :type Character%20Object%20Reference) (Enable? :type Boolean))
  (bind _returnvalue (Pawn|GetController Character))
  (bind _charactermovement (Variables|/Script/Engine.Character|GetCharacterMovement Character))
  (if Enable?
    (Pawn|Components|CharacterMovement|SetMovementMode _charactermovement "MOVE_Walking" 0)
    (Input|SetIgnoreLookInput _returnvalue false)
    (else
      (Pawn|Components|CharacterMovement|SetMovementMode _charactermovement "MOVE_None" 0)
      (Input|SetIgnoreLookInput _returnvalue true))))

(fn IsInteractable
  (return true))