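; Master medieval door actor that the player interacts with to open, close, unlock or lockpick, with optional shutter, knocker, latch bar and bolt.
; The construction script loads meshes and sounds from soft references, and BeginPlay shows or hides the optional parts.
; Interact branches on the hit component's name to drive each part's timeline.
; Locked doors check for a key item or lockpicks, using lockpicking components to track success.
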(event Custom|Event%20Inspect%20Door
  (bind _returnvalue (Actor|GetComponentbyClass "/Game/MRPGT/Lockpicking_Minigame/Blueprints/Actor_Components/AC_Lockpicking_Successful.AC_Lockpicking_Successful_C"))
  (bind _returnvalue_2 (Actor|GetComponentbyClass "/Game/MRPGT/Lockpicking_Minigame/Blueprints/Actor_Components/AC_Lockpicking.AC_Lockpicking_C"))
  (Utilities|FlowControl|Sequence
    (:then_0
      ;[0 1 0.7422] Check if the door is locked
      (if (not (Variables|Default|GetIsLocked))
        (CallFunction|EventOpenDoor :!label _label)
        (elif (Variables|Default|GetbRequiresKeyToUnlock)
          ;[0 0.4375 1] Does the player have the correct key?
          (bind _hasitem (Class|InterfaceInventory1|PlayerHasItembyItemID(Message) (Game|GetPlayerController 0) (Variables|Default|GetKeyRequiredItemID)))
          (if _hasitem
            ;[0 0.4375 1] Unlock the door with the key
            (bind _item (Class|InterfaceItems|GetItembyID(Message) (Game|GetGameInstance) (Variables|Default|GetKeyRequiredItemID)))
            (Variables|Default|SetKeyDetails _item)
            (Game|AddComponentbyClass "/Game/MRPGT/Lockpicking_Minigame/Blueprints/Actor_Components/AC_Lockpicking_Successful.AC_Lockpicking_Successful_C")
            (Class|InterfaceMessaging|SendShortMessage(Message) (Game|GetPlayerController 0) (Utilities|Text|FormatText "You use the {key} to unlock the door" (.Name (Utilities|Struct|BreakItemStruct (Variables|Default|GetKeyDetails)))))
            ;[0 0.4375 1] Check if door has been lockpicked
            (Utilities|IsValid _returnvalue :!label _label_2
              (:Is%20Valid
                (Variables|Default|SetIsLocked false)
                (Components|DestroyComponent _returnvalue)
                (goto _label))
              (:Is%20Not%20Valid
                ;[1 0 0.5859] Lockpicking
                (Utilities|IsValid _returnvalue_2
                  (:Is%20Valid
                    (Default|EventGenerateLockSettings _returnvalue_2 (Variables|Default|GetLock%20Difficulty))
                    (Default|EventLockpicking _returnvalue_2 (Variables|Default|GetInteracting%20Actor))))))
            (else
              ;[0 0.3203 1] Check if the door can be lockpicked
              (if (Variables|Default|GetIsUnlockable) :!label _label_3
                ;[0 0.4375 1] Does player have any lockpicks?
                (bind _numlockpicks (Class|InterfaceInventory1|GetNumLockpicks(Message) (Game|GetPlayerController 0)))
                (if (> _numlockpicks 0)
                  (goto _label_2)
                  (else
                    ;[0 0.4375 1] Display on screen message that the player does not have any lockpicks
                    (Class|InterfaceMessaging|SendShortMessage(Message) (Game|GetPlayerController 0) "You do not have any lockpicks")))
                (else
                  ;[0 0.4375 1] Display on screen message that the door cannot be lockpicked
                  (Development|PrintString "Door cannot be lockpicked.")
                  (Class|InterfaceMessaging|SendShortMessage(Message) (Game|GetPlayerController 0) "This door cannot be lockpicked")))))
          (else
            (goto _label_3)))))
    (:then_1
      (Variables|Default|SetIs%20In%20Use? false))))

(event Custom|Event%20Reset%20Lock
  (bind _returnvalue (Actor|GetComponentbyClass "/Game/MRPGT/Lockpicking_Minigame/Blueprints/Actor_Components/AC_Lockpicking_Successful.AC_Lockpicking_Successful_C"))
  ;[0.00045 0.3125 0] Reset door lock
  (Utilities|IsValid _returnvalue
    (:Is%20Valid
      (Components|DestroyComponent _returnvalue))
    (:Is%20Not%20Valid
      _))
  (Variables|Default|SetLock%20Difficulty (Utilities|Enum|ByteToEnumE_Lock_Difficulties (Math|Conversions|ToByte(Integer) (Math|Random|RandomInteger 5))))
  (Variables|Default|SetIsLocked true))

(event Custom|Event%20Open%20Door
  (bind _original_door_rotation (Variables|Default|GetOriginal%20Door%20Rotation))
  ;[0 1 0.1328] Rotate door to open it
  (bind _isa (Utilities|FlowControl|FlipFlop)
    (:A
      _)
    (:B
      _))
  (if _isa
    (if (<= (Components|Timeline|GetPlaybackPosition (Variables|Default|GetDoorRotation)) 0.0)
      (CallFunction|EventOpenDoorSound)
      (Variables|Default|SetIs%20Door%20Open? true)
      (bind _rotation (Timeline|DoorRotation Play)
        (:Update
          (Transformation|SetWorldRotation (Variables|Default|GetDoor) (Math|Rotator|MakeRotator (.roll _original_door_rotation) (.pitch _original_door_rotation) (+ (* _rotation (* (Variables|Default|GetOpen%20Door%20Angle) (Math|Float|SelectFloat -1.0 1.0 (Variables|Default|GetReverse%20Direction?)))) (.yaw _original_door_rotation))) false false)
          (if (<= (Components|Timeline|GetPlaybackPosition (Variables|Default|GetDoorRotation)) 0.1)
            (Utilities|FlowControl|DoOnce false :!label _label
              (:Completed
                (CallFunction|EventCloseDoorSound)))
            (else
              (goto _label Reset))))
        (:Finished
          (goto _label Reset)))
      (else
        (Timeline|DoorRotation Play)))
    (else
      (Variables|Default|SetIs%20Door%20Open? false)
      (Timeline|DoorRotation Reverse))))

(event Custom|Event%20Open%20Door%20Sound
  ;[0 0.6953 1] Play opening sound at door
  (Audio|PlaySoundatLocation (Variables|Default|GetOpen%20Sound) (Transformation|GetWorldLocation (Variables|Default|GetDoor)) "0, 0, 0" 1.0 1.0 0.0 0 0 0 0))

(event Custom|Event%20Close%20Door%20Sound
  ;[1 0.6711 0] Play closing sound at door
  (Audio|PlaySoundatLocation (Variables|Default|GetClose%20Sound) (Transformation|GetWorldLocation (Variables|Default|GetDoor)) "0, 0, 0" 1.0 1.0 0.0 0 0 0 0))

(event EventUnlocked
  (CallFunction|EventOpenDoor))

(event EventInteract
  (params (HitComponent :type Actor%20Component%20Object%20Reference) (InteractingActor :type Actor%20Object%20Reference))
  (bind _returnvalue (Utilities|GetObjectName HitComponent))
  (bind _bolt (Variables|Default|GetBolt))
  (bind _initiallatchbarrotation (Variables|Default|GetInitialLatchBarRotation))
  (bind _latch_bar (Variables|Default|GetLatch_Bar))
  (bind _debug (Variables|Default|GetDebug))
  (bind _initialboltlocation (Variables|Default|GetInitialBoltLocation))
  (bind _shutter (Variables|Default|GetShutter))
  (bind _initialknockerrotation (Variables|Default|GetInitialKnockerRotation))
  (bind _knocker (Variables|Default|GetKnocker))
  (bind _initialshutterrotation (Variables|Default|GetInitialShutterRotation))
  (bind _debug_2 (Variables|Default|GetDebug))
  (bind _relativelocation (Variables|/Script/Engine.SceneComponent|GetRelativeLocation _bolt))
  ;[1 1 1] The E key will open, unlock, pick, close door, or open and close the shutter or rap the knocker or move the bolt left and right
  (Class|InterfaceGeneralCharacter|SetIsInteractingwithObject(Message) (Game|GetPlayerCharacter 0) true)
  (if (Variables|Default|GetIs%20In%20Use?)
    (Development|PrintString "Door already in use" _debug _debug)
    (else
      (Variables|Default|SetIs%20In%20Use? true)
      (CallFunction|InitialiseTransforms)
      (Development|PrintString _returnvalue _debug _debug)
      (Utilities|FlowControl|Sequence
        (:then_0
          (switch string _returnvalue
            (:Default
              (Development|PrintString "Do nothing"))
            (:Door
              ;[0.7344 0 1] Interaction with door
              (Variables|Default|SetInteracting%20Actor InteractingActor)
              (CallFunction|EventInspectDoor))
            (:Shutter
              ;[1 1 1] Open or close shutter
              (bind _rotation (Timeline|ShutterTimeline PlayFromStart)
                (:Update
                  (if (Variables|Default|GetReverse%20Direction?)
                    (if (Variables|Default|GetIs%20Shutter%20Open?)
                      (Transformation|SetRelativeRotation _shutter (Math|Rotator|MakeRotator 0.0 0.0 (- _initialshutterrotation (* _rotation (Variables|Default|GetMax%20Shutter%20Rotation%20%28degrees%29)))) false false :!label _label)
                      (else
                        (Transformation|SetRelativeRotation _shutter (Math|Rotator|MakeRotator 0.0 0.0 (+ _initialshutterrotation (* _rotation (Variables|Default|GetMax%20Shutter%20Rotation%20%28degrees%29)))) false false :!label _label_2)))
                    (elif (Variables|Default|GetIs%20Shutter%20Open?)
                      (goto _label_2)
                      (else
                        (goto _label)))))
                (:Finished
                  (Variables|Default|SetIs%20Shutter%20Open? (not (Variables|Default|GetIs%20Shutter%20Open?)))
                  (Variables|Default|SetIs%20In%20Use? false))))
            (:Knocker
              ;[1 1 1] Rap knocker
              (bind _rotation_2 (Timeline|KnockerTimeline PlayFromStart)
                (:Update
                  (if (Variables|Default|GetReverse%20Direction?)
                    (Transformation|SetRelativeRotation _knocker (Math|Rotator|MakeRotator (+ _initialknockerrotation (* _rotation_2 (Variables|Default|GetMax%20Knocker%20Rotation%20%28degrees%29))) 0.0 0.0) false false)
                    (else
                      (Transformation|SetRelativeRotation _knocker (Math|Rotator|MakeRotator (- _initialknockerrotation (* _rotation_2 (Variables|Default|GetMax%20Knocker%20Rotation%20%28degrees%29))) 0.0 0.0) false false)))
                  (Development|PrintString "Anyone home?" _debug_2 _debug_2))
                (:Finished
                  (Audio|PlaySoundatLocation "/Game/MRPGT/MedievalBuildings01/Audio/SoundCues/DoorKnocker_Cue.DoorKnocker_Cue" "0, 0, 0" "0, 0, 0" 1.0 1.0 0.0 0 0 0 0)
                  (Variables|Default|SetIs%20In%20Use? false))))
            (:Latch_Bar
              ;[1 1 1] Open or close latch bar
              (bind _rotation_3 (Timeline|Latch%20Timeline PlayFromStart)
                (:Update
                  (if (Variables|Default|GetIs%20Latch%20Open?)
                    (Transformation|SetRelativeRotation _latch_bar (Math|Rotator|MakeRotator 0.0 (+ _initiallatchbarrotation (* _rotation_3 (Variables|Default|GetMaxLatchBarRotation%20%28degrees%29))) 0.0) false false)
                    (else
                      (Transformation|SetRelativeRotation _latch_bar (Math|Rotator|MakeRotator 0.0 (- _initiallatchbarrotation (* _rotation_3 (Variables|Default|GetMaxLatchBarRotation%20%28degrees%29))) 0.0) false false))))
                (:Finished
                  (Variables|Default|SetIs%20Latch%20Open? (not (Variables|Default|GetIs%20Latch%20Open?)))
                  (Variables|Default|SetIs%20In%20Use? false))))
            (:Bolt
              ;[1 1 1] Close or open bolt
              (bind _rotation_4 (Timeline|Bolt%20Timeline PlayFromStart)
                (:Update
                  (if (Variables|Default|GetIs%20Bolt%20Closed?)
                    (Transformation|SetRelativeLocation _bolt (Math|Vector|MakeVector (+ _initialboltlocation (* _rotation_4 (Variables|Default|GetMaxBoltDistance))) (.y _relativelocation) (.z _relativelocation)) false false)
                    (else
                      (Transformation|SetRelativeLocation _bolt (Math|Vector|MakeVector (- _initialboltlocation (* _rotation_4 (Variables|Default|GetMaxBoltDistance))) (.y _relativelocation) (.z _relativelocation)) false false))))
                (:Finished
                  (Variables|Default|SetIs%20Bolt%20Closed? (not (Variables|Default|GetIs%20Bolt%20Closed?)))
                  (Variables|Default|SetIs%20In%20Use? false))))))))))

(event EventBeginPlay
  ;[1 1 1] BeginPlay - initialize visibility of mesh components such as shutter or knocker
  (CallFunction|InitialisePlayRates)
  (CallFunction|InitializeVisibility))

(fn ConstructionScript
  (Utilities|FlowControl|Sequence
    (:then_0
      ;[1 0.9609 0] Define door's world rotation
      (Variables|Default|SetOriginal%20Door%20Rotation (Transformation|GetWorldRotation (Variables|Default|GetDoor))))
    (:then_1
      ;[0.3359 0 1] Mesh - Door
      (bind _returnvalue (Utilities|LoadAssetBlocking (Variables|Default|GetSoft%20Door%20SM)))
      (bind _asstatic_mesh (Utilities|Casting|CastToStaticMesh _returnvalue))
      (Components|StaticMesh|SetStaticMesh (Variables|Default|GetDoor) _asstatic_mesh))
    (:then_2
      ;[1 0 0] Mesh - Door Frame
      (bind _returnvalue_2 (Utilities|LoadAssetBlocking (Variables|Default|GetSoft%20DoorFrame%20SM)))
      (bind _asstatic_mesh_2 (Utilities|Casting|CastToStaticMesh _returnvalue_2))
      (Components|StaticMesh|SetStaticMesh (Variables|Default|GetDoorFrame) _asstatic_mesh_2))
    (:then_3
      ;[0 0.6953 1] Sound - Open
      (bind _returnvalue_3 (Utilities|LoadAssetBlocking (Variables|Default|GetSoft%20Open%20Sound)))
      (bind _assound_base (Utilities|Casting|CastToSoundBase _returnvalue_3))
      (Variables|Default|SetOpen%20Sound _assound_base))
    (:then_4
      ;[1 0.3331 0] Sound - Close
      (bind _returnvalue_4 (Utilities|LoadAssetBlocking (Variables|Default|GetSoft%20Close%20Sound)))
      (bind _assound_base_2 (Utilities|Casting|CastToSoundBase _returnvalue_4))
      (Variables|Default|SetClose%20Sound _assound_base_2))
    (:then_5
      ;[0.3359 0 1] Mesh - Shutter
      (bind _returnvalue_5 (Utilities|LoadAssetBlocking (Variables|Default|GetSoft%20Shutter%20SM)))
      (bind _asstatic_mesh_3 (Utilities|Casting|CastToStaticMesh _returnvalue_5))
      (Components|StaticMesh|SetStaticMesh (Variables|Default|GetShutter) _asstatic_mesh_3))
    (:then_6
      ;[0.3359 0 1] Mesh - Knocker
      (bind _returnvalue_6 (Utilities|LoadAssetBlocking (Variables|Default|GetSoft%20Knocker%20SM)))
      (bind _asstatic_mesh_4 (Utilities|Casting|CastToStaticMesh _returnvalue_6))
      (Components|StaticMesh|SetStaticMesh (Variables|Default|GetKnocker) _asstatic_mesh_4))
    (:then_7
      ;[0.3359 0 1] Mesh - Latch bar
      (bind _returnvalue_7 (Utilities|LoadAssetBlocking (Variables|Default|GetSoft%20Latch%20Bar%20SM)))
      (bind _asstatic_mesh_5 (Utilities|Casting|CastToStaticMesh _returnvalue_7))
      (Components|StaticMesh|SetStaticMesh (Variables|Default|GetLatch_Bar) _asstatic_mesh_5))
    (:then_8
      ;[0.3359 0 1] Mesh - Bolt
      (bind _returnvalue_8 (Utilities|LoadAssetBlocking (Variables|Default|GetSoft%20Bolt%20SM)))
      (bind _asstatic_mesh_6 (Utilities|Casting|CastToStaticMesh _returnvalue_8))
      (Components|StaticMesh|SetStaticMesh (Variables|Default|GetBolt) _asstatic_mesh_6))))

(fn InitialiseTransforms
  (Variables|Default|SetInitialDoorRotation (.Yaw (Math|Rotator|BreakRotator (.rotation (Transformation|GetRelativeTransform (Variables|Default|GetDoor))))))
  (Variables|Default|SetInitialShutterRotation (.Yaw (Math|Rotator|BreakRotator (.rotation (Transformation|GetRelativeTransform (Variables|Default|GetShutter))))))
  (Variables|Default|SetInitialKnockerRotation (.Roll (Math|Rotator|BreakRotator (.rotation (Transformation|GetRelativeTransform (Variables|Default|GetKnocker))))))
  (Variables|Default|SetInitialLatchBarRotation (.Pitch (Math|Rotator|BreakRotator (.rotation (Transformation|GetRelativeTransform (Variables|Default|GetLatch_Bar))))))
  (Variables|Default|SetInitialBoltLocation (.X (Math|Vector|BreakVector (.location (Transformation|GetRelativeTransform (Variables|Default|GetBolt)))))))

(fn InitialisePlayRates
  (Components|Timeline|SetPlayRate (Variables|Default|GetShutterTimeline) (Variables|Default|GetShutter%20Open%20Close%20Rate))
  (Components|Timeline|SetPlayRate (Variables|Default|GetKnockerTimeline) (Variables|Default|GetKnocker%20Rap%20Rate)))

(fn InitializeVisibility
  (Utilities|FlowControl|Sequence
    (:then_0
      (if (Variables|Default|GetIs%20Shutter%20Enabled?)
        (Rendering|SetVisibility (Variables|Default|GetShutter) true false)
        (Development|PrintString "Visible" false false)
        (Collision|SetCollisionEnabled (Variables|Default|GetShutter) "QueryAndPhysics")
        (else
          (Rendering|SetVisibility (Variables|Default|GetShutter) false false)
          (Development|PrintString "Not Visible" false false)
          (Collision|SetCollisionEnabled (Variables|Default|GetShutter) "NoCollision"))))
    (:then_1
      (if (Variables|Default|GetIs%20Knocker%20Enabled?)
        (Rendering|SetVisibility (Variables|Default|GetKnocker) true false)
        (Development|PrintString "Visible" false false)
        (Collision|SetCollisionEnabled (Variables|Default|GetKnocker) "QueryAndPhysics")
        (else
          (Rendering|SetVisibility (Variables|Default|GetKnocker) false false)
          (Development|PrintString "Not Visible" false false)
          (Collision|SetCollisionEnabled (Variables|Default|GetKnocker) "NoCollision"))))
    (:then_2
      (if (Variables|Default|GetIs%20Latch%20Bar%20Enabled?)
        (Rendering|SetVisibility (Variables|Default|GetLatch_Bar) true false)
        (Development|PrintString "Visible" false false)
        (Collision|SetCollisionEnabled (Variables|Default|GetLatch_Bar) "QueryAndPhysics")
        (else
          (Rendering|SetVisibility (Variables|Default|GetLatch_Bar) false false)
          (Development|PrintString "Not Visible" false false)
          (Collision|SetCollisionEnabled (Variables|Default|GetLatch_Bar) "NoCollision"))))
    (:then_3
      (if (Variables|Default|GetIs%20Bolt%20Enabled?)
        (Rendering|SetVisibility (Variables|Default|GetBolt) true false)
        (Development|PrintString "Visible" false false)
        (Collision|SetCollisionEnabled (Variables|Default|GetBolt) "QueryAndPhysics")
        (else
          (Rendering|SetVisibility (Variables|Default|GetBolt) false false)
          (Development|PrintString "Not Visible" false false)
          (Collision|SetCollisionEnabled (Variables|Default|GetBolt) "NoCollision"))))))

(fn GetID
  (return ""))

(fn GetLauncherActor
  (return 0))

(fn GetObjectName
  (bind _ac_lockpicking (Variables|Default|GetAC_Lockpicking)
    (:then
      (if (Variables|Default|GetIsLocked)
        (if (Variables|Default|GetIsUnlockable)
          (bind _numlockpicks (Class|InterfaceInventory1|GetNumLockpicks(Message) (Game|GetPlayerController 0)))
          (if (> _numlockpicks 0)
            (return (Utilities|String|SelectString "Locked" "" (and (Variables|/Game/MRPGT/Lockpicking_Minigame/Blueprints/Actor_Components/AC_Lockpicking.AC_Lockpicking_C|GetbIsLocked _ac_lockpicking) (not (Variables|/Game/MRPGT/Lockpicking_Minigame/Blueprints/Actor_Components/AC_Lockpicking.AC_Lockpicking_C|GetbLockpickingInProgress _ac_lockpicking)))))
            (else
              (return (Utilities|String|SelectString "Locked (No lockpicks)" "" (and (Variables|/Game/MRPGT/Lockpicking_Minigame/Blueprints/Actor_Components/AC_Lockpicking.AC_Lockpicking_C|GetbIsLocked _ac_lockpicking) (not (Variables|/Game/MRPGT/Lockpicking_Minigame/Blueprints/Actor_Components/AC_Lockpicking.AC_Lockpicking_C|GetbLockpickingInProgress _ac_lockpicking)))))))
          (else
            (return "Locked (Cannot be picked)")))
        (else
          (return (Utilities|String|SelectString "Close Door" "Open Door" (Variables|Default|GetIs%20Door%20Open?))))))
    (:else)))

(fn IsProjectile
  (return false))