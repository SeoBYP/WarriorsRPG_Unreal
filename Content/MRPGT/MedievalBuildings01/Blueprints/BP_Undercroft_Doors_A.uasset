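; Undercroft door Blueprint that adds an animated bar tip to the shutter open/close behaviour inherited from its parent.
; On Lookingat, a busy flag rejects repeat use while two timelines rotate the bar tip's yaw, with a flag to reverse direction.
; Opening rotates the bar tip before calling the parent; closing calls the parent first, then rotates it back after a fixed delay.
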(event EventLookingat
  (params (HitComponent :type Actor%20Component%20Object%20Reference))
  (bind _debug (Variables|Default|GetDebug))
  (bind _debug_2 (Variables|Default|GetDebug))
  (bind _debug_3 (Variables|Default|GetDebug))
  (bind _debug_4 (Variables|Default|GetDebug))
  (bind _bartip (Variables|Default|GetBarTip))
  (bind _bartip_2 (Variables|Default|GetBarTip))
  ;[1 1 1] Initialise vars
  (if (Variables|Default|GetShutters%20Can%20Be%20Opened?)
    (if (Variables|Default|GetBar%20Tip%20Is%20Rotating)
      (Development|PrintString "Door already being used. Please wait." _debug_2 _debug_2)
      (else
        (Variables|Default|SetBar%20Tip%20Is%20Rotating true)
        (Variables|Default|SetInitial%20Bar%20Tip%20Rotation (.rotation (Transformation|GetRelativeTransform (Variables|Default|GetBarTip))))
        (Components|Timeline|SetPlayRate (Variables|Default|GetBarTipCloseTimeline) (Variables|Default|GetBar%20Tip%20Open%20Rate))
        ;[1 1 1] If door is open then close the bar tip otherwise open the bar tip
        (if (Variables|Default|GetShutters%20Are%20Open)
          (|CallParentFunction 0)
          (Utilities|FlowControl|Delay 3.0)
          (Development|PrintString "Closing bar tip" _debug_4 _debug_4)
          (Variables|Default|SetInitial%20Bar%20Tip%20Rotation (Variables|/Script/Engine.SceneComponent|GetRelativeRotation (Variables|Default|GetBarTip)))
          (bind _rotation (Timeline|BarTipCloseTimeline PlayFromStart)
            (:Update
              (if (Variables|Default|GetReverse%20Bar%20Tip%20Rotation)
                (Transformation|SetRelativeRotation _bartip (Math|Rotator|MakeRotator (.roll (Variables|Default|GetInitial%20Bar%20Tip%20Rotation)) (.pitch (Variables|Default|GetInitial%20Bar%20Tip%20Rotation)) (- (.yaw (Variables|Default|GetInitial%20Bar%20Tip%20Rotation)) (* _rotation (Variables|Default|GetMax%20Bar%20Tip%20Rotation%20%28degrees%29)))) false false)
                (else
                  (Transformation|SetRelativeRotation _bartip (Math|Rotator|MakeRotator (.roll (Variables|Default|GetInitial%20Bar%20Tip%20Rotation)) (.pitch (Variables|Default|GetInitial%20Bar%20Tip%20Rotation)) (+ (* _rotation (Variables|Default|GetMax%20Bar%20Tip%20Rotation%20%28degrees%29)) (.yaw (Variables|Default|GetInitial%20Bar%20Tip%20Rotation)))) false false)))
              (Development|PrintString (Utilities|String|Append "Bar tip relative rotation: " (Utilities|String|ToString(Rotator) (Variables|/Script/Engine.SceneComponent|GetRelativeRotation (Variables|Default|GetBarTip)))) _debug_3 _debug_3 :!label _label))
            (:Finished
              (Variables|Default|SetBar%20Tip%20Is%20Rotating false)))
          (else
            (Development|PrintString "Opening bar tip" _debug _debug)
            (bind _rotation_2 (Timeline|BarTipOpenTimeline PlayFromStart)
              (:Update
                (if (Variables|Default|GetReverse%20Bar%20Tip%20Rotation)
                  (Transformation|SetRelativeRotation _bartip_2 (Math|Rotator|MakeRotator (.roll (Variables|Default|GetInitial%20Bar%20Tip%20Rotation)) (.pitch (Variables|Default|GetInitial%20Bar%20Tip%20Rotation)) (+ (* _rotation_2 (Variables|Default|GetMax%20Bar%20Tip%20Rotation%20%28degrees%29)) (.yaw (Variables|Default|GetInitial%20Bar%20Tip%20Rotation)))) false false)
                  (goto _label)
                  (else
                    (Transformation|SetRelativeRotation _bartip_2 (Math|Rotator|MakeRotator (.roll (Variables|Default|GetInitial%20Bar%20Tip%20Rotation)) (.pitch (Variables|Default|GetInitial%20Bar%20Tip%20Rotation)) (- (.yaw (Variables|Default|GetInitial%20Bar%20Tip%20Rotation)) (* _rotation_2 (Variables|Default|GetMax%20Bar%20Tip%20Rotation%20%28degrees%29)))) false false)
                    (goto _label))))
              (:Finished
                (Variables|Default|SetBar%20Tip%20Is%20Rotating false)
                (|CallParentFunction 0)))))))))

(fn ConstructionScript
  (|CallParentFunction))