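; Cabinet Blueprint whose two doors swing open on the Lookingat event, hold, then close automatically, with an IsInUse flag blocking retriggers.
; OpeningTimeline and a reversed ClosingTimeline drive door yaw from stored starting rotations, with configurable speed, angle and direction.
; The top door uses an offset on the timeline value to trail the bottom one when opening.
; Open and close sounds play at world origin, and debug prints are optional.
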(event EventLookingat
  (params (HitComponent :type Actor%20Component%20Object%20Reference))
  (bind _debug (Variables|Default|GetDebug))
  (bind _debug_2 (Variables|Default|GetDebug))
  (bind _debug_3 (Variables|Default|GetDebug))
  (bind _debug_4 (Variables|Default|GetDebug))
  (bind _bottomdoor (Variables|Default|GetBottomDoor))
  ;[1 1 1] Open the doors then close after waiting 2 seconds
  ;;[1 1 1] Initialize starting rotation of doors
  (if (not (Variables|Default|GetIsInUse))
    (Variables|Default|SetIsInUse true)
    (Variables|Default|SetTop%20Door%20Rotation (Variables|/Script/Engine.SceneComponent|GetRelativeRotation (Variables|Default|GetBottomDoor)))
    (Variables|Default|SetBottom%20Door%20Rotation (Variables|/Script/Engine.SceneComponent|GetRelativeRotation (Variables|Default|GetTopDoor)))
    (Variables|Default|SetIsMoving true)
    (Components|Timeline|SetPlayRate (Variables|Default|GetOpeningTimeline) (Variables|Default|GetDoor%20Movement%20Rate))
    (Audio|PlaySoundatLocation "/Game/MRPGT/MedievalBuildings01/Audio/SoundCues/CabinetOpen_Cue.CabinetOpen_Cue" "0, 0, 0" "0, 0, 0" 1.0 1.0 0.0 0 0 0 0)
    ;;[1 1 1] Loop through a timeline for 1 second
    (bind _doorangle (Timeline|OpeningTimeline PlayFromStart)
      (:Update
        ;;[1 1 1] Rotate bottom door in the z axis every loop iteration
        (if (Variables|Default|GetOpenTheDoorsTheOtherWay?)
          (Transformation|SetRelativeRotation (Variables|Default|GetBottomDoor) (Math|Rotator|MakeRotator (.roll (Variables|Default|GetBottom%20Door%20Rotation)) (.pitch (Variables|Default|GetBottom%20Door%20Rotation)) (- (.yaw (Variables|Default|GetBottom%20Door%20Rotation)) (* _doorangle (Variables|Default|GetMax%20Door%20Rotation)))) false false)
          (else
            (Transformation|SetRelativeRotation (Variables|Default|GetBottomDoor) (Math|Rotator|MakeRotator (.roll (Variables|Default|GetBottom%20Door%20Rotation)) (.pitch (Variables|Default|GetBottom%20Door%20Rotation)) (+ (* _doorangle (Variables|Default|GetMax%20Door%20Rotation)) (.yaw (Variables|Default|GetBottom%20Door%20Rotation)))) false false)))
        ;;[1 1 1] Debug info
        (Development|PrintString (Utilities|String|Append "Opening." "Bottom door yaws:" (Utilities|String|ToString(Float) (.yaw (Variables|Default|GetBottom%20Door%20Rotation)))) _debug_4 _debug_4)
        ;;[1 1 1] Start moving top drawer a little later than the bottom drawer
        (if (> (- _doorangle (Variables|Default|GetDelayFor2ndDoor%28secs%29)) 0.0)
          (if (Variables|Default|GetOpenTheDoorsTheOtherWay?)
            (Transformation|SetRelativeRotation (Variables|Default|GetTopDoor) (Math|Rotator|MakeRotator (.roll (Variables|Default|GetBottom%20Door%20Rotation)) (.pitch (Variables|Default|GetBottom%20Door%20Rotation)) (- (.yaw (Variables|Default|GetBottom%20Door%20Rotation)) (* (- _doorangle (Variables|Default|GetDelayFor2ndDoor%28secs%29)) (- (Variables|Default|GetMax%20Door%20Rotation) 4.0)))) false false)
            (else
              (Transformation|SetRelativeRotation (Variables|Default|GetTopDoor) (Math|Rotator|MakeRotator (.roll (Variables|Default|GetBottom%20Door%20Rotation)) (.pitch (Variables|Default|GetBottom%20Door%20Rotation)) (+ (* (- _doorangle (Variables|Default|GetDelayFor2ndDoor%28secs%29)) (- (Variables|Default|GetMax%20Door%20Rotation) 4.0)) (.yaw (Variables|Default|GetBottom%20Door%20Rotation)))) false false)))))
      (:Finished
        (Development|PrintString "Fully opened" _debug _debug)
        ;;[1 1 1] Set status variables after opening completed
        (Variables|Default|SetIsMoving false)
        (Variables|Default|SetIs%20Fully%20Open true)
        ;;[1 1 1] Pause when drawer is completely open
        (Utilities|FlowControl|Delay (Variables|Default|GetOpened%20Duration%20%28secs%29))
        ;;[1 1 1] Set status variables to indicate closing is beginning
        (Variables|Default|SetIsMoving true)
        (Variables|Default|SetIs%20Fully%20Open false)
        ;;[1 1 1] Do the reverse to close the bottom drawer
        (Components|Timeline|SetPlayRate (Variables|Default|GetClosingTimeline) (Variables|Default|GetDoor%20Movement%20Rate))
        (bind _doorangle_2 (Timeline|ClosingTimeline ReverseFromEnd)
          (:Update
            (if (Variables|Default|GetOpenTheDoorsTheOtherWay?)
              (Transformation|SetRelativeRotation _bottomdoor (Math|Rotator|MakeRotator (.roll (Variables|Default|GetTop%20Door%20Rotation)) (.pitch (Variables|Default|GetTop%20Door%20Rotation)) (- (.yaw (Variables|Default|GetTop%20Door%20Rotation)) (* _doorangle_2 (Variables|Default|GetMax%20Door%20Rotation)))) false false)
              (else
                (Transformation|SetRelativeRotation _bottomdoor (Math|Rotator|MakeRotator (.roll (Variables|Default|GetTop%20Door%20Rotation)) (.pitch (Variables|Default|GetTop%20Door%20Rotation)) (+ (* _doorangle_2 (Variables|Default|GetMax%20Door%20Rotation)) (.yaw (Variables|Default|GetTop%20Door%20Rotation)))) false false)))
            ;;[1 1 1] Debug info
            (Development|PrintString (Utilities|String|Append "Closing. " "Bottom door yaw:" (Utilities|String|ToString(Float) (.yaw (Variables|Default|GetTop%20Door%20Rotation)))) _debug_3 _debug_3)
            ;;[1 1 1] Start moving bottom drawer a little later than the top drawer
            (if (> (- _doorangle_2 (Variables|Default|GetDelayFor2ndDoor%28secs%29)) 0.0)
              (if (Variables|Default|GetOpenTheDoorsTheOtherWay?)
                (Transformation|SetRelativeRotation (Variables|Default|GetTopDoor) (Math|Rotator|MakeRotator (.roll (Variables|Default|GetBottom%20Door%20Rotation)) (.pitch (Variables|Default|GetBottom%20Door%20Rotation)) (- (.yaw (Variables|Default|GetBottom%20Door%20Rotation)) (* (- _doorangle_2 (Variables|Default|GetDelayFor2ndDoor%28secs%29)) (- (Variables|Default|GetMax%20Door%20Rotation) 4.0)))) false false)
                (else
                  (Transformation|SetRelativeRotation (Variables|Default|GetTopDoor) (Math|Rotator|MakeRotator (.roll (Variables|Default|GetBottom%20Door%20Rotation)) (.pitch (Variables|Default|GetBottom%20Door%20Rotation)) (+ (* (- _doorangle_2 (Variables|Default|GetDelayFor2ndDoor%28secs%29)) (- (Variables|Default|GetMax%20Door%20Rotation) 4.0)) (.yaw (Variables|Default|GetBottom%20Door%20Rotation)))) false false)))))
          (:Finished
            (Development|PrintString "Fully closed" _debug_2 _debug_2)
            (Variables|Default|SetIsInUse false)
            (Audio|PlaySoundatLocation "/Game/MRPGT/MedievalBuildings01/Audio/SoundCues/CabinetClose_Cue.CabinetClose_Cue" "0, 0, 0" "0, 0, 0" 1.0 1.0 0.0 0 0 0 0)))))))

(fn ConstructionScript)