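; BP_Candle_B is an interactable candle prop with a flame particle and a light that can be lit or blown out.
; The construction script applies exposed color, visibility, intensity, radius and contact shadow settings.
; Both the Lookingat and Interact events toggle flame and light visibility.
; GetObjectName picks the "Blow Out Candle" or "Light Candle" prompt from IsVisible, which the toggle never updates.
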(event EventInteract
  (params (HitComponent :type Actor%20Component%20Object%20Reference) (InteractingActor :type Actor%20Object%20Reference))
  ;[1 1 1] E key will toggle light
  (Rendering|ToggleVisibility (Variables|Default|GetP_CandleFlame1) false))

(event EventLookingat
  (params (HitComponent :type Actor%20Component%20Object%20Reference))
  ;[1 1 1] E key will toggle light
  (Rendering|ToggleVisibility (Variables|Default|GetP_CandleFlame1) false))

(fn ConstructionScript
  (Rendering|Components|Light|SetLightColor (Variables|Default|GetLight) (Variables|Default|GetLight%20Color) true)
  (Rendering|SetVisibility (Variables|Default|GetLight) (Variables|Default|GetIs%20Visible) false)
  (Rendering|Lighting|SetAttenuationRadius (Variables|Default|GetLight) (Variables|Default|GetAttenuation%20Radius))
  (Rendering|Components|Light|SetIntensity (Variables|Default|GetLight) (Variables|Default|GetIntensity))
  (Class|PointLightComponent|SetSourceRadius (Variables|Default|GetLight) (Variables|Default|GetSource%20Radius))
  (Variables|/Script/Engine.LightComponent|SetContactShadowLength (Variables|Default|GetLight) (Variables|Default|GetContact%20Shadow%20Length)))

(fn GetID
  (return ""))

(fn GetLauncherActor
  (return 0))

(fn GetObjectName
  (if (Variables|Default|GetIs%20Visible)
    (return "Blow Out Candle")
    (else
      (return "Light Candle"))))

(fn IsProjectile
  (return false))