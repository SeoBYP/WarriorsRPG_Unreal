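; A configurable Viking medium house building Blueprint for level dressing, assembled from Roof, Base and Porch mesh components.
; The construction script swaps the roof mesh by RoofType and the siding material, set by slot name on the base, by BaseType.
; HasPorch toggles both the porch's visibility and its collision.
; All variation resolves at construction; the event graph holds only disabled placeholder events.
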(event EventBeginPlay)

(event Collision|EventActorBeginOverlap
  (params (OtherActor :type Actor%20Object%20Reference)))

(event EventTick
  (params (DeltaSeconds :type Float%20%28single-precision%29)))

(fn ConstructionScript
  (Utilities|FlowControl|Sequence
    (:then_0
      (switch Utilities|FlowControl|Switch|SwitchonVikingRoofTypeEnum (Variables|Customization|GetRoofType)
        (:NewEnumerator0
          (Components|StaticMesh|SetStaticMesh (Variables|Default|GetRoof) "/Game/MRPGT/MedievalBuildings01/StaticMeshes/VikingMediumHouse/SM_VMH_Roof_A.SM_VMH_Roof_A"))
        (:NewEnumerator1
          (Components|StaticMesh|SetStaticMesh (Variables|Default|GetRoof) "/Game/MRPGT/MedievalBuildings01/StaticMeshes/VikingMediumHouse/SM_VMH_Roof_B.SM_VMH_Roof_B"))
        (:NewEnumerator8
          (Components|StaticMesh|SetStaticMesh (Variables|Default|GetRoof) "/Game/MRPGT/MedievalBuildings01/StaticMeshes/VikingMediumHouse/SM_VMH_Roof_C.SM_VMH_Roof_C"))))
    (:then_1
      (switch Utilities|FlowControl|Switch|SwitchonVikingBaseTypeEnum (Variables|Customization|GetBaseType)
        (:NewEnumerator0
          (Rendering|Material|SetMaterialbyName (Variables|Default|GetBase) "M_Siding" "/Game/MRPGT/MedievalBuildings01/MaterialInstances/M_Wooden_Siding02.M_Wooden_Siding02"))
        (:NewEnumerator1
          (Rendering|Material|SetMaterialbyName (Variables|Default|GetBase) "M_Siding" "/Game/MRPGT/MedievalBuildings01/MaterialInstances/M_Wattle_and_Daub_with_Dirt.M_Wattle_and_Daub_with_Dirt"))
        (:NewEnumerator9
          (Rendering|Material|SetMaterialbyName (Variables|Default|GetBase) "M_Siding" "/Game/MRPGT/MedievalBuildings01/MaterialInstances/M_WoodenSiding008_VertBlend.M_WoodenSiding008_VertBlend"))))
    (:then_2
      (Rendering|SetVisibility (Variables|Default|GetPorch) (Variables|Customization|GetHasPorch?) false)
      (if (Variables|Customization|GetHasPorch?)
        (Collision|SetCollisionEnabled (Variables|Default|GetPorch) "QueryAndPhysics")
        (else
          (Collision|SetCollisionEnabled (Variables|Default|GetPorch) "NoCollision"))))))