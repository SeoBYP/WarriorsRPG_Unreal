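; Prefab large peasant's house (variant B) building Blueprint with customizable wattle-and-daub, wood and front door colors.
; The Construction Script loops over static mesh children of SharedRoot, pushing daub tint, wood tint and wood desaturation (for an aged look) into material parameters.
; A second pass applies tint, intensity and desaturation settings to the meshes under FrontDoor.
; The event graph holds no active logic.
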(event EventBeginPlay)

(event Collision|EventActorBeginOverlap
  (params (OtherActor :type Actor%20Object%20Reference)))

(event EventTick
  (params (DeltaSeconds :type Float%20%28single-precision%29)))

(fn ConstructionScript
  ;[1 1 1] Set the color of the daub on all meshes when the Wattle and Daub Paint Color variable is changed
  (Utilities|FlowControl|Sequence
    (:then_0
      (for _array_element (Components|GetChildrenComponents (Variables|Default|GetSharedRoot) true)
        (bind _asstatic_mesh_component (Utilities|Casting|CastToStaticMeshComponent _array_element))
        (Rendering|Material|SetVectorParameterValueonMaterials _asstatic_mesh_component "Base Daub Color Tint" (Math|Conversions|ToVector(LinearColor) (Variables|Customization|GetWattle%20and%20Daub%20Paint%20Color)))
        (Rendering|Material|SetVectorParameterValueonMaterials _asstatic_mesh_component "Top Daub Color Tint" (Math|Conversions|ToVector(LinearColor) (Variables|Customization|GetWattle%20and%20Daub%20Paint%20Color)))
        ;[1 1 1] Set the color tint of the wood on all meshes when the Wood Tint variable is changed
        (Rendering|Material|SetVectorParameterValueonMaterials _asstatic_mesh_component "Wood Color Tint" (Math|Conversions|ToVector(LinearColor) (Variables|Customization|GetWood%20Tint)))
        ;[1 1 1] Set the desaturation of the wood. More desaturation = older looking wood
        (Rendering|Material|SetScalarParameterValueonMaterials _asstatic_mesh_component "Wood Desaturation Amount" (Variables|Customization|GetWood%20Desaturation%20Amount))))
    (:then_1
      ;[1 1 1] Set the color of the front door
      (for _array_element_2 (Components|GetChildrenComponents (Variables|Default|GetFrontDoor) true)
        (bind _asstatic_mesh_component_2 (Utilities|Casting|CastToStaticMeshComponent _array_element_2))
        (Rendering|Material|SetVectorParameterValueonMaterials _asstatic_mesh_component_2 "Front Door Color Tint" (Math|Conversions|ToVector(LinearColor) (Variables|Customization|GetFront%20Door%20Tint)))
        (Rendering|Material|SetScalarParameterValueonMaterials _asstatic_mesh_component_2 "Front Door Color Intensity" (Variables|Customization|GetFront%20Door%20Color%20Intensity))
        (Rendering|Material|SetScalarParameterValueonMaterials _asstatic_mesh_component_2 "Front Door Tint Intensity" (Variables|Customization|GetFront%20Door%20Tint%20Intensity))
        (Rendering|Material|SetScalarParameterValueonMaterials _asstatic_mesh_component_2 "Front Door Desaturation Amount" (Variables|Customization|GetFront%20Door%20Desaturation%20Amount))))))