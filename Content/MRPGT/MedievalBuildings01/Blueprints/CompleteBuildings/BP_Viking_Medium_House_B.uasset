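; Configurable medium Viking house building (variant B) whose look is set through exposed options and applied in the Construction Script.
; Roof type swaps the roof mesh and toggles matching vertical or shingle decal groups, while base type replaces the siding material by slot name.
; Dragon ornament type sets or clears both head meshes, and a porch flag toggles its visibility and collision.
; The event graph holds no runtime logic.
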(event EventBeginPlay)

(event Collision|EventActorBeginOverlap
  (params (OtherActor :type Actor%20Object%20Reference)))

(event EventTick
  (params (DeltaSeconds :type Float%20%28single-precision%29)))

(fn ConstructionScript
  (Utilities|FlowControl|Sequence
    (:then_0
      (switch Utilities|FlowControl|Switch|SwitchonVikingRoofTypeEnum (Variables|Customization|GetRoofType)
        (:NewEnumerator0
          (Components|StaticMesh|SetStaticMesh (Variables|Default|GetRoof) "/Game/MRPGT/MedievalBuildings01/StaticMeshes/VikingMediumHouse/SM_VMH_Roof_D.SM_VMH_Roof_D")
          (Rendering|SetVisibility (Variables|Default|GetVerticalRoofDecals) true true)
          (Rendering|SetVisibility (Variables|Default|GetShingleRoofDecals) false true))
        (:NewEnumerator1
          (Components|StaticMesh|SetStaticMesh (Variables|Default|GetRoof) "/Game/MRPGT/MedievalBuildings01/StaticMeshes/VikingMediumHouse/SM_VMH_Roof_E.SM_VMH_Roof_E")
          (Rendering|SetVisibility (Variables|Default|GetVerticalRoofDecals) false true)
          (Rendering|SetVisibility (Variables|Default|GetShingleRoofDecals) true true))
        (:NewEnumerator8
          (Components|StaticMesh|SetStaticMesh (Variables|Default|GetRoof) "/Game/MRPGT/MedievalBuildings01/StaticMeshes/VikingMediumHouse/SM_VMH_Roof_F.SM_VMH_Roof_F")
          (Rendering|SetVisibility (Variables|Default|GetVerticalRoofDecals) false true)
          (Rendering|SetVisibility (Variables|Default|GetShingleRoofDecals) true true))))
    (:then_1
      (switch Utilities|FlowControl|Switch|SwitchonVikingBaseTypeEnum (Variables|Customization|GetBaseType)
        (:NewEnumerator0
          (Rendering|Material|SetMaterialbyName (Variables|Default|GetBase) "M_Siding" "/Game/MRPGT/MedievalBuildings01/MaterialInstances/M_Wooden_Siding02.M_Wooden_Siding02"))
        (:NewEnumerator1
          (Rendering|Material|SetMaterialbyName (Variables|Default|GetBase) "M_Siding" "/Game/MRPGT/MedievalBuildings01/MaterialInstances/M_Wattle_and_Daub_with_Dirt.M_Wattle_and_Daub_with_Dirt"))
        (:NewEnumerator9
          (Rendering|Material|SetMaterialbyName (Variables|Default|GetBase) "M_Siding" "/Game/MRPGT/MedievalBuildings01/MaterialInstances/M_WoodenSiding008_VertBlend.M_WoodenSiding008_VertBlend"))))
    (:then_2
      (switch Utilities|FlowControl|Switch|SwitchonVikingDragonOrnamentEnum (Variables|Customization|GetDragon%20Ornament)
        (:NewEnumerator0
          (Components|StaticMesh|SetStaticMesh (Variables|Default|GetDragon_Head1) "/Game/MRPGT/MedievalBuildings01/StaticMeshes/VikingMediumHouse/SM_Viking_Dragon_Head_A.SM_Viking_Dragon_Head_A")
          (Components|StaticMesh|SetStaticMesh (Variables|Default|GetDragon_Head2) "/Game/MRPGT/MedievalBuildings01/StaticMeshes/VikingMediumHouse/SM_Viking_Dragon_Head_A.SM_Viking_Dragon_Head_A"))
        (:NewEnumerator1
          (Components|StaticMesh|SetStaticMesh (Variables|Default|GetDragon_Head1) "/Game/MRPGT/MedievalBuildings01/StaticMeshes/VikingLonghouse/SM_VLH_Dragon_Head_A.SM_VLH_Dragon_Head_A")
          (Components|StaticMesh|SetStaticMesh (Variables|Default|GetDragon_Head2) "/Game/MRPGT/MedievalBuildings01/StaticMeshes/VikingLonghouse/SM_VLH_Dragon_Head_A.SM_VLH_Dragon_Head_A"))
        (:NewEnumerator8
          (Components|StaticMesh|SetStaticMesh (Variables|Default|GetDragon_Head1) 0)
          (Components|StaticMesh|SetStaticMesh (Variables|Default|GetDragon_Head2) 0))))
    (:then_3
      (Rendering|SetVisibility (Variables|Default|GetPorch) (Variables|Customization|GetHas%20Porch?) false)
      (if (Variables|Customization|GetHas%20Porch?)
        (Collision|SetCollisionEnabled (Variables|Default|GetPorch) "QueryAndPhysics")
        (else
          (Collision|SetCollisionEnabled (Variables|Default|GetPorch) "NoCollision"))))))