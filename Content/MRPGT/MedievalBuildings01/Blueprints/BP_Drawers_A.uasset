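; Drawer prop Blueprint that opens its top and bottom drawers when its Lookingat event fires, then closes them after a configurable pause.
; Opening and closing timelines slide the drawers along local Y from their saved starting positions at an adjustable rate, with sound cues.
; The bottom drawer trails the top one with a slightly shorter travel.
; An in-use flag blocks retriggering until closing finishes, and a Debug flag toggles print logging.
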(event EventLookingat
  (params (HitComponent :type Actor%20Component%20Object%20Reference))
  (bind _debug (Variables|Default|GetDebug))
  (bind _debug_2 (Variables|Default|GetDebug))
  (bind _debug_3 (Variables|Default|GetDebug))
  (bind _debug_4 (Variables|Default|GetDebug))
  ;[1 1 1] Open the drawer then close it after waiting 2 seconds
  ;;[1 1 1] Initialize starting location of drawers
  (if (not (Variables|Default|GetIsInUse))
    (Variables|Default|SetIsInUse true)
    (Variables|Default|SetTop%20Drawer%20Location (Transformation|GetRelativeTransform (Variables|Default|GetTopDrawer)))
    (Variables|Default|SetBottom%20Drawer%20Location (Transformation|GetRelativeTransform (Variables|Default|GetBottomDrawer)))
    (Variables|Default|SetIsMoving true)
    (Components|Timeline|SetPlayRate (Variables|Default|GetOpening_Timeline) (Variables|Default|GetDrawer%20Movement%20Rate))
    (Audio|PlaySoundatLocation "/Game/MRPGT/MedievalBuildings01/Audio/SoundCues/DrawerOpen_Cue.DrawerOpen_Cue" "0, 0, 0" "0, 0, 0" 1.0 1.0 0.0 0 0 0 0)
    ;;[1 1 1] Loop through a timeline for 1 second
    (bind _drawerposition (Timeline|Opening_Timeline PlayFromStart)
      (:Update
        ;;[1 1 1] Move drawer in the y direction every loop iteration (x and z locations doesnt change)
        (Transformation|SetRelativeLocation (Variables|Default|GetTopDrawer) (Math|Vector|MakeVector (.x (.location (Variables|Default|GetTop%20Drawer%20Location))) (+ (* _drawerposition (Variables|Default|GetMax%20Drawer%20Extent)) (.y (.location (Variables|Default|GetTop%20Drawer%20Location)))) (.z (.location (Variables|Default|GetTop%20Drawer%20Location)))) false false)
        ;;[1 1 1] Debug info
        (Development|PrintString (Utilities|String|Append "Opening." "Top drawer location:" (Utilities|String|ToString(Vector) (.location (Variables|Default|GetTop%20Drawer%20Location)))) _debug_4 _debug_4)
        ;;[1 1 1] Start moving bottom drawer a little later than the top drawer
        (if (> (- _drawerposition 0.2) 0.0)
          (Transformation|SetRelativeLocation (Variables|Default|GetBottomDrawer) (Math|Vector|MakeVector (.x (.location (Variables|Default|GetBottom%20Drawer%20Location))) (+ (* (- _drawerposition 0.2) (- (Variables|Default|GetMax%20Drawer%20Extent) 4.0)) (.y (.location (Variables|Default|GetBottom%20Drawer%20Location)))) (.z (.location (Variables|Default|GetBottom%20Drawer%20Location)))) false false)))
      (:Finished
        (Development|PrintString "Fully opened" _debug _debug)
        ;;[1 1 1] Set status variables after opening completed
        (Variables|Default|SetIsMoving false)
        (Variables|Default|SetIs%20Fully%20Open true)
        ;;[1 1 1] Pause when drawer is completely open
        (Utilities|FlowControl|Delay (Variables|Default|GetOpened%20Duration%20%28secs%29))
        ;;[1 1 1] Set status variables to indicate closing is beginning
        (Variables|Default|SetIsMoving true)
        (Variables|Default|SetIs%20Fully%20Open false)
        ;;[1 1 1] Do the reverse to close the top drawer
        (Components|Timeline|SetPlayRate (Variables|Default|GetClosing_Timeline) (Variables|Default|GetDrawer%20Movement%20Rate))
        (Audio|PlaySoundatLocation "/Game/MRPGT/MedievalBuildings01/Audio/SoundCues/DrawerClose_Cue.DrawerClose_Cue" "0, 0, 0" "0, 0, 0" 1.0 1.0 0.0 0 0 0 0)
        (bind _drawerposition_2 (Timeline|Closing_Timeline ReverseFromEnd)
          (:Update
            (Transformation|SetRelativeLocation (Variables|Default|GetTopDrawer) (Math|Vector|MakeVector (.x (.location (Variables|Default|GetTop%20Drawer%20Location))) (+ (* _drawerposition_2 (Variables|Default|GetMax%20Drawer%20Extent)) (.y (.location (Variables|Default|GetTop%20Drawer%20Location)))) (.z (.location (Variables|Default|GetTop%20Drawer%20Location)))) false false)
            ;;[1 1 1] Debug info
            (Development|PrintString (Utilities|String|Append "Closing. " "Top drawer Y location:" (Utilities|String|ToString(Vector) (.location (Variables|Default|GetTop%20Drawer%20Location)))) _debug_3 _debug_3)
            ;;[1 1 1] Start moving bottom drawer a little later than the top drawer
            (if (> (- _drawerposition_2 0.2) 0.0)
              (Transformation|SetRelativeLocation (Variables|Default|GetBottomDrawer) (Math|Vector|MakeVector (.x (.location (Variables|Default|GetBottom%20Drawer%20Location))) (+ (* (- _drawerposition_2 0.2) (- (Variables|Default|GetMax%20Drawer%20Extent) 4.0)) (.y (.location (Variables|Default|GetBottom%20Drawer%20Location)))) (.z (.location (Variables|Default|GetBottom%20Drawer%20Location)))) false false)))
          (:Finished
            (Development|PrintString "Fully closed" _debug_2 _debug_2)
            (Variables|Default|SetIsInUse false)))))))

(fn ConstructionScript)