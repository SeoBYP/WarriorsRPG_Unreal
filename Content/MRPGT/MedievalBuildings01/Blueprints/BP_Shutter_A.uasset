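; BP_Shutter_A is an interactable window shutter with an optional security bar, swung open and closed by timelines with sounds.
; Opening lifts any visible bar before rotating the shutter; closing rotates the shutter before lowering the bar.
; An optional partner shutter shares the IsRotating lock, and bar visibility enforces that the barred shutter opens first and closes last.
; The construction script can pre-open it, with configurable rotation directions and bar axis.
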(event EventInteract
  (params (HitComponent :type Actor%20Component%20Object%20Reference) (InteractingActor :type Actor%20Object%20Reference))
  (bind _shutter (Variables|Default|GetShutter))
  (bind _debug (Variables|Default|GetDebug))
  (bind _debug_2 (Variables|Default|GetDebug))
  (bind _debug_3 (Variables|Default|GetDebug))
  (bind _debug_4 (Variables|Default|GetDebug))
  (bind _debug_5 (Variables|Default|GetDebug))
  (bind _debug_6 (Variables|Default|GetDebug))
  (bind _debug_7 (Variables|Default|GetDebug))
  (bind _debug_8 (Variables|Default|GetDebug))
  (bind _shutterpartner (Variables|Default|GetShutterPartner))
  (bind _shutterpartner_2 (Variables|Default|GetShutterPartner))
  (bind _shutterpartner_3 (Variables|Default|GetShutterPartner))
  (bind _shutterpartner_4 (Variables|Default|GetShutterPartner))
  (bind _shutterpartner_5 (Variables|Default|GetShutterPartner))
  (bind _shutterpartner_6 (Variables|Default|GetShutterPartner))
  (bind _bar (Variables|Default|GetBar))
  (bind _bar_2 (Variables|Default|GetBar))
  (bind _shutter_2 (Variables|Default|GetShutter))
  (bind _debug_9 (Variables|Default|GetDebug))
  ;[1 1 1] Initialise vars
  (if (Variables|Default|GetCan%20Be%20Opened?)
    (if (Variables|Default|GetIsRotating)
      (Development|PrintString "Shutter already being used. Please wait." _debug_6 _debug_6)
      (else
        (Variables|Default|SetIsRotating true)
        (if (Utilities|IsValid _shutterpartner_3)
          (Variables|BP_Shutter_A_C|SetIsRotating _shutterpartner_3 true))
        (Variables|Default|SetInitial%20Shutter%20Rotation (.rotation (Transformation|GetRelativeTransform (Variables|Default|GetShutter))))
        (Variables|Default|SetInitial%20Bar%20Rotation (.rotation (Transformation|GetRelativeTransform (Variables|Default|GetBar))))
        (Components|Timeline|SetPlayRate (Variables|Default|GetOpenShutterTimeline) (Variables|Default|GetOpen%20Close%20Rate))
        ;[1 1 1] Print some debug info
        (Development|PrintString (Utilities|String|Append "Initial shutter rotation" (Utilities|String|ToString(Rotator) (Variables|Default|GetInitial%20Shutter%20Rotation))) _debug_8 _debug_8 "(R=0.000000,G=0.660000,B=1.000000,A=1.000000)" 4.0)
        (Development|PrintString (Utilities|String|Append "Initial bar rotation" (Utilities|String|ToString(Rotator) (Variables|Default|GetInitial%20Bar%20Rotation))) _debug_8 _debug_8 "(R=0.000000,G=0.660000,B=1.000000,A=1.000000)" 4.0)
        (Development|PrintString (Utilities|String|Append "Shutter partner:" (Utilities|String|ToString(Boolean) (Utilities|IsValid (Variables|Default|GetShutterPartner)))) _debug_5 _debug_5)
        ;[1 1 1] If shutter is open then close it otherwise open it
        (if (Variables|Default|GetIsOpen)
          ;[1 1 1] If trying to close shutter then check whether any required partner shutter is closed first
          (if (Utilities|IsValid _shutterpartner_2)
            (if (Rendering|IsVisible (Variables|Default|GetBar))
              (if (Variables|BP_Shutter_A_C|GetIsOpen _shutterpartner_2)
                (Development|PrintString "You cannot close this shutter before the other shutter")
                (Variables|Default|SetIsRotating false)
                (Variables|BP_Shutter_A_C|SetIsRotating (Variables|Default|GetShutterPartner) false)
                (else
                  ;[1 1 1] Close the shutter then lower the security bar
                  (Development|PrintString "Closing shutter" _debug_2 _debug_2 :!label _label)
                  (Audio|PlaySoundatLocation (Variables|Default|GetShutterClosingSound) "0, 0, 0" "0, 0, 0" 1.0 1.0 0.0 0 0 0 0)
                  (bind _rotation (Timeline|CloseShutterTimeline PlayFromStart)
                    (:Update
                      (if (Variables|Default|GetReverse%20Shutter%20Open%20Direction?)
                        (Transformation|SetRelativeRotation _shutter_2 (Math|Rotator|MakeRotator (.roll (Variables|Default|GetInitial%20Shutter%20Rotation)) (.pitch (Variables|Default|GetInitial%20Shutter%20Rotation)) (- (.yaw (Variables|Default|GetInitial%20Shutter%20Rotation)) (* _rotation (Variables|Default|GetMax%20Shutter%20Rotation%20%28degrees%29)))) false false)
                        (else
                          (Transformation|SetRelativeRotation _shutter_2 (Math|Rotator|MakeRotator (.roll (Variables|Default|GetInitial%20Shutter%20Rotation)) (.pitch (Variables|Default|GetInitial%20Shutter%20Rotation)) (+ (* _rotation (Variables|Default|GetMax%20Shutter%20Rotation%20%28degrees%29)) (.yaw (Variables|Default|GetInitial%20Shutter%20Rotation)))) false false))))
                    (:Finished
                      (Audio|PlaySoundatLocation (Variables|Default|GetShutterClosedSound) "0, 0, 0" "0, 0, 0" 1.0 1.0 0.0 0 0 0 0)
                      (if (Rendering|IsVisible (Variables|Default|GetBar))
                        (Development|PrintString "Lowering bar" _debug_3 _debug_3)
                        (Variables|Default|SetInitial%20Bar%20Rotation (Variables|/Script/Engine.SceneComponent|GetRelativeRotation (Variables|Default|GetBar)))
                        (Audio|PlaySoundatLocation (Variables|Default|GetBarLoweringSound) "0, 0, 0" "0, 0, 0" 1.0 1.0 0.0 0 0 0 0)
                        (bind _rotation_2 (Timeline|LowerBarTimeline PlayFromStart)
                          (:Update
                            (if (Variables|Default|GetReverse%20Bar%20Rotation%20Direction?)
                              (switch Utilities|FlowControl|Switch|SwitchonAxisEnum (Variables|Default|GetBar%20Rotation%20Axis)
                                (:NewEnumerator0
                                  (Transformation|SetRelativeRotation _bar_2 (Math|Rotator|MakeRotator (- (.roll (Variables|Default|GetInitial%20Bar%20Rotation)) (* _rotation_2 (Variables|Default|GetMax%20Bar%20Rotation%20%28degrees%29))) (.pitch (Variables|Default|GetInitial%20Bar%20Rotation)) (.yaw (Variables|Default|GetInitial%20Bar%20Rotation))) false false))
                                (:NewEnumerator1
                                  (Transformation|SetRelativeRotation _bar_2 (Math|Rotator|MakeRotator (.roll (Variables|Default|GetInitial%20Bar%20Rotation)) (- (.pitch (Variables|Default|GetInitial%20Bar%20Rotation)) (* _rotation_2 (Variables|Default|GetMax%20Bar%20Rotation%20%28degrees%29))) (.yaw (Variables|Default|GetInitial%20Bar%20Rotation))) false false))
                                (:NewEnumerator2
                                  (Transformation|SetRelativeRotation _bar_2 (Math|Rotator|MakeRotator (.roll (Variables|Default|GetInitial%20Bar%20Rotation)) (.pitch (Variables|Default|GetInitial%20Bar%20Rotation)) (- (.yaw (Variables|Default|GetInitial%20Bar%20Rotation)) (* _rotation_2 (Variables|Default|GetMax%20Bar%20Rotation%20%28degrees%29)))) false false)))
                              (else
                                (switch Utilities|FlowControl|Switch|SwitchonAxisEnum (Variables|Default|GetBar%20Rotation%20Axis)
                                  (:NewEnumerator0
                                    (Transformation|SetRelativeRotation _bar_2 (Math|Rotator|MakeRotator (+ (* _rotation_2 (Variables|Default|GetMax%20Bar%20Rotation%20%28degrees%29)) (.roll (Variables|Default|GetInitial%20Bar%20Rotation))) (.pitch (Variables|Default|GetInitial%20Bar%20Rotation)) (.yaw (Variables|Default|GetInitial%20Bar%20Rotation))) false false))
                                  (:NewEnumerator1
                                    (Transformation|SetRelativeRotation _bar_2 (Math|Rotator|MakeRotator (.roll (Variables|Default|GetInitial%20Bar%20Rotation)) (+ (* _rotation_2 (Variables|Default|GetMax%20Bar%20Rotation%20%28degrees%29)) (.pitch (Variables|Default|GetInitial%20Bar%20Rotation))) (.yaw (Variables|Default|GetInitial%20Bar%20Rotation))) false false))
                                  (:NewEnumerator2
                                    (Transformation|SetRelativeRotation _bar_2 (Math|Rotator|MakeRotator (.roll (Variables|Default|GetInitial%20Bar%20Rotation)) (.pitch (Variables|Default|GetInitial%20Bar%20Rotation)) (+ (* _rotation_2 (Variables|Default|GetMax%20Bar%20Rotation%20%28degrees%29)) (.yaw (Variables|Default|GetInitial%20Bar%20Rotation)))) false false)))))
                            (Development|PrintString (Utilities|String|Append "Bar rotation:" (Utilities|String|ToString(Rotator) (.Rotation (Math|Transform|BreakTransform (Transformation|GetRelativeTransform _bar_2))))) _debug_7 _debug_7 "(R=1.000000,G=0.000000,B=0.036710,A=1.000000)"))
                          (:Finished
                            (Variables|Default|SetIsOpen false :!label _label_2)
                            (Variables|Default|SetIsRotating false)
                            (if (Utilities|IsValid _shutterpartner_4)
                              (Variables|BP_Shutter_A_C|SetIsRotating _shutterpartner_4 false))
                            (Audio|PlaySoundatLocation (Variables|Default|GetBarLoweredSound) "0, 0, 0" "0, 0, 0" 1.0 1.0 0.0 0 0 0 0)))
                        (else
                          (goto _label_2)))))))
              (else
                (goto _label)))
            (else
              (goto _label)))
          (else
            ;[1 1 1] Check for a partner shutter and if there is one then check its open, if its still closed then this shutter wont open (because the security bar is still in the lowered position)
            (if (Utilities|IsValid _shutterpartner)
              (if (Rendering|IsVisible (Variables|BP_Shutter_A_C|GetBar _shutterpartner))
                (if (Variables|BP_Shutter_A_C|GetIsOpen _shutterpartner)
                  ;[1 1 1] Lift the security bar then open the shutter
                  (if (Rendering|IsVisible (Variables|Default|GetBar)) :!label _label_3
                    (Development|PrintString "Lifting bar" _debug_4 _debug_4)
                    (Audio|PlaySoundatLocation (Variables|Default|GetBarRaisingSound) "0, 0, 0" "0, 0, 0" 1.0 1.0 0.0 0 0 0 0)
                    (bind _rotation_3 (Timeline|LiftBarTimeline PlayFromStart)
                      (:Update
                        (if (Variables|Default|GetReverse%20Bar%20Rotation%20Direction?)
                          (switch Utilities|FlowControl|Switch|SwitchonAxisEnum (Variables|Default|GetBar%20Rotation%20Axis)
                            (:NewEnumerator0
                              (Transformation|SetRelativeRotation _bar (Math|Rotator|MakeRotator (+ (* _rotation_3 (Variables|Default|GetMax%20Bar%20Rotation%20%28degrees%29)) (.roll (Variables|Default|GetInitial%20Bar%20Rotation))) (.pitch (Variables|Default|GetInitial%20Bar%20Rotation)) (.yaw (Variables|Default|GetInitial%20Bar%20Rotation))) false false))
                            (:NewEnumerator1
                              (Transformation|SetRelativeRotation _bar (Math|Rotator|MakeRotator (.roll (Variables|Default|GetInitial%20Bar%20Rotation)) (+ (* _rotation_3 (Variables|Default|GetMax%20Bar%20Rotation%20%28degrees%29)) (.pitch (Variables|Default|GetInitial%20Bar%20Rotation))) (.yaw (Variables|Default|GetInitial%20Bar%20Rotation))) false false))
                            (:NewEnumerator2
                              (Transformation|SetRelativeRotation _bar (Math|Rotator|MakeRotator (.roll (Variables|Default|GetInitial%20Bar%20Rotation)) (.pitch (Variables|Default|GetInitial%20Bar%20Rotation)) (+ (* _rotation_3 (Variables|Default|GetMax%20Bar%20Rotation%20%28degrees%29)) (.yaw (Variables|Default|GetInitial%20Bar%20Rotation)))) false false)))
                          (else
                            (switch Utilities|FlowControl|Switch|SwitchonAxisEnum (Variables|Default|GetBar%20Rotation%20Axis)
                              (:NewEnumerator0
                                (Transformation|SetRelativeRotation _bar (Math|Rotator|MakeRotator (- (.roll (Variables|Default|GetInitial%20Bar%20Rotation)) (* _rotation_3 (Variables|Default|GetMax%20Bar%20Rotation%20%28degrees%29))) (.pitch (Variables|Default|GetInitial%20Bar%20Rotation)) (.yaw (Variables|Default|GetInitial%20Bar%20Rotation))) false false))
                              (:NewEnumerator1
                                (Transformation|SetRelativeRotation _bar (Math|Rotator|MakeRotator (.roll (Variables|Default|GetInitial%20Bar%20Rotation)) (- (.pitch (Variables|Default|GetInitial%20Bar%20Rotation)) (* _rotation_3 (Variables|Default|GetMax%20Bar%20Rotation%20%28degrees%29))) (.yaw (Variables|Default|GetInitial%20Bar%20Rotation))) false false))
                              (:NewEnumerator2
                                (Transformation|SetRelativeRotation _bar (Math|Rotator|MakeRotator (.roll (Variables|Default|GetInitial%20Bar%20Rotation)) (.pitch (Variables|Default|GetInitial%20Bar%20Rotation)) (- (.yaw (Variables|Default|GetInitial%20Bar%20Rotation)) (* _rotation_3 (Variables|Default|GetMax%20Bar%20Rotation%20%28degrees%29)))) false false)))))
                        (Development|PrintString (Utilities|String|Append "Bar rotation:" (Utilities|String|ToString(Rotator) (.Rotation (Math|Transform|BreakTransform (Transformation|GetRelativeTransform _bar))))) _debug _debug "(R=1.000000,G=0.000000,B=0.053420,A=1.000000)"))
                      (:Finished
                        (Audio|PlaySoundatLocation (Variables|Default|GetBarRaisedSound) "0, 0, 0" "0, 0, 0" 1.0 1.0 0.0 0 0 0 0)
                        (Development|PrintString "Opening shutter" _debug_9 _debug_9 :!label _label_4)
                        (bind _rotation_4 (Timeline|OpenShutterTimeline PlayFromStart)
                          (:Update
                            (if (Variables|Default|GetReverse%20Shutter%20Open%20Direction?)
                              (Transformation|SetRelativeRotation _shutter (Math|Rotator|MakeRotator (.roll (Variables|Default|GetInitial%20Shutter%20Rotation)) (.pitch (Variables|Default|GetInitial%20Shutter%20Rotation)) (+ (* _rotation_4 (Variables|Default|GetMax%20Shutter%20Rotation%20%28degrees%29)) (.yaw (Variables|Default|GetInitial%20Shutter%20Rotation)))) false false)
                              (else
                                (Transformation|SetRelativeRotation _shutter (Math|Rotator|MakeRotator (.roll (Variables|Default|GetInitial%20Shutter%20Rotation)) (.pitch (Variables|Default|GetInitial%20Shutter%20Rotation)) (- (.yaw (Variables|Default|GetInitial%20Shutter%20Rotation)) (* _rotation_4 (Variables|Default|GetMax%20Shutter%20Rotation%20%28degrees%29)))) false false))))
                          (:Finished
                            (Variables|Default|SetIsOpen true)
                            (Variables|Default|SetIsRotating false)
                            (if (Utilities|IsValid _shutterpartner_6)
                              (Variables|BP_Shutter_A_C|SetIsRotating _shutterpartner_6 false))))))
                    (else
                      (goto _label_4)))
                  (else
                    (Development|PrintString "You cannot open this shutter before the other shutter")
                    (Variables|Default|SetIsRotating false)
                    (if (Utilities|IsValid _shutterpartner_5)
                      (Variables|BP_Shutter_A_C|SetIsRotating _shutterpartner_5 false))))
                (else
                  (goto _label_3)))
              (else
                (goto _label_3)))))))))

(event EventLookingat
  (params (HitComponent :type Actor%20Component%20Object%20Reference))
  (bind _shutter (Variables|Default|GetShutter))
  (bind _debug (Variables|Default|GetDebug))
  (bind _debug_2 (Variables|Default|GetDebug))
  (bind _debug_3 (Variables|Default|GetDebug))
  (bind _debug_4 (Variables|Default|GetDebug))
  (bind _debug_5 (Variables|Default|GetDebug))
  (bind _debug_6 (Variables|Default|GetDebug))
  (bind _debug_7 (Variables|Default|GetDebug))
  (bind _debug_8 (Variables|Default|GetDebug))
  (bind _shutterpartner (Variables|Default|GetShutterPartner))
  (bind _shutterpartner_2 (Variables|Default|GetShutterPartner))
  (bind _shutterpartner_3 (Variables|Default|GetShutterPartner))
  (bind _shutterpartner_4 (Variables|Default|GetShutterPartner))
  (bind _shutterpartner_5 (Variables|Default|GetShutterPartner))
  (bind _shutterpartner_6 (Variables|Default|GetShutterPartner))
  (bind _bar (Variables|Default|GetBar))
  (bind _bar_2 (Variables|Default|GetBar))
  (bind _shutter_2 (Variables|Default|GetShutter))
  (bind _debug_9 (Variables|Default|GetDebug))
  ;[1 1 1] Initialise vars
  (if (Variables|Default|GetCan%20Be%20Opened?)
    (if (Variables|Default|GetIsRotating)
      (Development|PrintString "Shutter already being used. Please wait." _debug_6 _debug_6)
      (else
        (Variables|Default|SetIsRotating true)
        (if (Utilities|IsValid _shutterpartner_3)
          (Variables|BP_Shutter_A_C|SetIsRotating _shutterpartner_3 true))
        (Variables|Default|SetInitial%20Shutter%20Rotation (.rotation (Transformation|GetRelativeTransform (Variables|Default|GetShutter))))
        (Variables|Default|SetInitial%20Bar%20Rotation (.rotation (Transformation|GetRelativeTransform (Variables|Default|GetBar))))
        (Components|Timeline|SetPlayRate (Variables|Default|GetOpenShutterTimeline) (Variables|Default|GetOpen%20Close%20Rate))
        ;[1 1 1] Print some debug info
        (Development|PrintString (Utilities|String|Append "Initial shutter rotation" (Utilities|String|ToString(Rotator) (Variables|Default|GetInitial%20Shutter%20Rotation))) _debug_8 _debug_8 "(R=0.000000,G=0.660000,B=1.000000,A=1.000000)" 4.0)
        (Development|PrintString (Utilities|String|Append "Initial bar rotation" (Utilities|String|ToString(Rotator) (Variables|Default|GetInitial%20Bar%20Rotation))) _debug_8 _debug_8 "(R=0.000000,G=0.660000,B=1.000000,A=1.000000)" 4.0)
        (Development|PrintString (Utilities|String|Append "Shutter partner:" (Utilities|String|ToString(Boolean) (Utilities|IsValid (Variables|Default|GetShutterPartner)))) _debug_5 _debug_5)
        ;[1 1 1] If shutter is open then close it otherwise open it
        (if (Variables|Default|GetIsOpen)
          ;[1 1 1] If trying to close shutter then check whether any required partner shutter is closed first
          (if (Utilities|IsValid _shutterpartner_2)
            (if (Rendering|IsVisible (Variables|Default|GetBar))
              (if (Variables|BP_Shutter_A_C|GetIsOpen _shutterpartner_2)
                (Development|PrintString "You cannot close this shutter before the other shutter")
                (Variables|Default|SetIsRotating false)
                (Variables|BP_Shutter_A_C|SetIsRotating (Variables|Default|GetShutterPartner) false)
                (else
                  ;[1 1 1] Close the shutter then lower the security bar
                  (Development|PrintString "Closing shutter" _debug_2 _debug_2 :!label _label)
                  (Audio|PlaySoundatLocation (Variables|Default|GetShutterClosingSound) "0, 0, 0" "0, 0, 0" 1.0 1.0 0.0 0 0 0 0)
                  (bind _rotation (Timeline|CloseShutterTimeline PlayFromStart)
                    (:Update
                      (if (Variables|Default|GetReverse%20Shutter%20Open%20Direction?)
                        (Transformation|SetRelativeRotation _shutter_2 (Math|Rotator|MakeRotator (.roll (Variables|Default|GetInitial%20Shutter%20Rotation)) (.pitch (Variables|Default|GetInitial%20Shutter%20Rotation)) (- (.yaw (Variables|Default|GetInitial%20Shutter%20Rotation)) (* _rotation (Variables|Default|GetMax%20Shutter%20Rotation%20%28degrees%29)))) false false)
                        (else
                          (Transformation|SetRelativeRotation _shutter_2 (Math|Rotator|MakeRotator (.roll (Variables|Default|GetInitial%20Shutter%20Rotation)) (.pitch (Variables|Default|GetInitial%20Shutter%20Rotation)) (+ (* _rotation (Variables|Default|GetMax%20Shutter%20Rotation%20%28degrees%29)) (.yaw (Variables|Default|GetInitial%20Shutter%20Rotation)))) false false))))
                    (:Finished
                      (Audio|PlaySoundatLocation (Variables|Default|GetShutterClosedSound) "0, 0, 0" "0, 0, 0" 1.0 1.0 0.0 0 0 0 0)
                      (if (Rendering|IsVisible (Variables|Default|GetBar))
                        (Development|PrintString "Lowering bar" _debug_3 _debug_3)
                        (Variables|Default|SetInitial%20Bar%20Rotation (Variables|/Script/Engine.SceneComponent|GetRelativeRotation (Variables|Default|GetBar)))
                        (Audio|PlaySoundatLocation (Variables|Default|GetBarLoweringSound) "0, 0, 0" "0, 0, 0" 1.0 1.0 0.0 0 0 0 0)
                        (bind _rotation_2 (Timeline|LowerBarTimeline PlayFromStart)
                          (:Update
                            (if (Variables|Default|GetReverse%20Bar%20Rotation%20Direction?)
                              (switch Utilities|FlowControl|Switch|SwitchonAxisEnum (Variables|Default|GetBar%20Rotation%20Axis)
                                (:NewEnumerator0
                                  (Transformation|SetRelativeRotation _bar_2 (Math|Rotator|MakeRotator (- (.roll (Variables|Default|GetInitial%20Bar%20Rotation)) (* _rotation_2 (Variables|Default|GetMax%20Bar%20Rotation%20%28degrees%29))) (.pitch (Variables|Default|GetInitial%20Bar%20Rotation)) (.yaw (Variables|Default|GetInitial%20Bar%20Rotation))) false false))
                                (:NewEnumerator1
                                  (Transformation|SetRelativeRotation _bar_2 (Math|Rotator|MakeRotator (.roll (Variables|Default|GetInitial%20Bar%20Rotation)) (- (.pitch (Variables|Default|GetInitial%20Bar%20Rotation)) (* _rotation_2 (Variables|Default|GetMax%20Bar%20Rotation%20%28degrees%29))) (.yaw (Variables|Default|GetInitial%20Bar%20Rotation))) false false))
                                (:NewEnumerator2
                                  (Transformation|SetRelativeRotation _bar_2 (Math|Rotator|MakeRotator (.roll (Variables|Default|GetInitial%20Bar%20Rotation)) (.pitch (Variables|Default|GetInitial%20Bar%20Rotation)) (- (.yaw (Variables|Default|GetInitial%20Bar%20Rotation)) (* _rotation_2 (Variables|Default|GetMax%20Bar%20Rotation%20%28degrees%29)))) false false)))
                              (else
                                (switch Utilities|FlowControl|Switch|SwitchonAxisEnum (Variables|Default|GetBar%20Rotation%20Axis)
                                  (:NewEnumerator0
                                    (Transformation|SetRelativeRotation _bar_2 (Math|Rotator|MakeRotator (+ (* _rotation_2 (Variables|Default|GetMax%20Bar%20Rotation%20%28degrees%29)) (.roll (Variables|Default|GetInitial%20Bar%20Rotation))) (.pitch (Variables|Default|GetInitial%20Bar%20Rotation)) (.yaw (Variables|Default|GetInitial%20Bar%20Rotation))) false false))
                                  (:NewEnumerator1
                                    (Transformation|SetRelativeRotation _bar_2 (Math|Rotator|MakeRotator (.roll (Variables|Default|GetInitial%20Bar%20Rotation)) (+ (* _rotation_2 (Variables|Default|GetMax%20Bar%20Rotation%20%28degrees%29)) (.pitch (Variables|Default|GetInitial%20Bar%20Rotation))) (.yaw (Variables|Default|GetInitial%20Bar%20Rotation))) false false))
                                  (:NewEnumerator2
                                    (Transformation|SetRelativeRotation _bar_2 (Math|Rotator|MakeRotator (.roll (Variables|Default|GetInitial%20Bar%20Rotation)) (.pitch (Variables|Default|GetInitial%20Bar%20Rotation)) (+ (* _rotation_2 (Variables|Default|GetMax%20Bar%20Rotation%20%28degrees%29)) (.yaw (Variables|Default|GetInitial%20Bar%20Rotation)))) false false)))))
                            (Development|PrintString (Utilities|String|Append "Bar rotation:" (Utilities|String|ToString(Rotator) (.Rotation (Math|Transform|BreakTransform (Transformation|GetRelativeTransform _bar_2))))) _debug_7 _debug_7 "(R=1.000000,G=0.000000,B=0.036710,A=1.000000)"))
                          (:Finished
                            (Variables|Default|SetIsOpen false :!label _label_2)
                            (Variables|Default|SetIsRotating false)
                            (if (Utilities|IsValid _shutterpartner_4)
                              (Variables|BP_Shutter_A_C|SetIsRotating _shutterpartner_4 false))
                            (Audio|PlaySoundatLocation (Variables|Default|GetBarLoweredSound) "0, 0, 0" "0, 0, 0" 1.0 1.0 0.0 0 0 0 0)))
                        (else
                          (goto _label_2)))))))
              (else
                (goto _label)))
            (else
              (goto _label)))
          (else
            ;[1 1 1] Check for a partner shutter and if there is one then check its open, if its still closed then this shutter wont open (because the security bar is still in the lowered position)
            (if (Utilities|IsValid _shutterpartner)
              (if (Rendering|IsVisible (Variables|BP_Shutter_A_C|GetBar _shutterpartner))
                (if (Variables|BP_Shutter_A_C|GetIsOpen _shutterpartner)
                  ;[1 1 1] Lift the security bar then open the shutter
                  (if (Rendering|IsVisible (Variables|Default|GetBar)) :!label _label_3
                    (Development|PrintString "Lifting bar" _debug_4 _debug_4)
                    (Audio|PlaySoundatLocation (Variables|Default|GetBarRaisingSound) "0, 0, 0" "0, 0, 0" 1.0 1.0 0.0 0 0 0 0)
                    (bind _rotation_3 (Timeline|LiftBarTimeline PlayFromStart)
                      (:Update
                        (if (Variables|Default|GetReverse%20Bar%20Rotation%20Direction?)
                          (switch Utilities|FlowControl|Switch|SwitchonAxisEnum (Variables|Default|GetBar%20Rotation%20Axis)
                            (:NewEnumerator0
                              (Transformation|SetRelativeRotation _bar (Math|Rotator|MakeRotator (+ (* _rotation_3 (Variables|Default|GetMax%20Bar%20Rotation%20%28degrees%29)) (.roll (Variables|Default|GetInitial%20Bar%20Rotation))) (.pitch (Variables|Default|GetInitial%20Bar%20Rotation)) (.yaw (Variables|Default|GetInitial%20Bar%20Rotation))) false false))
                            (:NewEnumerator1
                              (Transformation|SetRelativeRotation _bar (Math|Rotator|MakeRotator (.roll (Variables|Default|GetInitial%20Bar%20Rotation)) (+ (* _rotation_3 (Variables|Default|GetMax%20Bar%20Rotation%20%28degrees%29)) (.pitch (Variables|Default|GetInitial%20Bar%20Rotation))) (.yaw (Variables|Default|GetInitial%20Bar%20Rotation))) false false))
                            (:NewEnumerator2
                              (Transformation|SetRelativeRotation _bar (Math|Rotator|MakeRotator (.roll (Variables|Default|GetInitial%20Bar%20Rotation)) (.pitch (Variables|Default|GetInitial%20Bar%20Rotation)) (+ (* _rotation_3 (Variables|Default|GetMax%20Bar%20Rotation%20%28degrees%29)) (.yaw (Variables|Default|GetInitial%20Bar%20Rotation)))) false false)))
                          (else
                            (switch Utilities|FlowControl|Switch|SwitchonAxisEnum (Variables|Default|GetBar%20Rotation%20Axis)
                              (:NewEnumerator0
                                (Transformation|SetRelativeRotation _bar (Math|Rotator|MakeRotator (- (.roll (Variables|Default|GetInitial%20Bar%20Rotation)) (* _rotation_3 (Variables|Default|GetMax%20Bar%20Rotation%20%28degrees%29))) (.pitch (Variables|Default|GetInitial%20Bar%20Rotation)) (.yaw (Variables|Default|GetInitial%20Bar%20Rotation))) false false))
                              (:NewEnumerator1
                                (Transformation|SetRelativeRotation _bar (Math|Rotator|MakeRotator (.roll (Variables|Default|GetInitial%20Bar%20Rotation)) (- (.pitch (Variables|Default|GetInitial%20Bar%20Rotation)) (* _rotation_3 (Variables|Default|GetMax%20Bar%20Rotation%20%28degrees%29))) (.yaw (Variables|Default|GetInitial%20Bar%20Rotation))) false false))
                              (:NewEnumerator2
                                (Transformation|SetRelativeRotation _bar (Math|Rotator|MakeRotator (.roll (Variables|Default|GetInitial%20Bar%20Rotation)) (.pitch (Variables|Default|GetInitial%20Bar%20Rotation)) (- (.yaw (Variables|Default|GetInitial%20Bar%20Rotation)) (* _rotation_3 (Variables|Default|GetMax%20Bar%20Rotation%20%28degrees%29)))) false false)))))
                        (Development|PrintString (Utilities|String|Append "Bar rotation:" (Utilities|String|ToString(Rotator) (.Rotation (Math|Transform|BreakTransform (Transformation|GetRelativeTransform _bar))))) _debug _debug "(R=1.000000,G=0.000000,B=0.053420,A=1.000000)"))
                      (:Finished
                        (Audio|PlaySoundatLocation (Variables|Default|GetBarRaisedSound) "0, 0, 0" "0, 0, 0" 1.0 1.0 0.0 0 0 0 0)
                        (Development|PrintString "Opening shutter" _debug_9 _debug_9 :!label _label_4)
                        (bind _rotation_4 (Timeline|OpenShutterTimeline PlayFromStart)
                          (:Update
                            (if (Variables|Default|GetReverse%20Shutter%20Open%20Direction?)
                              (Transformation|SetRelativeRotation _shutter (Math|Rotator|MakeRotator (.roll (Variables|Default|GetInitial%20Shutter%20Rotation)) (.pitch (Variables|Default|GetInitial%20Shutter%20Rotation)) (+ (* _rotation_4 (Variables|Default|GetMax%20Shutter%20Rotation%20%28degrees%29)) (.yaw (Variables|Default|GetInitial%20Shutter%20Rotation)))) false false)
                              (else
                                (Transformation|SetRelativeRotation _shutter (Math|Rotator|MakeRotator (.roll (Variables|Default|GetInitial%20Shutter%20Rotation)) (.pitch (Variables|Default|GetInitial%20Shutter%20Rotation)) (- (.yaw (Variables|Default|GetInitial%20Shutter%20Rotation)) (* _rotation_4 (Variables|Default|GetMax%20Shutter%20Rotation%20%28degrees%29)))) false false))))
                          (:Finished
                            (Variables|Default|SetIsOpen true)
                            (Variables|Default|SetIsRotating false)
                            (if (Utilities|IsValid _shutterpartner_6)
                              (Variables|BP_Shutter_A_C|SetIsRotating _shutterpartner_6 false))))))
                    (else
                      (goto _label_4)))
                  (else
                    (Development|PrintString "You cannot open this shutter before the other shutter")
                    (Variables|Default|SetIsRotating false)
                    (if (Utilities|IsValid _shutterpartner_5)
                      (Variables|BP_Shutter_A_C|SetIsRotating _shutterpartner_5 false))))
                (else
                  (goto _label_3)))
              (else
                (goto _label_3)))))))))

(fn ConstructionScript
  (bind _shutter (Variables|Default|GetShutter))
  (bind _max_bar_rotation__degrees_ (Variables|Default|GetMax%20Bar%20Rotation%20%28degrees%29))
  (bind _max_shutter_rotation__degrees_ (Variables|Default|GetMax%20Shutter%20Rotation%20%28degrees%29))
  (bind _max_bar_rotation__degrees__2 (Variables|Default|GetMax%20Bar%20Rotation%20%28degrees%29))
  (if (Variables|Default|GetOpen%20By%20Default?)
    (Variables|Default|SetInitial%20Shutter%20Rotation (.rotation (Transformation|GetRelativeTransform (Variables|Default|GetShutter))))
    (Variables|Default|SetInitial%20Bar%20Rotation (.rotation (Transformation|GetRelativeTransform (Variables|Default|GetBar))))
    ;[1 1 1] Open the wooden bar
    (Variables|Default|SetIsOpen true)
    (if (Rendering|IsVisible (Variables|Default|GetBar))
      (if (Variables|Default|GetReverse%20Bar%20Rotation%20Direction?)
        (switch Utilities|FlowControl|Switch|SwitchonAxisEnum (Variables|Default|GetBar%20Rotation%20Axis)
          (:NewEnumerator0
            (Transformation|SetRelativeRotation (Variables|Default|GetBar) (Math|Rotator|MakeRotator (+ (Variables|Default|GetMax%20Bar%20Rotation%20%28degrees%29) (.roll (Variables|Default|GetInitial%20Bar%20Rotation))) (.pitch (Variables|Default|GetInitial%20Bar%20Rotation)) (.yaw (Variables|Default|GetInitial%20Bar%20Rotation))) false false))
          (:NewEnumerator1
            (Transformation|SetRelativeRotation (Variables|Default|GetBar) (Math|Rotator|MakeRotator _max_bar_rotation__degrees_ (+ _max_bar_rotation__degrees_ (.pitch (Variables|Default|GetInitial%20Bar%20Rotation))) (.yaw (Variables|Default|GetInitial%20Bar%20Rotation))) false false))
          (:NewEnumerator2
            (Transformation|SetRelativeRotation (Variables|Default|GetBar) (Math|Rotator|MakeRotator (.roll (Variables|Default|GetInitial%20Bar%20Rotation)) (.pitch (Variables|Default|GetInitial%20Bar%20Rotation)) (+ _max_bar_rotation__degrees__2 (.yaw (Variables|Default|GetInitial%20Bar%20Rotation)))) false false)))
        (else
          (switch Utilities|FlowControl|Switch|SwitchonAxisEnum (Variables|Default|GetBar%20Rotation%20Axis)
            (:NewEnumerator0
              (Transformation|SetRelativeRotation (Variables|Default|GetBar) (Math|Rotator|MakeRotator (- (.roll (Variables|Default|GetInitial%20Bar%20Rotation)) _max_bar_rotation__degrees_) (.pitch (Variables|Default|GetInitial%20Bar%20Rotation)) (.yaw (Variables|Default|GetInitial%20Bar%20Rotation))) false false))
            (:NewEnumerator1
              (Transformation|SetRelativeRotation (Variables|Default|GetBar) (Math|Rotator|MakeRotator (.roll (Variables|Default|GetInitial%20Bar%20Rotation)) (- (.pitch (Variables|Default|GetInitial%20Bar%20Rotation)) _max_bar_rotation__degrees__2) (.yaw (Variables|Default|GetInitial%20Bar%20Rotation))) false false))
            (:NewEnumerator2
              (Transformation|SetRelativeRotation (Variables|Default|GetBar) (Math|Rotator|MakeRotator (.roll (Variables|Default|GetInitial%20Bar%20Rotation)) (.pitch (Variables|Default|GetInitial%20Bar%20Rotation)) (- (.yaw (Variables|Default|GetInitial%20Bar%20Rotation)) (Variables|Default|GetMax%20Bar%20Rotation%20%28degrees%29))) false false))))))
    ;[1 1 1] Open the shutter door
    (if (Variables|Default|GetReverse%20Shutter%20Open%20Direction?)
      (Transformation|SetRelativeRotation _shutter (Math|Rotator|MakeRotator (.roll (Variables|Default|GetInitial%20Shutter%20Rotation)) (.pitch (Variables|Default|GetInitial%20Shutter%20Rotation)) (+ _max_shutter_rotation__degrees_ (.yaw (Variables|Default|GetInitial%20Shutter%20Rotation)))) false false)
      (else
        (Transformation|SetRelativeRotation _shutter (Math|Rotator|MakeRotator (.roll (Variables|Default|GetInitial%20Shutter%20Rotation)) (.pitch (Variables|Default|GetInitial%20Shutter%20Rotation)) (- (.yaw (Variables|Default|GetInitial%20Shutter%20Rotation)) _max_shutter_rotation__degrees_)) false false)))))

(fn GetID
  (return ""))

(fn GetLauncherActor
  (return 0))

(fn GetObjectName
  (if (Variables|Default|GetIsOpen)
    (return "Close Shutter")
    (else
      (return "Open Shutter"))))

(fn IsProjectile
  (return false))