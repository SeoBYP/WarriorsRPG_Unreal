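; Lantern prop Blueprint with three candle flame components and a light that can be switched on and off.
; The construction script applies the exposed color, intensity, attenuation radius, source radius and initial visibility to the components.
; The Lookingat event, noted as the E key interaction, toggles visibility of the light and all three flames together.
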(event EventLookingat
  (params (HitComponent :type Actor%20Component%20Object%20Reference))
  ;[1 1 1] E key will toggle light
  (Rendering|ToggleVisibility (Variables|Default|GetP_CandleFlame1) false))

(fn ConstructionScript
  (Rendering|Components|Light|SetLightColor (Variables|Default|GetLight) (Variables|Default|GetLight%20Color) true)
  (Rendering|SetVisibility (Variables|Default|GetLight) (Variables|Default|GetIs%20Visible) false)
  (Rendering|Lighting|SetAttenuationRadius (Variables|Default|GetLight) (Variables|Default|GetAttenuation%20Radius))
  (Rendering|Components|Light|SetIntensity (Variables|Default|GetLight) (Variables|Default|GetIntensity))
  (Class|PointLightComponent|SetSourceRadius (Variables|Default|GetLight) (Variables|Default|GetSource%20Radius)))