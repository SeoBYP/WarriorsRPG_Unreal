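; Interactable chest Blueprint whose lid swings open on a Lookingat event, stays open for OpenedDurationSecs, then closes itself.
; OpenTimeline and a reversed CloseTimeline drive Lid roll from its starting angle, scaled by MaxAngleOfLid at OpenCloseRate.
; IsInUse blocks retriggering until the cycle finishes, while IsRotating and IsFullyOpen track lid state.
; Open and close cues play at the start and end, located at world origin rather than the chest.
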(event EventLookingat
  (params (HitComponent :type Actor%20Component%20Object%20Reference))
  (bind _lid (Variables|Default|GetLid))
  (bind _relativerotation (Variables|/Script/Engine.SceneComponent|GetRelativeRotation _lid))
  ;[1 1 1] Open the chest then close it after waiting 2 seconds
  (if (not (Variables|Default|GetIsInUse))
    (Variables|Default|SetIsInUse true)
    (Variables|Default|SetLidAngle (.roll _relativerotation))
    (Variables|Default|SetIsRotating true)
    (Components|Timeline|SetPlayRate (Variables|Default|GetOpenTimeline) (Variables|Default|GetOpenCloseRate))
    (Audio|PlaySoundatLocation "/Game/MRPGT/MedievalBuildings01/Audio/SoundCues/ChestOpen_Cue.ChestOpen_Cue" "0, 0, 0" "0, 0, 0" 1.0 1.0 0.0 0 0 0 0)
    (bind _lidangle (Timeline|OpenTimeline PlayFromStart)
      (:Update
        (Transformation|SetRelativeRotation (Variables|Default|GetLid) (Math|Rotator|MakeRotator (- (Variables|Default|GetLidAngle) (* _lidangle (Variables|Default|GetMax%20Angle%20of%20Lid))) 0.0 0.0) false false)
        (Development|PrintString (Utilities|String|Append "Opening." "Lid angle: " (Utilities|String|ToString(Float) (.roll _relativerotation))) false false))
      (:Finished
        (Development|PrintString "Fully opened" false false)
        (Variables|Default|SetIsRotating false)
        (Variables|Default|SetIsFullyOpen true)
        (Utilities|FlowControl|Delay (Variables|Default|GetOpened%20Duration%20%28secs%29))
        (Variables|Default|SetIsRotating true)
        (Variables|Default|SetIsFullyOpen false)
        (Components|Timeline|SetPlayRate (Variables|Default|GetCloseTimeline) (Variables|Default|GetOpenCloseRate))
        (bind _lidangle_2 (Timeline|CloseTimeline ReverseFromEnd)
          (:Update
            (Transformation|SetRelativeRotation (Variables|Default|GetLid) (Math|Rotator|MakeRotator (- (Variables|Default|GetLidAngle) (* _lidangle_2 (Variables|Default|GetMax%20Angle%20of%20Lid))) 0.0 0.0) false false)
            (Development|PrintString (Utilities|String|Append "Closing. " "Lid angle: " (Utilities|String|ToString(Float) (.roll _relativerotation))) false false))
          (:Finished
            (Development|PrintString "Fully closed" false false)
            (Variables|Default|SetIsInUse false)
            (Audio|PlaySoundatLocation "/Game/MRPGT/MedievalBuildings01/Audio/SoundCues/ChestClose_Cue.ChestClose_Cue" "0, 0, 0" "0, 0, 0" 1.0 1.0 0.0 0 0 0 0)))))))

(fn ConstructionScript)