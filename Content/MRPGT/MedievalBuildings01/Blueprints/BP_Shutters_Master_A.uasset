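; Interactable medieval-building shutter pair with an optional security bar, toggled open or closed by player interaction or opened at BeginPlay.
; Timelines scale configurable rotations: opening lifts any visible bar before swinging both shutters, while closing swings them shut before lowering it.
; An in-use flag blocks re-triggering, with sounds and debug prints along the sequence.
; Interface functions supply the open/close label, and interaction state is messaged to the player character.
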(event EventInteract
  (params (HitComponent :type Actor%20Component%20Object%20Reference) (InteractingActor :type Actor%20Object%20Reference))
  (bind _debug (Variables|Default|GetDebug))
  (bind _debug_2 (Variables|Default|GetDebug))
  (bind _rightshutter (Variables|Default|GetRightShutter))
  (bind _debug_3 (Variables|Default|GetDebug))
  (bind _leftshutter (Variables|Default|GetLeftShutter))
  (bind _debug_4 (Variables|Default|GetDebug))
  (bind _debug_5 (Variables|Default|GetDebug))
  (bind _debug_6 (Variables|Default|GetDebug))
  (bind _debug_7 (Variables|Default|GetDebug))
  (bind _debug_8 (Variables|Default|GetDebug))
  (bind _leftshutter_2 (Variables|Default|GetLeftShutter))
  (bind _debug_9 (Variables|Default|GetDebug))
  (bind _debug_10 (Variables|Default|GetDebug))
  (bind _debug_11 (Variables|Default|GetDebug))
  (bind _debug_12 (Variables|Default|GetDebug))
  (bind _debug_13 (Variables|Default|GetDebug))
  (bind _debug_14 (Variables|Default|GetDebug))
  (bind _bar (Variables|Default|GetBar))
  (bind _bar_2 (Variables|Default|GetBar))
  (bind _rightshutter_2 (Variables|Default|GetRightShutter))
  (bind _debug_15 (Variables|Default|GetDebug))
  ;[1 1 1] Initialise vars
  (Class|InterfaceGeneralCharacter|SetIsInteractingwithObject(Message) (Game|GetPlayerCharacter 0) true)
  (Development|PrintString (Utilities|String|Append "Hit component:" (Utilities|GetObjectName HitComponent)) _debug_14 _debug_14 "(R=0.000000,G=0.660000,B=1.000000,A=1.000000)" 5.0)
  (if (Variables|Default|GetShutters%20Can%20Be%20Opened?)
    (if (Variables|Default|GetIs%20In%20Use?)
      (Development|PrintString "Shutters already being used. Please wait." _debug_7 _debug_7)
      (else
        (Utilities|FlowControl|Sequence
          (:then_0
            (Variables|Default|SetIs%20In%20Use? true)
            (Variables|Default|SetInitial%20Left%20Shutter%20Rotation (.rotation (Transformation|GetRelativeTransform (Variables|Default|GetLeftShutter))))
            (Variables|Default|SetInitial%20Right%20Shutter%20Rotation (.rotation (Transformation|GetRelativeTransform (Variables|Default|GetRightShutter))))
            (Variables|Default|SetInitial%20Bar%20Rotation (.rotation (Transformation|GetRelativeTransform (Variables|Default|GetBar))))
            (Components|Timeline|SetPlayRate (Variables|Default|GetOpenShutterTimeline) (Variables|Default|GetOpen%20And%20Close%20Rate))
            ;[1 1 1] Print some debug info
            (Development|PrintString (Utilities|String|Append "Initial left shutter rotation" (Utilities|String|ToString(Rotator) (Variables|Default|GetInitial%20Left%20Shutter%20Rotation))) _debug_9 _debug_9 "(R=0.000000,G=0.660000,B=1.000000,A=1.000000)" 4.0)
            (Development|PrintString (Utilities|String|Append "Initial right shutter rotation" (Utilities|String|ToString(Rotator) (Variables|Default|GetInitial%20Right%20Shutter%20Rotation))) _debug_10 _debug_10)
            (Development|PrintString (Utilities|String|Append "Initial bar rotation" (Utilities|String|ToString(Rotator) (Variables|Default|GetInitial%20Bar%20Rotation))) _debug_9 _debug_9 "(R=0.000000,G=0.660000,B=1.000000,A=1.000000)" 4.0)
            ;[1 1 1] If shutter is open then close it otherwise open it
            (if (Variables|Default|GetShutters%20Are%20Open)
              ;[1 1 1] Close the shutters then lower the security bar
              (Development|PrintString "Closing shutters" _debug_2 _debug_2)
              (Utilities|FlowControl|Sequence
                (:then_0
                  (Audio|PlaySoundatLocation (Variables|Default|GetShutterClosingSound) "0, 0, 0" "0, 0, 0" 1.0 1.0 0.0 0 0 0 0)
                  (bind _rotation (Timeline|CloseShutterTimeline PlayFromStart)
                    (:Update
                      (if (Variables|Default|GetReverse%20Shutter%20Open%20Direction?)
                        (Transformation|SetRelativeRotation _leftshutter_2 (Math|Rotator|MakeRotator (.roll (Variables|Default|GetInitial%20Left%20Shutter%20Rotation)) (.pitch (Variables|Default|GetInitial%20Left%20Shutter%20Rotation)) (+ (.yaw (Variables|Default|GetInitial%20Left%20Shutter%20Rotation)) (* _rotation (Variables|Default|GetMax%20Shutter%20Rotation%20%28degrees%29)))) false false)
                        (else
                          (Transformation|SetRelativeRotation _leftshutter_2 (Math|Rotator|MakeRotator (.roll (Variables|Default|GetInitial%20Left%20Shutter%20Rotation)) (.pitch (Variables|Default|GetInitial%20Left%20Shutter%20Rotation)) (- (.yaw (Variables|Default|GetInitial%20Left%20Shutter%20Rotation)) (* _rotation (Variables|Default|GetMax%20Shutter%20Rotation%20%28degrees%29)))) false false)))
                      (Development|PrintString (Utilities|String|Append "Left shutter rotation:" (Utilities|String|ToString(Rotator) (Variables|/Script/Engine.SceneComponent|GetRelativeRotation (Variables|Default|GetLeftShutter)))) _debug_11 _debug_11 "(R=0.000000,G=0.660000,B=1.000000,A=1.000000)" 4.0 :!label _label)
                      (Development|PrintString (Utilities|String|Append "Right shutter rotation:" (Utilities|String|ToString(Rotator) (Variables|/Script/Engine.SceneComponent|GetRelativeRotation (Variables|Default|GetRightShutter)))) _debug_12 _debug_12))
                    (:Finished
                      (Audio|PlaySoundatLocation (Variables|Default|GetShutterClosedSound) "0, 0, 0" "0, 0, 0" 1.0 1.0 0.0 0 0 0 0))))
                (:then_1
                  (Audio|PlaySoundatLocation (Variables|Default|GetShutterClosingSound) "0, 0, 0" "0, 0, 0" 1.0 1.0 0.0 0 0 0 0)
                  (bind _rotation_2 (Timeline|Timeline_1 PlayFromStart)
                    (:Update
                      (if (not (Variables|Default|GetReverse%20Shutter%20Open%20Direction?))
                        (Transformation|SetRelativeRotation _rightshutter_2 (Math|Rotator|MakeRotator (.roll (Variables|Default|GetInitial%20Right%20Shutter%20Rotation)) (.pitch (Variables|Default|GetInitial%20Right%20Shutter%20Rotation)) (+ (.yaw (Variables|Default|GetInitial%20Right%20Shutter%20Rotation)) (* _rotation_2 (Variables|Default|GetMax%20Shutter%20Rotation%20%28degrees%29)))) false false)
                        (goto _label)
                        (else
                          (Transformation|SetRelativeRotation _rightshutter_2 (Math|Rotator|MakeRotator (.roll (Variables|Default|GetInitial%20Right%20Shutter%20Rotation)) (.pitch (Variables|Default|GetInitial%20Right%20Shutter%20Rotation)) (- (.yaw (Variables|Default|GetInitial%20Right%20Shutter%20Rotation)) (* _rotation_2 (Variables|Default|GetMax%20Shutter%20Rotation%20%28degrees%29)))) false false)
                          (goto _label))))
                    (:Finished
                      (Audio|PlaySoundatLocation (Variables|Default|GetShutterClosedSound) "0, 0, 0" "0, 0, 0" 1.0 1.0 0.0 0 0 0 0)
                      (if (Rendering|IsVisible (Variables|Default|GetBar))
                        (Development|PrintString "Lowering bar" _debug_4 _debug_4)
                        (Variables|Default|SetInitial%20Bar%20Rotation (Variables|/Script/Engine.SceneComponent|GetRelativeRotation (Variables|Default|GetBar)))
                        (Audio|PlaySoundatLocation (Variables|Default|GetBarLoweringSound) "0, 0, 0" "0, 0, 0" 1.0 1.0 0.0 0 0 0 0)
                        (bind _rotation_3 (Timeline|LowerBarTimeline PlayFromStart)
                          (:Update
                            (if (Variables|Default|GetReverse%20Bar%20Rotation%20Direction?)
                              (switch Utilities|FlowControl|Switch|SwitchonAxisEnum (Variables|Default|GetBar%20Rotation%20Axis)
                                (:NewEnumerator0
                                  (Transformation|SetRelativeRotation _bar_2 (Math|Rotator|MakeRotator (- (.roll (Variables|Default|GetInitial%20Bar%20Rotation)) (* _rotation_3 (Variables|Default|GetMax%20Bar%20Rotation%20%28degrees%29))) (.pitch (Variables|Default|GetInitial%20Bar%20Rotation)) (.yaw (Variables|Default|GetInitial%20Bar%20Rotation))) false false))
                                (:NewEnumerator1
                                  (Transformation|SetRelativeRotation _bar_2 (Math|Rotator|MakeRotator (.roll (Variables|Default|GetInitial%20Bar%20Rotation)) (- (.pitch (Variables|Default|GetInitial%20Bar%20Rotation)) (* _rotation_3 (Variables|Default|GetMax%20Bar%20Rotation%20%28degrees%29))) (.yaw (Variables|Default|GetInitial%20Bar%20Rotation))) false false))
                                (:NewEnumerator2
                                  (Transformation|SetRelativeRotation _bar_2 (Math|Rotator|MakeRotator (.roll (Variables|Default|GetInitial%20Bar%20Rotation)) (.pitch (Variables|Default|GetInitial%20Bar%20Rotation)) (- (.yaw (Variables|Default|GetInitial%20Bar%20Rotation)) (* _rotation_3 (Variables|Default|GetMax%20Bar%20Rotation%20%28degrees%29)))) false false)))
                              (else
                                (switch Utilities|FlowControl|Switch|SwitchonAxisEnum (Variables|Default|GetBar%20Rotation%20Axis)
                                  (:NewEnumerator0
                                    (Transformation|SetRelativeRotation _bar_2 (Math|Rotator|MakeRotator (+ (* _rotation_3 (Variables|Default|GetMax%20Bar%20Rotation%20%28degrees%29)) (.roll (Variables|Default|GetInitial%20Bar%20Rotation))) (.pitch (Variables|Default|GetInitial%20Bar%20Rotation)) (.yaw (Variables|Default|GetInitial%20Bar%20Rotation))) false false))
                                  (:NewEnumerator1
                                    (Transformation|SetRelativeRotation _bar_2 (Math|Rotator|MakeRotator (.roll (Variables|Default|GetInitial%20Bar%20Rotation)) (+ (* _rotation_3 (Variables|Default|GetMax%20Bar%20Rotation%20%28degrees%29)) (.pitch (Variables|Default|GetInitial%20Bar%20Rotation))) (.yaw (Variables|Default|GetInitial%20Bar%20Rotation))) false false))
                                  (:NewEnumerator2
                                    (Transformation|SetRelativeRotation _bar_2 (Math|Rotator|MakeRotator (.roll (Variables|Default|GetInitial%20Bar%20Rotation)) (.pitch (Variables|Default|GetInitial%20Bar%20Rotation)) (+ (* _rotation_3 (Variables|Default|GetMax%20Bar%20Rotation%20%28degrees%29)) (.yaw (Variables|Default|GetInitial%20Bar%20Rotation)))) false false)))))
                            (Development|PrintString (Utilities|String|Append "Bar rotation:" (Utilities|String|ToString(Rotator) (.Rotation (Math|Transform|BreakTransform (Transformation|GetRelativeTransform _bar_2))))) _debug_8 _debug_8 "(R=1.000000,G=0.000000,B=0.036710,A=1.000000)"))
                          (:Finished
                            (Variables|Default|SetShutters%20Are%20Open false :!label _label_2)
                            (Variables|Default|SetIs%20In%20Use? false)
                            (Audio|PlaySoundatLocation (Variables|Default|GetBarLoweredSound) "0, 0, 0" "0, 0, 0" 1.0 1.0 0.0 0 0 0 0)))
                        (else
                          (goto _label_2)))))))
              (else
                ;[1 1 1] Lift the security bar then open the shutters
                (if (Rendering|IsVisible (Variables|Default|GetBar))
                  (Development|PrintString "Lifting bar" _debug_5 _debug_5)
                  (if (Variables|Default|GetBegin%20Open?)
                    (bind _rotation_4 (Timeline|LiftBarTimeline PlayFromStart)
                      (:Update
                        (if (Variables|Default|GetReverse%20Bar%20Rotation%20Direction?)
                          (switch Utilities|FlowControl|Switch|SwitchonAxisEnum (Variables|Default|GetBar%20Rotation%20Axis)
                            (:NewEnumerator0
                              (Transformation|SetRelativeRotation _bar (Math|Rotator|MakeRotator (+ (* _rotation_4 (Variables|Default|GetMax%20Bar%20Rotation%20%28degrees%29)) (.roll (Variables|Default|GetInitial%20Bar%20Rotation))) (.pitch (Variables|Default|GetInitial%20Bar%20Rotation)) (.yaw (Variables|Default|GetInitial%20Bar%20Rotation))) false false))
                            (:NewEnumerator1
                              (Transformation|SetRelativeRotation _bar (Math|Rotator|MakeRotator (.roll (Variables|Default|GetInitial%20Bar%20Rotation)) (+ (* _rotation_4 (Variables|Default|GetMax%20Bar%20Rotation%20%28degrees%29)) (.pitch (Variables|Default|GetInitial%20Bar%20Rotation))) (.yaw (Variables|Default|GetInitial%20Bar%20Rotation))) false false))
                            (:NewEnumerator2
                              (Transformation|SetRelativeRotation _bar (Math|Rotator|MakeRotator (.roll (Variables|Default|GetInitial%20Bar%20Rotation)) (.pitch (Variables|Default|GetInitial%20Bar%20Rotation)) (+ (* _rotation_4 (Variables|Default|GetMax%20Bar%20Rotation%20%28degrees%29)) (.yaw (Variables|Default|GetInitial%20Bar%20Rotation)))) false false)))
                          (else
                            (switch Utilities|FlowControl|Switch|SwitchonAxisEnum (Variables|Default|GetBar%20Rotation%20Axis)
                              (:NewEnumerator0
                                (Transformation|SetRelativeRotation _bar (Math|Rotator|MakeRotator (- (.roll (Variables|Default|GetInitial%20Bar%20Rotation)) (* _rotation_4 (Variables|Default|GetMax%20Bar%20Rotation%20%28degrees%29))) (.pitch (Variables|Default|GetInitial%20Bar%20Rotation)) (.yaw (Variables|Default|GetInitial%20Bar%20Rotation))) false false))
                              (:NewEnumerator1
                                (Transformation|SetRelativeRotation _bar (Math|Rotator|MakeRotator (.roll (Variables|Default|GetInitial%20Bar%20Rotation)) (- (.pitch (Variables|Default|GetInitial%20Bar%20Rotation)) (* _rotation_4 (Variables|Default|GetMax%20Bar%20Rotation%20%28degrees%29))) (.yaw (Variables|Default|GetInitial%20Bar%20Rotation))) false false))
                              (:NewEnumerator2
                                (Transformation|SetRelativeRotation _bar (Math|Rotator|MakeRotator (.roll (Variables|Default|GetInitial%20Bar%20Rotation)) (.pitch (Variables|Default|GetInitial%20Bar%20Rotation)) (- (.yaw (Variables|Default|GetInitial%20Bar%20Rotation)) (* _rotation_4 (Variables|Default|GetMax%20Bar%20Rotation%20%28degrees%29)))) false false)))))
                        (Development|PrintString (Utilities|String|Append "Bar rotation:" (Utilities|String|ToString(Rotator) (.Rotation (Math|Transform|BreakTransform (Transformation|GetRelativeTransform _bar))))) _debug _debug "(R=1.000000,G=0.000000,B=0.053420,A=1.000000)"))
                      (:Finished
                        (if (Variables|Default|GetBegin%20Open?)
                          _
                          (else
                            (Audio|PlaySoundatLocation (Variables|Default|GetBarRaisedSound) "0, 0, 0" "0, 0, 0" 1.0 1.0 0.0 0 0 0 0)))
                        (Utilities|FlowControl|Sequence :!label _label_3
                          (:then_0
                            (Development|PrintString "Opening right shutter" _debug_3 _debug_3)
                            (bind _rotation_5 (Timeline|OpenShutterTimeline PlayFromStart)
                              (:Update
                                (if (Variables|Default|GetReverse%20Shutter%20Open%20Direction?)
                                  (Transformation|SetRelativeRotation _rightshutter (Math|Rotator|MakeRotator (.roll (Variables|Default|GetInitial%20Left%20Shutter%20Rotation)) (.pitch (Variables|Default|GetInitial%20Left%20Shutter%20Rotation)) (+ (* _rotation_5 (Variables|Default|GetMax%20Shutter%20Rotation%20%28degrees%29)) (.yaw (Variables|Default|GetInitial%20Left%20Shutter%20Rotation)))) false false)
                                  (else
                                    (Transformation|SetRelativeRotation _rightshutter (Math|Rotator|MakeRotator (.roll (Variables|Default|GetInitial%20Left%20Shutter%20Rotation)) (.pitch (Variables|Default|GetInitial%20Left%20Shutter%20Rotation)) (- (.yaw (Variables|Default|GetInitial%20Left%20Shutter%20Rotation)) (* _rotation_5 (Variables|Default|GetMax%20Shutter%20Rotation%20%28degrees%29)))) false false)))
                                (Development|PrintString (Utilities|String|Append "Left shutter rotation:" (Utilities|String|ToString(Rotator) (Variables|/Script/Engine.SceneComponent|GetRelativeRotation (Variables|Default|GetLeftShutter)))) _debug_13 _debug_13 "(R=0.000000,G=0.660000,B=1.000000,A=1.000000)" 4.0 :!label _label_4)
                                (Development|PrintString (Utilities|String|Append "Right shutter rotation:" (Utilities|String|ToString(Rotator) (Variables|/Script/Engine.SceneComponent|GetRelativeRotation (Variables|Default|GetRightShutter)))) _debug_6 _debug_6)
                                (Variables|Default|SetBegin%20Open? false))))
                          (:then_1
                            (Development|PrintString "Opening left shutter" _debug_15 _debug_15)
                            (bind _rotation_6 (Timeline|Timeline_0 PlayFromStart)
                              (:Update
                                (if (not (Variables|Default|GetReverse%20Shutter%20Open%20Direction?))
                                  (Transformation|SetRelativeRotation _leftshutter (Math|Rotator|MakeRotator (.roll (Variables|Default|GetInitial%20Right%20Shutter%20Rotation)) (.pitch (Variables|Default|GetInitial%20Right%20Shutter%20Rotation)) (+ (* _rotation_6 (Variables|Default|GetMax%20Shutter%20Rotation%20%28degrees%29)) (.yaw (Variables|Default|GetInitial%20Right%20Shutter%20Rotation)))) false false)
                                  (goto _label_4)
                                  (else
                                    (Transformation|SetRelativeRotation _leftshutter (Math|Rotator|MakeRotator (.roll (Variables|Default|GetInitial%20Right%20Shutter%20Rotation)) (.pitch (Variables|Default|GetInitial%20Right%20Shutter%20Rotation)) (- (.yaw (Variables|Default|GetInitial%20Right%20Shutter%20Rotation)) (* _rotation_6 (Variables|Default|GetMax%20Shutter%20Rotation%20%28degrees%29)))) false false)
                                    (goto _label_4))))
                              (:Finished
                                (Variables|Default|SetShutters%20Are%20Open true)
                                (Variables|Default|SetIs%20In%20Use? false)))))))
                    (else
                      (Audio|PlaySoundatLocation (Variables|Default|GetBarRaisingSound) "0, 0, 0" "0, 0, 0" 1.0 1.0 0.0 0 0 0 0)
                      (Timeline|LiftBarTimeline PlayFromStart)))
                  (else
                    (goto _label_3))))))
          (:then_1
            (Class|InterfaceGeneralCharacter|SetIsInteractingwithObject(Message) (Game|GetPlayerCharacter 0) false)))))
    (else
      (Class|InterfaceGeneralCharacter|SetIsInteractingwithObject(Message) (Game|GetPlayerCharacter 0) false))))

(event EventLookingat
  (params (HitComponent :type Actor%20Component%20Object%20Reference))
  (bind _debug (Variables|Default|GetDebug))
  (bind _debug_2 (Variables|Default|GetDebug))
  (bind _rightshutter (Variables|Default|GetRightShutter))
  (bind _debug_3 (Variables|Default|GetDebug))
  (bind _leftshutter (Variables|Default|GetLeftShutter))
  (bind _debug_4 (Variables|Default|GetDebug))
  (bind _debug_5 (Variables|Default|GetDebug))
  (bind _debug_6 (Variables|Default|GetDebug))
  (bind _debug_7 (Variables|Default|GetDebug))
  (bind _debug_8 (Variables|Default|GetDebug))
  (bind _leftshutter_2 (Variables|Default|GetLeftShutter))
  (bind _debug_9 (Variables|Default|GetDebug))
  (bind _debug_10 (Variables|Default|GetDebug))
  (bind _debug_11 (Variables|Default|GetDebug))
  (bind _debug_12 (Variables|Default|GetDebug))
  (bind _debug_13 (Variables|Default|GetDebug))
  (bind _debug_14 (Variables|Default|GetDebug))
  (bind _bar (Variables|Default|GetBar))
  (bind _bar_2 (Variables|Default|GetBar))
  (bind _rightshutter_2 (Variables|Default|GetRightShutter))
  (bind _debug_15 (Variables|Default|GetDebug))
  ;[1 1 1] Initialise vars
  (Development|PrintString (Utilities|String|Append "Hit component:" (Utilities|GetObjectName (stale EventInteract HitComponent))) _debug_14 _debug_14 "(R=0.000000,G=0.660000,B=1.000000,A=1.000000)" 5.0)
  (if (Variables|Default|GetShutters%20Can%20Be%20Opened?)
    (if (Variables|Default|GetIs%20In%20Use?)
      (Development|PrintString "Shutters already being used. Please wait." _debug_7 _debug_7)
      (else
        (Utilities|FlowControl|Sequence
          (:then_0
            (Variables|Default|SetIs%20In%20Use? true)
            (Variables|Default|SetInitial%20Left%20Shutter%20Rotation (.rotation (Transformation|GetRelativeTransform (Variables|Default|GetLeftShutter))))
            (Variables|Default|SetInitial%20Right%20Shutter%20Rotation (.rotation (Transformation|GetRelativeTransform (Variables|Default|GetRightShutter))))
            (Variables|Default|SetInitial%20Bar%20Rotation (.rotation (Transformation|GetRelativeTransform (Variables|Default|GetBar))))
            (Components|Timeline|SetPlayRate (Variables|Default|GetOpenShutterTimeline) (Variables|Default|GetOpen%20And%20Close%20Rate))
            ;[1 1 1] Print some debug info
            (Development|PrintString (Utilities|String|Append "Initial left shutter rotation" (Utilities|String|ToString(Rotator) (Variables|Default|GetInitial%20Left%20Shutter%20Rotation))) _debug_9 _debug_9 "(R=0.000000,G=0.660000,B=1.000000,A=1.000000)" 4.0)
            (Development|PrintString (Utilities|String|Append "Initial right shutter rotation" (Utilities|String|ToString(Rotator) (Variables|Default|GetInitial%20Right%20Shutter%20Rotation))) _debug_10 _debug_10)
            (Development|PrintString (Utilities|String|Append "Initial bar rotation" (Utilities|String|ToString(Rotator) (Variables|Default|GetInitial%20Bar%20Rotation))) _debug_9 _debug_9 "(R=0.000000,G=0.660000,B=1.000000,A=1.000000)" 4.0)
            ;[1 1 1] If shutter is open then close it otherwise open it
            (if (Variables|Default|GetShutters%20Are%20Open)
              ;[1 1 1] Close the shutters then lower the security bar
              (Development|PrintString "Closing shutters" _debug_2 _debug_2)
              (Utilities|FlowControl|Sequence
                (:then_0
                  (Audio|PlaySoundatLocation (Variables|Default|GetShutterClosingSound) "0, 0, 0" "0, 0, 0" 1.0 1.0 0.0 0 0 0 0)
                  (bind _rotation (Timeline|CloseShutterTimeline PlayFromStart)
                    (:Update
                      (if (Variables|Default|GetReverse%20Shutter%20Open%20Direction?)
                        (Transformation|SetRelativeRotation _leftshutter_2 (Math|Rotator|MakeRotator (.roll (Variables|Default|GetInitial%20Left%20Shutter%20Rotation)) (.pitch (Variables|Default|GetInitial%20Left%20Shutter%20Rotation)) (+ (.yaw (Variables|Default|GetInitial%20Left%20Shutter%20Rotation)) (* _rotation (Variables|Default|GetMax%20Shutter%20Rotation%20%28degrees%29)))) false false)
                        (else
                          (Transformation|SetRelativeRotation _leftshutter_2 (Math|Rotator|MakeRotator (.roll (Variables|Default|GetInitial%20Left%20Shutter%20Rotation)) (.pitch (Variables|Default|GetInitial%20Left%20Shutter%20Rotation)) (- (.yaw (Variables|Default|GetInitial%20Left%20Shutter%20Rotation)) (* _rotation (Variables|Default|GetMax%20Shutter%20Rotation%20%28degrees%29)))) false false)))
                      (Development|PrintString (Utilities|String|Append "Left shutter rotation:" (Utilities|String|ToString(Rotator) (Variables|/Script/Engine.SceneComponent|GetRelativeRotation (Variables|Default|GetLeftShutter)))) _debug_11 _debug_11 "(R=0.000000,G=0.660000,B=1.000000,A=1.000000)" 4.0 :!label _label)
                      (Development|PrintString (Utilities|String|Append "Right shutter rotation:" (Utilities|String|ToString(Rotator) (Variables|/Script/Engine.SceneComponent|GetRelativeRotation (Variables|Default|GetRightShutter)))) _debug_12 _debug_12))
                    (:Finished
                      (Audio|PlaySoundatLocation (Variables|Default|GetShutterClosedSound) "0, 0, 0" "0, 0, 0" 1.0 1.0 0.0 0 0 0 0))))
                (:then_1
                  (Audio|PlaySoundatLocation (Variables|Default|GetShutterClosingSound) "0, 0, 0" "0, 0, 0" 1.0 1.0 0.0 0 0 0 0)
                  (bind _rotation_2 (Timeline|Timeline_1 PlayFromStart)
                    (:Update
                      (if (not (Variables|Default|GetReverse%20Shutter%20Open%20Direction?))
                        (Transformation|SetRelativeRotation _rightshutter_2 (Math|Rotator|MakeRotator (.roll (Variables|Default|GetInitial%20Right%20Shutter%20Rotation)) (.pitch (Variables|Default|GetInitial%20Right%20Shutter%20Rotation)) (+ (.yaw (Variables|Default|GetInitial%20Right%20Shutter%20Rotation)) (* _rotation_2 (Variables|Default|GetMax%20Shutter%20Rotation%20%28degrees%29)))) false false)
                        (goto _label)
                        (else
                          (Transformation|SetRelativeRotation _rightshutter_2 (Math|Rotator|MakeRotator (.roll (Variables|Default|GetInitial%20Right%20Shutter%20Rotation)) (.pitch (Variables|Default|GetInitial%20Right%20Shutter%20Rotation)) (- (.yaw (Variables|Default|GetInitial%20Right%20Shutter%20Rotation)) (* _rotation_2 (Variables|Default|GetMax%20Shutter%20Rotation%20%28degrees%29)))) false false)
                          (goto _label))))
                    (:Finished
                      (Audio|PlaySoundatLocation (Variables|Default|GetShutterClosedSound) "0, 0, 0" "0, 0, 0" 1.0 1.0 0.0 0 0 0 0)
                      (if (Rendering|IsVisible (Variables|Default|GetBar))
                        (Development|PrintString "Lowering bar" _debug_4 _debug_4)
                        (Variables|Default|SetInitial%20Bar%20Rotation (Variables|/Script/Engine.SceneComponent|GetRelativeRotation (Variables|Default|GetBar)))
                        (Audio|PlaySoundatLocation (Variables|Default|GetBarLoweringSound) "0, 0, 0" "0, 0, 0" 1.0 1.0 0.0 0 0 0 0)
                        (bind _rotation_3 (Timeline|LowerBarTimeline PlayFromStart)
                          (:Update
                            (if (Variables|Default|GetReverse%20Bar%20Rotation%20Direction?)
                              (switch Utilities|FlowControl|Switch|SwitchonAxisEnum (Variables|Default|GetBar%20Rotation%20Axis)
                                (:NewEnumerator0
                                  (Transformation|SetRelativeRotation _bar_2 (Math|Rotator|MakeRotator (- (.roll (Variables|Default|GetInitial%20Bar%20Rotation)) (* _rotation_3 (Variables|Default|GetMax%20Bar%20Rotation%20%28degrees%29))) (.pitch (Variables|Default|GetInitial%20Bar%20Rotation)) (.yaw (Variables|Default|GetInitial%20Bar%20Rotation))) false false))
                                (:NewEnumerator1
                                  (Transformation|SetRelativeRotation _bar_2 (Math|Rotator|MakeRotator (.roll (Variables|Default|GetInitial%20Bar%20Rotation)) (- (.pitch (Variables|Default|GetInitial%20Bar%20Rotation)) (* _rotation_3 (Variables|Default|GetMax%20Bar%20Rotation%20%28degrees%29))) (.yaw (Variables|Default|GetInitial%20Bar%20Rotation))) false false))
                                (:NewEnumerator2
                                  (Transformation|SetRelativeRotation _bar_2 (Math|Rotator|MakeRotator (.roll (Variables|Default|GetInitial%20Bar%20Rotation)) (.pitch (Variables|Default|GetInitial%20Bar%20Rotation)) (- (.yaw (Variables|Default|GetInitial%20Bar%20Rotation)) (* _rotation_3 (Variables|Default|GetMax%20Bar%20Rotation%20%28degrees%29)))) false false)))
                              (else
                                (switch Utilities|FlowControl|Switch|SwitchonAxisEnum (Variables|Default|GetBar%20Rotation%20Axis)
                                  (:NewEnumerator0
                                    (Transformation|SetRelativeRotation _bar_2 (Math|Rotator|MakeRotator (+ (* _rotation_3 (Variables|Default|GetMax%20Bar%20Rotation%20%28degrees%29)) (.roll (Variables|Default|GetInitial%20Bar%20Rotation))) (.pitch (Variables|Default|GetInitial%20Bar%20Rotation)) (.yaw (Variables|Default|GetInitial%20Bar%20Rotation))) false false))
                                  (:NewEnumerator1
                                    (Transformation|SetRelativeRotation _bar_2 (Math|Rotator|MakeRotator (.roll (Variables|Default|GetInitial%20Bar%20Rotation)) (+ (* _rotation_3 (Variables|Default|GetMax%20Bar%20Rotation%20%28degrees%29)) (.pitch (Variables|Default|GetInitial%20Bar%20Rotation))) (.yaw (Variables|Default|GetInitial%20Bar%20Rotation))) false false))
                                  (:NewEnumerator2
                                    (Transformation|SetRelativeRotation _bar_2 (Math|Rotator|MakeRotator (.roll (Variables|Default|GetInitial%20Bar%20Rotation)) (.pitch (Variables|Default|GetInitial%20Bar%20Rotation)) (+ (* _rotation_3 (Variables|Default|GetMax%20Bar%20Rotation%20%28degrees%29)) (.yaw (Variables|Default|GetInitial%20Bar%20Rotation)))) false false)))))
                            (Development|PrintString (Utilities|String|Append "Bar rotation:" (Utilities|String|ToString(Rotator) (.Rotation (Math|Transform|BreakTransform (Transformation|GetRelativeTransform _bar_2))))) _debug_8 _debug_8 "(R=1.000000,G=0.000000,B=0.036710,A=1.000000)"))
                          (:Finished
                            (Variables|Default|SetShutters%20Are%20Open false :!label _label_2)
                            (Variables|Default|SetIs%20In%20Use? false)
                            (Audio|PlaySoundatLocation (Variables|Default|GetBarLoweredSound) "0, 0, 0" "0, 0, 0" 1.0 1.0 0.0 0 0 0 0)))
                        (else
                          (goto _label_2)))))))
              (else
                ;[1 1 1] Lift the security bar then open the shutters
                (if (Rendering|IsVisible (Variables|Default|GetBar))
                  (Development|PrintString "Lifting bar" _debug_5 _debug_5)
                  (if (Variables|Default|GetBegin%20Open?)
                    (bind _rotation_4 (Timeline|LiftBarTimeline PlayFromStart)
                      (:Update
                        (if (Variables|Default|GetReverse%20Bar%20Rotation%20Direction?)
                          (switch Utilities|FlowControl|Switch|SwitchonAxisEnum (Variables|Default|GetBar%20Rotation%20Axis)
                            (:NewEnumerator0
                              (Transformation|SetRelativeRotation _bar (Math|Rotator|MakeRotator (+ (* _rotation_4 (Variables|Default|GetMax%20Bar%20Rotation%20%28degrees%29)) (.roll (Variables|Default|GetInitial%20Bar%20Rotation))) (.pitch (Variables|Default|GetInitial%20Bar%20Rotation)) (.yaw (Variables|Default|GetInitial%20Bar%20Rotation))) false false))
                            (:NewEnumerator1
                              (Transformation|SetRelativeRotation _bar (Math|Rotator|MakeRotator (.roll (Variables|Default|GetInitial%20Bar%20Rotation)) (+ (* _rotation_4 (Variables|Default|GetMax%20Bar%20Rotation%20%28degrees%29)) (.pitch (Variables|Default|GetInitial%20Bar%20Rotation))) (.yaw (Variables|Default|GetInitial%20Bar%20Rotation))) false false))
                            (:NewEnumerator2
                              (Transformation|SetRelativeRotation _bar (Math|Rotator|MakeRotator (.roll (Variables|Default|GetInitial%20Bar%20Rotation)) (.pitch (Variables|Default|GetInitial%20Bar%20Rotation)) (+ (* _rotation_4 (Variables|Default|GetMax%20Bar%20Rotation%20%28degrees%29)) (.yaw (Variables|Default|GetInitial%20Bar%20Rotation)))) false false)))
                          (else
                            (switch Utilities|FlowControl|Switch|SwitchonAxisEnum (Variables|Default|GetBar%20Rotation%20Axis)
                              (:NewEnumerator0
                                (Transformation|SetRelativeRotation _bar (Math|Rotator|MakeRotator (- (.roll (Variables|Default|GetInitial%20Bar%20Rotation)) (* _rotation_4 (Variables|Default|GetMax%20Bar%20Rotation%20%28degrees%29))) (.pitch (Variables|Default|GetInitial%20Bar%20Rotation)) (.yaw (Variables|Default|GetInitial%20Bar%20Rotation))) false false))
                              (:NewEnumerator1
                                (Transformation|SetRelativeRotation _bar (Math|Rotator|MakeRotator (.roll (Variables|Default|GetInitial%20Bar%20Rotation)) (- (.pitch (Variables|Default|GetInitial%20Bar%20Rotation)) (* _rotation_4 (Variables|Default|GetMax%20Bar%20Rotation%20%28degrees%29))) (.yaw (Variables|Default|GetInitial%20Bar%20Rotation))) false false))
                              (:NewEnumerator2
                                (Transformation|SetRelativeRotation _bar (Math|Rotator|MakeRotator (.roll (Variables|Default|GetInitial%20Bar%20Rotation)) (.pitch (Variables|Default|GetInitial%20Bar%20Rotation)) (- (.yaw (Variables|Default|GetInitial%20Bar%20Rotation)) (* _rotation_4 (Variables|Default|GetMax%20Bar%20Rotation%20%28degrees%29)))) false false)))))
                        (Development|PrintString (Utilities|String|Append "Bar rotation:" (Utilities|String|ToString(Rotator) (.Rotation (Math|Transform|BreakTransform (Transformation|GetRelativeTransform _bar))))) _debug _debug "(R=1.000000,G=0.000000,B=0.053420,A=1.000000)"))
                      (:Finished
                        (if (Variables|Default|GetBegin%20Open?)
                          _
                          (else
                            (Audio|PlaySoundatLocation (Variables|Default|GetBarRaisedSound) "0, 0, 0" "0, 0, 0" 1.0 1.0 0.0 0 0 0 0)))
                        (Utilities|FlowControl|Sequence :!label _label_3
                          (:then_0
                            (Development|PrintString "Opening right shutter" _debug_3 _debug_3)
                            (bind _rotation_5 (Timeline|OpenShutterTimeline PlayFromStart)
                              (:Update
                                (if (Variables|Default|GetReverse%20Shutter%20Open%20Direction?)
                                  (Transformation|SetRelativeRotation _rightshutter (Math|Rotator|MakeRotator (.roll (Variables|Default|GetInitial%20Left%20Shutter%20Rotation)) (.pitch (Variables|Default|GetInitial%20Left%20Shutter%20Rotation)) (+ (* _rotation_5 (Variables|Default|GetMax%20Shutter%20Rotation%20%28degrees%29)) (.yaw (Variables|Default|GetInitial%20Left%20Shutter%20Rotation)))) false false)
                                  (else
                                    (Transformation|SetRelativeRotation _rightshutter (Math|Rotator|MakeRotator (.roll (Variables|Default|GetInitial%20Left%20Shutter%20Rotation)) (.pitch (Variables|Default|GetInitial%20Left%20Shutter%20Rotation)) (- (.yaw (Variables|Default|GetInitial%20Left%20Shutter%20Rotation)) (* _rotation_5 (Variables|Default|GetMax%20Shutter%20Rotation%20%28degrees%29)))) false false)))
                                (Development|PrintString (Utilities|String|Append "Left shutter rotation:" (Utilities|String|ToString(Rotator) (Variables|/Script/Engine.SceneComponent|GetRelativeRotation (Variables|Default|GetLeftShutter)))) _debug_13 _debug_13 "(R=0.000000,G=0.660000,B=1.000000,A=1.000000)" 4.0 :!label _label_4)
                                (Development|PrintString (Utilities|String|Append "Right shutter rotation:" (Utilities|String|ToString(Rotator) (Variables|/Script/Engine.SceneComponent|GetRelativeRotation (Variables|Default|GetRightShutter)))) _debug_6 _debug_6)
                                (Variables|Default|SetBegin%20Open? false))))
                          (:then_1
                            (Development|PrintString "Opening left shutter" _debug_15 _debug_15)
                            (bind _rotation_6 (Timeline|Timeline_0 PlayFromStart)
                              (:Update
                                (if (not (Variables|Default|GetReverse%20Shutter%20Open%20Direction?))
                                  (Transformation|SetRelativeRotation _leftshutter (Math|Rotator|MakeRotator (.roll (Variables|Default|GetInitial%20Right%20Shutter%20Rotation)) (.pitch (Variables|Default|GetInitial%20Right%20Shutter%20Rotation)) (+ (* _rotation_6 (Variables|Default|GetMax%20Shutter%20Rotation%20%28degrees%29)) (.yaw (Variables|Default|GetInitial%20Right%20Shutter%20Rotation)))) false false)
                                  (goto _label_4)
                                  (else
                                    (Transformation|SetRelativeRotation _leftshutter (Math|Rotator|MakeRotator (.roll (Variables|Default|GetInitial%20Right%20Shutter%20Rotation)) (.pitch (Variables|Default|GetInitial%20Right%20Shutter%20Rotation)) (- (.yaw (Variables|Default|GetInitial%20Right%20Shutter%20Rotation)) (* _rotation_6 (Variables|Default|GetMax%20Shutter%20Rotation%20%28degrees%29)))) false false)
                                    (goto _label_4))))
                              (:Finished
                                (Variables|Default|SetShutters%20Are%20Open true)
                                (Variables|Default|SetIs%20In%20Use? false)))))))
                    (else
                      (Audio|PlaySoundatLocation (Variables|Default|GetBarRaisingSound) "0, 0, 0" "0, 0, 0" 1.0 1.0 0.0 0 0 0 0)
                      (Timeline|LiftBarTimeline PlayFromStart)))
                  (else
                    (goto _label_3))))))
          (:then_1
            (Class|InterfaceGeneralCharacter|SetIsInteractingwithObject(Message) (Game|GetPlayerCharacter 0) false)))))
    (else
      (Class|InterfaceGeneralCharacter|SetIsInteractingwithObject(Message) (Game|GetPlayerCharacter 0) false))))

(event EventBeginPlay
  (bind _debug (Variables|Default|GetDebug))
  (if (Variables|Default|GetBegin%20Open?)
    (Development|PrintString (Utilities|String|Append "Setting  " (Utilities|GetObjectName self) "to be initially open") _debug _debug)
    (CallFunction|Lookingat)))

(fn ConstructionScript)

(fn GetID
  (return ""))

(fn GetLauncherActor
  (return 0))

(fn GetObjectName
  (if (Variables|Default|GetShutters%20Are%20Open)
    (return "Close Shutter")
    (else
      (return "Open Shutter"))))

(fn IsProjectile
  (return false))