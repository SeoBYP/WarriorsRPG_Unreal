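; Interactable two-drawer furniture container that slides open and opens a trading UI with its items.
; Interact, blocked while any UI is open or the drawers are in use, stores their starting transforms and runs a timeline, then fills the container.
; CloseContainer reverses a second timeline and clears the in-use flag; the timed auto-close is disconnected.
; The bottom drawer trails the top through a timeline offset and travels less far.
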(event EventInteract
  (params (HitComponent :type Actor%20Component%20Object%20Reference) (InteractingActor :type Actor%20Object%20Reference))
  ;[1 1 1] Open the drawer then close it after waiting 2 seconds
  (if (not (Default|IsAnyUIOpen (Variables|Default|GetGameInstance))) ; If a menu isnt currently open
    ;;[1 1 1] Initialize starting location of drawers
    (if (not (Variables|Default|GetIsInUse))
      (Variables|Default|SetIsInUse true)
      (Variables|MRPGT|ReferenceOnly|SetTop%20Drawer%20Location (Transformation|GetRelativeTransform (Variables|Default|GetTopDrawer)))
      (Variables|MRPGT|ReferenceOnly|SetBottom%20Drawer%20Location (Transformation|GetRelativeTransform (Variables|Default|GetBottomDrawer)))
      (Variables|MRPGT|ReferenceOnly|SetIsMoving true)
      (Components|Timeline|SetPlayRate (Variables|Default|GetOpening_Timeline) (Variables|MRPGT|Customizable|GetDrawer%20Movement%20Rate))
      (Audio|PlaySoundatLocation "/Game/MRPGT/MedievalBuildings01/Audio/SoundCues/DrawerOpen_Cue.DrawerOpen_Cue" "0, 0, 0" "0, 0, 0" 1.0 1.0 0.0 0 0 0 0)
      ;;[1 1 1] Loop through a timeline for 1 second
      (bind _drawerposition (Timeline|Opening_Timeline PlayFromStart)
        (:Update
          ;;[1 1 1] Move drawer in the y direction every loop iteration (x and z locations doesnt change)
          (Transformation|SetRelativeLocation (Variables|Default|GetTopDrawer) (Math|Vector|MakeVector (.x (.location (Variables|MRPGT|ReferenceOnly|GetTop%20Drawer%20Location))) (+ (* _drawerposition (Variables|MRPGT|Customizable|GetMax%20Drawer%20Extent)) (.y (.location (Variables|MRPGT|ReferenceOnly|GetTop%20Drawer%20Location)))) (.z (.location (Variables|MRPGT|ReferenceOnly|GetTop%20Drawer%20Location)))) false false)
          ;;[1 1 1] Debug info
          (Development|PrintString (Utilities|String|Append "Opening." "Top drawer location:" (Utilities|String|ToString(Vector) (.location (Variables|MRPGT|ReferenceOnly|GetTop%20Drawer%20Location)))) false (Variables|Default|GetDebug))
          ;;[1 1 1] Start moving bottom drawer a little later than the top drawer
          (if (> (- _drawerposition 0.2) 0.0)
            (Transformation|SetRelativeLocation (Variables|Default|GetBottomDrawer) (Math|Vector|MakeVector (.x (.location (Variables|MRPGT|ReferenceOnly|GetBottom%20Drawer%20Location))) (+ (* (- _drawerposition 0.2) (- (Variables|MRPGT|Customizable|GetMax%20Drawer%20Extent) 4.0)) (.y (.location (Variables|MRPGT|ReferenceOnly|GetBottom%20Drawer%20Location)))) (.z (.location (Variables|MRPGT|ReferenceOnly|GetBottom%20Drawer%20Location)))) false false)))
        (:Finished
          (Development|PrintString "Fully opened" false (Variables|Default|GetDebug))
          ;;[1 1 1] Set status variables after opening completed
          (Variables|MRPGT|ReferenceOnly|SetIsMoving false)
          (Variables|MRPGT|ReferenceOnly|SetIs%20Fully%20Open true)
          (CallFunction|AddItemstoContainer)
          (CallFunction|OpenTradingUI))))))

(event EventCloseContainer
  (bind _bottom_drawer_location (Variables|MRPGT|ReferenceOnly|GetBottom%20Drawer%20Location))
  (bind _top_drawer_location (Variables|MRPGT|ReferenceOnly|GetTop%20Drawer%20Location))
  ;[1 1 1] Open the drawer then close it after waiting 2 seconds
  ;;[1 1 1] Set status variables to indicate closing is beginning
  (Variables|MRPGT|ReferenceOnly|SetIsMoving true)
  (Variables|MRPGT|ReferenceOnly|SetIs%20Fully%20Open false)
  ;;[1 1 1] Do the reverse to close the top drawer
  (Components|Timeline|SetPlayRate (Variables|Default|GetClosing_Timeline) (Variables|MRPGT|Customizable|GetDrawer%20Movement%20Rate))
  (Audio|PlaySoundatLocation "/Game/MRPGT/MedievalBuildings01/Audio/SoundCues/DrawerClose_Cue.DrawerClose_Cue" "0, 0, 0" "0, 0, 0" 1.0 1.0 0.0 0 0 0 0)
  (bind _drawerposition (Timeline|Closing_Timeline ReverseFromEnd)
    (:Update
      (Transformation|SetRelativeLocation (Variables|Default|GetTopDrawer) (Math|Vector|MakeVector (.x (.location _top_drawer_location)) (+ (* _drawerposition (Variables|MRPGT|Customizable|GetMax%20Drawer%20Extent)) (.y (.location _top_drawer_location))) (.z (.location _top_drawer_location))) false false)
      ;;[1 1 1] Debug info
      (Development|PrintString (Utilities|String|Append "Closing. " "Top drawer Y location:" (Utilities|String|ToString(Vector) (.location (Variables|MRPGT|ReferenceOnly|GetTop%20Drawer%20Location)))) false (Variables|Default|GetDebug))
      ;;[1 1 1] Start moving bottom drawer a little later than the top drawer
      (if (> (- _drawerposition 0.2) 0.0)
        (Transformation|SetRelativeLocation (Variables|Default|GetBottomDrawer) (Math|Vector|MakeVector (.x (.location _bottom_drawer_location)) (+ (* (- _drawerposition 0.2) (- (Variables|MRPGT|Customizable|GetMax%20Drawer%20Extent) 4.0)) (.y (.location _bottom_drawer_location))) (.z (.location _bottom_drawer_location))) false false)))
    (:Finished
      (Development|PrintString "Fully closed" false (Variables|Default|GetDebug))
      (Variables|Default|SetIsInUse false))))

(fn ConstructionScript)

(fn GetName
  (return (Utilities|String|Append (Utilities|String|SelectString "Close " "Open " (Variables|MRPGT|ReferenceOnly|GetIs%20Fully%20Open)) (Utilities|String|ToString(Text) (.Name (Utilities|Struct|BreakContainerStruct (Variables|Default|GetContainerInfo)))))))