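; BP_TestItem is a collectable item that the player hero picks up through interaction.
; On interact, it adds its item ID and quantity from the item data component to the hero's inventory component, then destroys itself.
; On destruction, it records itself in the save subsystem's removed-actor list for the level.
; At BeginPlay, it configures its interactable component from a "Collectable" data table row.
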(event OnInteract(Interactable)
  (params (Interactor :type Interactor%20Component%20Object%20Reference) (Interactable :type Interactable%20Component%20Object%20Reference))
  (bind _bp_itemdatacomponent (Variables|Default|GetBP_ItemDataComponent))
  (bind _aswarrior_hero_character (Utilities|Casting|CastToWarriorHeroCharacter (Components|GetOwner Interactor)))
  (Class|InventoryComponent|AddInventory (Actor|GetComponentbyClass _aswarrior_hero_character "/Game/Inventory/BP_InventoryComponent.BP_InventoryComponent_C") (.rowname (Variables|/Script/Warriors.ItemDataComponent|GetItemID _bp_itemdatacomponent)) (Variables|/Script/Warriors.ItemDataComponent|GetQuantity _bp_itemdatacomponent))
  (Actor|DestroyActor))

(event EventBeginPlay
  (Class|InteractableComponent|SetInteractableDataBasedonDataTable (Variables|Default|GetInteractable) "/Game/DataTables/DT_InteractDataTable.DT_InteractDataTable" "Collectable"))

(event EventDestroyed
  (Utilities|Array|AddUnique (Variables|/Script/Warriors.LevelSaveData|GetActorsRemoved (Variables|/Script/Warriors.SaveLoadSubSystem|GetLevelSaveData (Subsystems|GetSaveLoadSubSystem))) (Utilities|ResolveSoftReference self)))

(fn ConstructionScript)