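; Game instance that sets up persistent quest save data when the game starts.
; Init calls SaveQuestData, which loads the quest slot or creates a new save object and caches it, without writing to disk.
; RemoveSaveData deletes the quest slot under user index 1, whereas loading uses index 0.
; A similar inventory load-or-create chain that also saves to slot is disconnected and never runs.
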(event EventInit
  (CallFunction|SaveQuestData))

(fn RemoveSaveData
  (SaveGame|DeleteGameinSlot "QuestSaveData" 1))

(fn SaveQuestData
  (bind _returnvalue (SaveGame|DoesSaveGameExist "QuestSaveData"))
  (if _returnvalue
    (bind _returnvalue_2 (SaveGame|LoadGamefromSlot "QuestSaveData"))
    (bind _asquest_save_game (Utilities|Casting|CastToQuestSaveGame _returnvalue_2))
    (Variables|Default|SetQuestSaveGame _asquest_save_game)
    (else
      (bind _returnvalue_3 (SaveGame|CreateSaveGameObject "/Game/Resources/Data/SaveData/QuestSaveGame.QuestSaveGame_C"))
      (Variables|Default|SetQuestSaveGame _returnvalue_3))))