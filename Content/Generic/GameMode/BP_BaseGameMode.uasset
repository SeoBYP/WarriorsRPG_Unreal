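; Base game mode meant to persist per-level actor changes in a save game, though its load logic is disconnected and BeginPlay is empty.
; EndPlay saves LevelSaveGame to the LevelDataSlot slot.
; The unwired chain names the slot after the level, then creates a new save or loads the existing one to respawn added actors and destroy removed ones.
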(event EventBeginPlay)

(event EventEndPlay
  (params (EndPlayReason :type EEndPlayReason%20Enum :default "Destroyed"))
  (SaveGame|SaveGametoSlot (Variables|Default|GetLevelSaveGame) (Variables|Default|GetLevelDataSlot)))

(fn ConstructionScript)