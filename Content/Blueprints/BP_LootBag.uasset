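; BP_LootBag is a loot bag actor with an inventory component that registers itself for level persistence.
; On BeginPlay it records its class and transform in the save subsystem's ActorsAdded data and saves the level.
; Logic to close the container menu, record removal and destroy the bag once empty is disconnected, so the inventory update and Destroyed events do nothing.
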(event OnUpdatedInventory(BP_InventoryComponent))

(event EventBeginPlay
  (Utilities|Map|Add (Variables|/Script/Warriors.LevelSaveData|GetActorsAdded (Variables|/Script/Warriors.SaveLoadSubSystem|GetLevelSaveData (Subsystems|GetSaveLoadSubSystem))) (Utilities|ResolveSoftReference (Utilities|GetClass self)) (Transformation|GetActorTransform))
  (Class|SaveLoadSubSystem|SaveLevelSaveData (Subsystems|GetSaveLoadSubSystem)))

(event EventDestroyed)

(fn ConstructionScript
  (|CallParentFunction))