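; BP_Chest is an interactable container that opens its inventory in the hero HUD when the player interacts with it.
; On BeginPlay it sets up its Interactable component from the "Collect" data table row, then loads its inventory component after a short delay marked as provisional.
; On interact it gets the hero HUD from the Warrior game instance and passes the inventory component to ShowContainer.
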(event OnInteract(Interactable)
  (params (Interactor :type Interactor%20Component%20Object%20Reference) (Interactable :type Interactable%20Component%20Object%20Reference))
  (bind _returnvalue (Class|WarriorFunctionLibrary|GetWarriorGameInstance))
  (bind _returnvalue_2 (Class|WarriorGameInstance|GetHeroHUD _returnvalue))
  (Utilities|IsValid _returnvalue_2
    (:Is%20Valid
      (bind _aswbp_hero_hud (Utilities|Casting|CastToWBP_HeroHUD _returnvalue_2))
      (Default|ShowContainer _aswbp_hero_hud (Variables|Default|GetBP_InventoryComponent)))))

(event EventBeginPlay
  (Class|InteractableComponent|SetInteractableDataBasedonDataTable (Variables|Default|GetInteractable) "/Game/DataTables/DT_InteractDataTable.DT_InteractDataTable" "Collect")
  ;[1 1 1] 딜레이 추후 수정
  (Utilities|FlowControl|Delay 0.2)
  (Class|InventoryComponent|LoadInventory (Variables|Default|GetBP_InventoryComponent)))

(fn ConstructionScript)