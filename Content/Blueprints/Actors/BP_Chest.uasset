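; BP_Chest is a chest actor that opens or closes a container inventory screen when interacted with.
; Its InteractableComponent's OnInteract event removes and clears any valid container widget held by the widget subsystem.
; Otherwise it creates a WBP_ContainerInventory bound to its InventoryComponent, registers it with the subsystem and adds it to the viewport.
; The toggle checks the subsystem's shared reference, so interacting closes whichever container screen is registered there.
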(event OnInteract(InteractableComponent)
  (params (Interactor :type Interactor%20Component%20Object%20Reference) (Interactable :type Interactable%20Component%20Object%20Reference))
  (Utilities|IsValid (Variables|/Script/Warriors.WidgetSubSystem|GetHeroContainerInventory (Subsystems|GetWidgetSubSystem))
    (:Is%20Valid
      (Widget|RemovefromParent (Variables|/Script/Warriors.WidgetSubSystem|GetHeroContainerInventory (Subsystems|GetWidgetSubSystem)))
      (Class|WidgetSubSystem|SetContainerInventory (Subsystems|GetWidgetSubSystem)))
    (:Is%20Not%20Valid
      (bind _returnvalue (UserInterface|CreateWidget "/Game/Widgets/InventoryWidget/WBP_ContainerInventory.WBP_ContainerInventory_C" 0 (Variables|Default|GetInventoryComponent)))
      (Class|WidgetSubSystem|SetContainerInventory (Subsystems|GetWidgetSubSystem) _returnvalue)
      (UserInterface|Viewport|AddtoViewport _returnvalue 0))))

(event EventBeginPlay)

(event Collision|EventActorBeginOverlap
  (params (OtherActor :type Actor%20Object%20Reference)))

(event EventTick
  (params (DeltaSeconds :type Float%20%28single-precision%29)))

(fn ConstructionScript)