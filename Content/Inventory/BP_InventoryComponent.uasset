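; Inventory component that restores its contents at BeginPlay and saves them automatically whenever they change.
; BeginPlay calls LoadInventory, resizes Contents to InventorySize, then binds AutoSaveInventory to OnUpdatedInventory, which calls SaveInventory.
; DropItemEvent2 is an empty stub.
; Disconnected leftover nodes sketch dropping items in front of the owner, as a loot bag or as an item actor recorded in level save data.
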(event Custom|DropItemEvent2)

(event Custom|AutoSaveInventory
  (Class|InventoryComponent|SaveInventory))

(event EventBeginPlay
  (Class|InventoryComponent|LoadInventory)
  (Utilities|Array|Resize (Variables|Default|GetContents) (Variables|Default|GetInventorySize))
  (EventDispatchers|BindEventtoOnUpdatedInventory (delegate Custom|AutoSaveInventory)))

(event EventTick
  (params (DeltaSeconds :type Float%20%28single-precision%29)))